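; BP_FlowerBell is a flower bell hazard actor that punishes the SecondGameplayCharacter for touching it.
; On overlap with that character it closes its referenced Door, applies damage, posts the FlowerBell Wwise event and prints a debug string.
; Each tick it reads WindIntensity from the MPCWind parameter collection and snaps its roll to a fixed tilt when wind is non-zero, upright otherwise.
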(event `self.ReceiveTick`
  (params (DeltaSeconds :type "Float (single-precision)"))
  (bind (_returnvalue_roll _returnvalue_pitch _returnvalue_yaw) (`KismetMathLibrary.BreakRotator` (`self.K2_GetActorRotation`)))
  (bind _returnvalue (`KismetMaterialLibrary.GetScalarParameterValue` (`self.MPC_Wind`) (`self.Wind Intensity`)))
  (if (== _returnvalue 0.0)
    (`self.K2_SetActorRotation` (`KismetMathLibrary.MakeRotator` 0.0 _returnvalue_pitch _returnvalue_yaw) true)
    (else
      (`self.K2_SetActorRotation` (`KismetMathLibrary.MakeRotator` 20.0 _returnvalue_pitch _returnvalue_yaw) true))))

(event `self.ReceiveActorBeginOverlap`
  (params (OtherActor :type "Actor Object Reference"))
  (bind _assecond_gameplay_character (cast `/Game/ThirdPersonCPP/Blueprints/SecondGameplayCharacter` OtherActor))
  (`/Game/ThirdPersonCPP/Blueprints/Francois/Door.CloseDoor` (`self.door`))
  (`GameplayStatics.ApplyDamage` _assecond_gameplay_character 1.0 null self)
  (`AkGameplayStatics.PostEvent` "/Game/Dream_Hunter/Sound/flowerBell.flowerBell" self)
  (`KismetSystemLibrary.PrintString` "deal damage"))

(fn `UserConstructionScript`)