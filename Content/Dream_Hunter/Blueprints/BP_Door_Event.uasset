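; BP_Door_Event is a door Blueprint that slides open and closed through a single OpenDoor event.
; Each call flips IsOpen and plays or reverses DoorTimeline to match.
; The timeline's DoorAnim track lerps the Door component's relative location between StartPos and StartPos plus the EndLoaction offset, without sweeping.
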(event `OpenDoor`
  (if (`self.isOpen`)
    (set `self.isOpen` false)
    (bind (_direction _dooranim) (`Timeline|DoorTimeline` :!via `Reverse` :!label _label)
      (:`Update`
        (`SceneComponent.K2_SetRelativeLocation` (`self.Door`) (`KismetMathLibrary.VLerp` (`self.StartPos`) (+ (`self.EndLoaction`) (`self.StartPos`)) _dooranim) false false)))
    (else
      (set `self.isOpen` true)
      (goto _label))))

(fn `UserConstructionScript`)