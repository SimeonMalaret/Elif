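; PipeActivator is a trigger actor that sends a SecondGameplayCharacter along a linked Pipe's path.
; Its Box overlap arms it and stores the player, disarming when the player leaves.
; Pressing K while armed calls StartPath on the Pipe with the direction and itself as start point.
; The Cylinder turns red and blocks re-triggering for a set duration, then reverts to violet.
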(event `Key|K`
  (params (Key :type "Key Structure"))
  (:`Pressed`
    (`KismetSystemLibrary.PrintString` "Hello")
    (if (`self.isActivate`)
      (if (not (`self.isActive`))
        (set `self.isActive` true)
        (`/Game/Dream_Hunter/Blueprints/Pipe.StartPath` (`self.Pipe`) (`self.Player`) (`self.isPositiveDirection`) self)
        (`PrimitiveComponent.SetMaterial` (`self.Cylinder`) 0 "/Game/Dream_Hunter/Blueprints/Red.Red")
        (`KismetSystemLibrary.Delay` (`self.Duration`))
        (set `self.isActive` false)
        (`PrimitiveComponent.SetMaterial` (`self.Cylinder`) 0 "/Game/Dream_Hunter/Blueprints/Violet.Violet")))))

(event `self.Box.OnComponentBeginOverlap`
  (params (OverlappedComponent :type "PrimitiveComponent Object Reference") (OtherActor :type "Actor Object Reference") (OtherComp :type "PrimitiveComponent Object Reference") (OtherBodyIndex :type Integer) (bFromSweep :type Boolean) (SweepResult :type "HitResult Structure (by ref)"))
  (cast `/Game/ThirdPersonCPP/Blueprints/SecondGameplayCharacter` OtherActor)
  (set `self.isActivate` true)
  (set `self.Player` OtherActor))

(event `self.Box.OnComponentEndOverlap`
  (params (OverlappedComponent :type "PrimitiveComponent Object Reference") (OtherActor :type "Actor Object Reference") (OtherComp :type "PrimitiveComponent Object Reference") (OtherBodyIndex :type Integer))
  (cast `/Game/ThirdPersonCPP/Blueprints/SecondGameplayCharacter` OtherActor)
  (set `self.isActivate` false))

(fn `UserConstructionScript`)