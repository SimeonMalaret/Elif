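; Pillar actor that, when StartMovement is called, moves by the EndPosition offset, waits, then returns to its start, apparently sinking and rising again.
; StartMovement ignores calls while active and turns off the cube's collision before the outbound timeline plays.
; When that finishes, MovingUp waits DurationDown, plays the return timeline, then restores collision and clears IsActive for reuse.
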(event `self.ReceiveBeginPlay`
  (bind _output_get (set `self.Start Position` (`self.K2_GetActorLocation`)))
  (set `self.Final Position` (+ _output_get (`self.End Position`))))

(event `MoveTime`
  (bind (_direction _newtrack_0) (`Timeline|MovementTimeline` :!via `PlayFromStart`)
    (:`Update`
      (`self.K2_SetActorLocation` self (`KismetMathLibrary.VLerp` (`self.Start Position`) (+ (`self.Start Position`) (`self.End Position`)) _newtrack_0) false false))
    (:`Finished`
      (set `self.isActive` true)
      (`self.MovingUp`))))

(event `MovingUp`
  (if (`self.isActive`)
    (`KismetSystemLibrary.Delay` (`self.Duration Down`))
    (bind (_direction _newtrack_0) (`Timeline|Timeline_0` :!via `PlayFromStart`)
      (:`Update`
        (`self.K2_SetActorLocation` self (`KismetMathLibrary.VLerp` (`self.Final Position`) (- (`self.Final Position`) (`self.End Position`)) _newtrack_0) false false))
      (:`Finished`
        (`PrimitiveComponent.SetCollisionEnabled` (`self.Cube`) "QueryAndPhysics")
        (set `self.isActive` false)))))

(fn `StartMovement`
  (if (not (`self.isActive`))
    (set `self.isActive` true)
    (`PrimitiveComponent.SetCollisionEnabled` (`self.Cube`) "NoCollision")
    (`self.MoveTime`))
  (return))

(fn `UserConstructionScript`)