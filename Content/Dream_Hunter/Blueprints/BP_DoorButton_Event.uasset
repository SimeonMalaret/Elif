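; BP_DoorButton_Event is a trigger button that opens every BP_Door_Event door in the level when the player character overlaps it.
; On BeginPlay it caches all BP_Door_Event actors with GetAllActorsOfClass.
; On overlap by a ThirdPersonCharacterDashSimple, it calls OpenDoor on each cached door if the character is dashing or if DashConstraint is off.
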(event `self.ReceiveBeginPlay`
  (bind _outactors (`GameplayStatics.GetAllActorsOfClass` "/Game/Dream_Hunter/Blueprints/BP_Door_Event.BP_Door_Event_C"))
  (set `self.Out Actors` _outactors))

(event `self.ReceiveActorBeginOverlap`
  (params (OtherActor :type "Actor Object Reference"))
  (bind _asthird_person_character_dash_simple (cast `/Game/ThirdPersonCPP/Blueprints/ThirdPersonCharacterDashSimple` OtherActor))
  (if (`/Game/ThirdPersonCPP/Blueprints/ThirdPersonCharacterDashSimple.isDashing` _asthird_person_character_dash_simple)
    (for _array_element (`self.Out Actors`) :!label _label
      (`/Game/Dream_Hunter/Blueprints/BP_Door_Event.OpenDoor` _array_element))
    (elif (not (`self.dashConstraint`))
      (goto _label))))

(fn `UserConstructionScript`)