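; Rocket actor that gives a character a timed forward dash through its BoostDash function.
; BoostDash, gated by CanDash, stores the passed actor as Player and multiplies its max walk speed by a coefficient.
; Tick counts down the dash duration while forcing forward movement input, then restores the speed and re-arms the dash after a cooldown delay.
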(event `self.ReceiveBeginPlay`
  (`parent.ReceiveBeginPlay`)
  (set `self.DurationLeft` (`self.DurationDash`)))

(event `self.ReceiveTick`
  (params (DeltaSeconds :type "Float (single-precision)"))
  (bind _player (`self.Player`))
  (bind _charactermovement (`Character.CharacterMovement` (`self.Player`)))
  (if (`self.Dashing`)
    (bind _output_get (set `self.DurationLeft` (- (`self.DurationLeft`) DeltaSeconds)))
    (if (> _output_get 0.0)
      (`Pawn.AddMovementInput` _player (`self.GetActorForwardVector` _player) (`self.PowerDash`) true)
      (else
        (set `self.DurationLeft` (`self.DurationDash`))
        (set `CharacterMovementComponent.MaxWalkSpeed` (/ (`CharacterMovementComponent.MaxWalkSpeed` _charactermovement) (`self.CoefSpeed`)) _charactermovement)
        (set `self.Dashing` false)
        (`KismetSystemLibrary.Delay` (`self.Cooldown`))
        (set `self.Player` null)
        (set `self.CanDash` true)))))

(fn `BoostDash`
  (params (Actor :type "/Game/ThirdPersonCPP/Blueprints/SecondGameplayCharacter Object Reference"))
  (if (`self.CanDash`)
    (bind _output_get (set `self.Player` Actor))
    (bind _charactermovement (`Character.CharacterMovement` _output_get))
    (set `CharacterMovementComponent.MaxWalkSpeed` (* (`CharacterMovementComponent.MaxWalkSpeed` _charactermovement) (`self.CoefSpeed`)) _charactermovement)
    (set `self.CanDash` false)
    (set `self.Dashing` true)
    (return)))

(fn `UserConstructionScript`
  (`parent.UserConstructionScript`))