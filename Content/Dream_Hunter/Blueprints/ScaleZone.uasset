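; ScaleZone is a trigger volume that gradually resizes the SecondGameplayCharacter as it moves between two markers, PosA and PosB.
; While the character overlaps the box, Tick derives a target size between BaseSize and EndSize from its relative distances to both markers.
; Capsule scale eases toward that target by a fixed per-frame fraction.
; The resulting size also interpolates camera boom height and socket offset.
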(event `self.ReceiveBeginPlay`
  (bind (_returnvalue_x _returnvalue_y _returnvalue_z) (`KismetMathLibrary.BreakVector` (`self.GetActorScale3D` (`self.Character`))))
  (bind _returnvalue (`GameplayStatics.GetActorOfClass` "/Game/ThirdPersonCPP/Blueprints/SecondGameplayCharacter.SecondGameplayCharacter_C"))
  (set `self.Character` _returnvalue)
  (set `self.CurrentSize` _returnvalue_z))

(event `self.ReceiveTick`
  (params (DeltaSeconds :type "Float (single-precision)"))
  (if (`self.isOverlap`)
    (`self.SetScale`)))

(event `SetScale`
  (bind _returnvalue (/ (- (`self.CurrentSize`) (`self.BaseSize`)) (- (`self.EndSize`) (`self.BaseSize`))))
  (bind _returnvalue_2 (`KismetMathLibrary.Vector_Distance` (`self.K2_GetActorLocation` (`self.Character`)) (`self.K2_GetActorLocation` (`self.PosA`))))
  (set `self.lastSize` (`self.CurrentSize`))
  (set `self.TargetSize` (+ (`self.BaseSize`) (* (/ _returnvalue_2 (+ _returnvalue_2 (`KismetMathLibrary.Vector_Distance` (`self.K2_GetActorLocation` (`self.Character`)) (`self.K2_GetActorLocation` (`self.PosB`))))) (- (`self.EndSize`) (`self.BaseSize`)))))
  (bind _output_get (set `self.CurrentSize` (+ (* (- (`self.TargetSize`) (`self.CurrentSize`)) 0.1) (`self.CurrentSize`))))
  (`SceneComponent.SetWorldScale3D` (`Character.CapsuleComponent` (`self.Character`)) (* (`KismetMathLibrary.Vector_One`) _output_get))
  (`SceneComponent.K2_SetRelativeLocation` (`DreamHuntersCharacter.CameraBoom` (`self.Character`)) (`KismetMathLibrary.MakeVector` 0.0 0.0 (`KismetMathLibrary.Lerp` (`.ZPos_2_E563CAE64AD16A3A9D4255A63945FF9E` (break `/Game/ThirdPersonCPP/Blueprints/CamBoomParam` (`self.BoomStart`))) (`.ZPos_2_E563CAE64AD16A3A9D4255A63945FF9E` (break `/Game/ThirdPersonCPP/Blueprints/CamBoomParam` (`self.BoomEnd`))) _returnvalue)) false true)
  (set `SpringArmComponent.SocketOffset` (`KismetMathLibrary.VLerp` (`.socketOffset_5_D560C2FC4F13490F8959F899861DF0DF` (break `/Game/ThirdPersonCPP/Blueprints/CamBoomParam` (`self.BoomStart`))) (`.socketOffset_5_D560C2FC4F13490F8959F899861DF0DF` (break `/Game/ThirdPersonCPP/Blueprints/CamBoomParam` (`self.BoomEnd`))) _returnvalue) (`DreamHuntersCharacter.CameraBoom` (`self.Character`))))

(event `self.Box.OnComponentBeginOverlap`
  (params (OverlappedComponent :type "PrimitiveComponent Object Reference") (OtherActor :type "Actor Object Reference") (OtherComp :type "PrimitiveComponent Object Reference") (OtherBodyIndex :type Integer) (bFromSweep :type Boolean) (SweepResult :type "HitResult Structure (by ref)"))
  ;[1 1 1] Overlap
  (bind _assecond_gameplay_character (cast `/Game/ThirdPersonCPP/Blueprints/SecondGameplayCharacter` OtherActor))
  (set `self.Character` _assecond_gameplay_character)
  (set `self.isOverlap` true)
  (`KismetSystemLibrary.PrintString` "On"))

(event `self.Box.OnComponentEndOverlap`
  (params (OverlappedComponent :type "PrimitiveComponent Object Reference") (OtherActor :type "Actor Object Reference") (OtherComp :type "PrimitiveComponent Object Reference") (OtherBodyIndex :type Integer))
  ;[1 1 1] Overlap
  (cast `/Game/ThirdPersonCPP/Blueprints/SecondGameplayCharacter` OtherActor)
  (set `self.isOverlap` false)
  (`KismetSystemLibrary.PrintString` "Off"))

(fn `UserConstructionScript`)