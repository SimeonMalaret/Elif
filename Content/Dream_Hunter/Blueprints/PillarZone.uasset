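; PillarZone is an enemy kill zone that grows into place once all of its linked pillars are active.
; On BeginPlay it stores its authored scale, collapses to zero and registers itself on each pillar.
; TestZoneActivation checks every pillar, then either plays a timeline scaling the root back to full size or prints a warning.
; Any Enemy that begins overlapping the kill zone component is destroyed.
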(event `self.ReceiveBeginPlay`
  (bind _defaultsceneroot (`self.DefaultSceneRoot`))
  (set `self.killSize` (`SceneComponent.K2_GetComponentScale` _defaultsceneroot))
  (`SceneComponent.SetWorldScale3D` _defaultsceneroot (0.0 0.0 0.0))
  (for _array_element (`self.Pillars`)
    (set `/Game/Dream_Hunter/Blueprints/Pillar.Zone` self _array_element)))

(event `TestZoneActivation`
  (set `self.canActivate` true)
  (for _array_element (`self.Pillars`)
    (if (not (`/Game/Dream_Hunter/Blueprints/Pillar.isActive` _array_element))
      (set `self.canActivate` false)))
  (if (`self.canActivate`)
    (set `self.isActive` true)
    (bind (_direction _grow) (`Timeline|Grow` :!via `PlayFromStart`)
      (:`Update`
        (`SceneComponent.SetWorldScale3D` (`self.DefaultSceneRoot`) (* (`self.killSize`) _grow))))
    (else
      (`KismetSystemLibrary.PrintString` "1 or more pillar is inactive"))))

(event `self.EnnemyKillZone.OnComponentBeginOverlap`
  (params (OverlappedComponent :type "PrimitiveComponent Object Reference") (OtherActor :type "Actor Object Reference") (OtherComp :type "PrimitiveComponent Object Reference") (OtherBodyIndex :type Integer) (bFromSweep :type Boolean) (SweepResult :type "HitResult Structure (by ref)"))
  (bind _asenemy (cast `/Game/ThirdPersonCPP/Blueprints/Enemy` OtherActor))
  (`self.K2_DestroyActor` _asenemy))

(fn `UserConstructionScript`)