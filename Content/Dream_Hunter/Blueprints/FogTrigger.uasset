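; FogTrigger is an overlap trigger that clears the level's fog when the SecondGameplayCharacter enters it.
; It finds the first ExponentialHeightFog in the level and records its current start distance and max opacity.
; The FogDissipate timeline lerps both values toward configurable end values.
; When the timeline finishes, it destroys that fog, the first AtmosphericFog and the trigger itself.
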(event `self.ReceiveActorBeginOverlap`
  (params (OtherActor :type "Actor Object Reference"))
  (bind _component (`ExponentialHeightFog.Component` (`self.Fog`)))
  (cast `/Game/ThirdPersonCPP/Blueprints/SecondGameplayCharacter` OtherActor)
  (`KismetSystemLibrary.PrintString` "Hello")
  (bind _outactors (`GameplayStatics.GetAllActorsOfClass` "/Script/Engine.ExponentialHeightFog"))
  (bind _output_get (set `self.Fog` (`|GetArrayItem` _outactors)))
  (bind _component_2 (`ExponentialHeightFog.Component` _output_get))
  (set `self.InitialStartDistance` (`ExponentialHeightFogComponent.StartDistance` _component_2))
  (set `self.InitialMaxOpacity` (`ExponentialHeightFogComponent.FogMaxOpacity` _component_2))
  (bind (_direction _timedissipate) (`Timeline|FogDissipate` :!via `PlayFromStart`)
    (:`Update`
      (`ExponentialHeightFogComponent.SetFogMaxOpacity` _component (`KismetMathLibrary.Lerp` (`self.InitialMaxOpacity`) (`self.EndMaxOpacity`) _timedissipate))
      (`ExponentialHeightFogComponent.SetStartDistance` _component (`KismetMathLibrary.Lerp` (`self.InitialStartDistance`) (`self.EndStartDistance`) _timedissipate)))
    (:`Finished`
      (`self.K2_DestroyActor` (`self.Fog`))
      (bind _outactors_2 (`GameplayStatics.GetAllActorsOfClass` "/Script/Engine.AtmosphericFog"))
      (`self.K2_DestroyActor` (`|GetArrayItem` _outactors_2))
      (`self.K2_DestroyActor`))))

(fn `UserConstructionScript`)