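; Wind trigger actor that shifts the wind and turns bell flowers when the SecondGameplayCharacter overlaps it.
; Each overlap restarts a timeline that sweeps the WindIntensity parameter in the MPCWind material parameter collection between opposite values.
; A second timeline, played or reversed by IsOnRight, lerps the yaw of every BP_FlowerBell between StartRotation and EndRotation, flipping that flag when finished.
; It fetches all flower actors on every timeline update.
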(event `self.CollisionComponent.OnComponentBeginOverlap`
  (params (OverlappedComponent :type "PrimitiveComponent Object Reference") (OtherActor :type "Actor Object Reference") (OtherComp :type "PrimitiveComponent Object Reference") (OtherBodyIndex :type Integer) (bFromSweep :type Boolean) (SweepResult :type "HitResult Structure (by ref)")))

(event `self.ReceiveActorBeginOverlap`
  (params (OtherActor :type "Actor Object Reference"))
  (cast `/Game/ThirdPersonCPP/Blueprints/SecondGameplayCharacter` OtherActor)
  (`|ExecutionSequence`
    (:`then_0`
      (bind (_direction _windlerp) (`Timeline|Wind Transition` :!via `PlayFromStart`)
        (:`Update`
          (`KismetMaterialLibrary.SetScalarParameterValue` (`self.MPC_Wind`) (`self.Wind Intensity`) (`KismetMathLibrary.Lerp` -7.0 7.0 _windlerp)))))
    (:`then_1`
      (if (`self.IsOnRight`)
        (bind (_direction_2 _flowerrotation) (`Timeline|Flower Rotation` :!label _label)
          (:`Update`
            (bind _outactors (`GameplayStatics.GetAllActorsOfClass` "/Game/Dream_Hunter/FlowerBell/BP_FlowerBell.BP_FlowerBell_C"))
            (for _array_element _outactors
              (bind (_returnvalue_roll _returnvalue_pitch) (`KismetMathLibrary.BreakRotator` (`self.K2_GetActorRotation` _array_element)))
              (`self.K2_SetActorRotation` _array_element (`KismetMathLibrary.MakeRotator` _returnvalue_roll _returnvalue_pitch (`KismetMathLibrary.Lerp` (`self.StartRotation`) (`self.EndRotation`) _flowerrotation)) true)))
          (:`Finished`
            (set `self.IsOnRight` (not (`self.IsOnRight`)))))
        (else
          (goto _label :!via `Reverse`))))))

(fn `UserConstructionScript`)