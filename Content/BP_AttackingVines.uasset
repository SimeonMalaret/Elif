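; BP_AttackingVines is a trap that moves its mesh between two relative positions when the player character enters its sphere.
; The overlap sets a one-shot flag, spawns a scaled-down water ripple as a warning, then waits a preparation delay.
; A timeline lerps the mesh out, and its update starts the cooldown delay.
; ResetTrap then clears the flag, destroys the ripple and reverses the timeline, re-arming the trap.
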(event `self.Sphere.OnComponentBeginOverlap`
  (params (OverlappedComponent :type "PrimitiveComponent Object Reference") (OtherActor :type "Actor Object Reference") (OtherComp :type "PrimitiveComponent Object Reference") (OtherBodyIndex :type Integer) (bFromSweep :type Boolean) (SweepResult :type "HitResult Structure (by ref)"))
  (cast `/Game/ThirdPersonCPP/Blueprints/LevelDesignTest_TpsCharacter` OtherActor)
  (if (not (`self.IsTriggered`))
    (set `self.IsTriggered` true)
    (bind _returnvalue (`|SpawnActorFromClass` "/Game/CartoonWaterShader/Blueprints/CartoonWaterBlueprints/BP_WaterRipple_River.BP_WaterRipple_River_C" (`KismetMathLibrary.MakeTransform` (+ (`self.RipplePlacement`) (`SceneComponent.K2_GetComponentLocation` (`self.DefaultSceneRoot`)))) "Undefined" "OverrideRootScale" null null))
    (bind _output_get (set `self.Ripple` _returnvalue))
    (`self.SetActorScale3D` _output_get (0.25 0.25 0.25))
    (`KismetSystemLibrary.Delay` (`self.Preparation`))
    (bind (_direction _activation) (`Timeline|TrapActivation` :!label _label)
      (:`Update`
        (`SceneComponent.K2_SetRelativeLocation` (`self.StaticMesh`) (`KismetMathLibrary.VLerp` (`self.PositionA`) (`self.PositionB`) _activation) false false)
        (if (`self.IsTriggered`)
          (`KismetSystemLibrary.Delay` (`self.Cooldown`))
          (`self.ResetTrap`))))))

(event `ResetTrap`
  (set `self.IsTriggered` false)
  (`self.K2_DestroyActor` (`self.Ripple`))
  (goto _label :!via `ReverseFromEnd`))

(fn `UserConstructionScript`)