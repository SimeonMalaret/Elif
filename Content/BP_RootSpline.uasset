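; BP_RootSpline builds a root from spline mesh components laid along an editable spline.
; The construction script grows or trims RootDataArray to match the spline point count, filling new entries from RootMeshDefaults.
; It then loops over the points, adding RootMesh segments shaped by point locations and tangents, with per-point width, thickness and bank.
; A Collisions flag toggles collision on each segment; the event graph is empty.
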(fn `Build Root Element`
  (params (LoopIndex :type Integer) (RootElementMesh :type "StaticMesh Object Reference"))
  (locals (Local_CurrentLoopIndex :type Integer) (Local_NextLoopIndex :type Integer) (Local_RootElementMesh :type "StaticMesh Object Reference") (Local_StartLocation :type "Vector Structure") (Local_StartTangent :type "Vector Structure") (Local_EndLocation :type "Vector Structure") (Local_EndTangent :type "Vector Structure") (Local_CurrentSplineMesh :type "SplineMeshComponent Object Reference") (Local_StartRoll :type "Float (double-precision)") (Local_StartScale :type "Vector2D Structure") (Local_EndRoll :type "Float (double-precision)") (Local_EndScale :type "Vector2D Structure"))
  (bind (_location _tangent) (`SplineComponent.GetLocationAndTangentAtSplinePoint` (`self.Spline`) (`local.Local_NextLoopIndex`) "Local"))
  (bind (_location_2 _tangent_2) (`SplineComponent.GetLocationAndTangentAtSplinePoint` (`self.Spline`) (`local.Local_CurrentLoopIndex`) "Local"))
  (bind (_output_rootbank _output_rootwidth _output_rootthickness) (break `/Game/RootData` (`|GetArrayItem` (`self.RootDataArray`) (`local.Local_NextLoopIndex`))))
  (bind (_output_rootbank_2 _output_rootwidth_2 _output_rootthickness_2) (break `/Game/RootData` (`|GetArrayItem` (`self.RootDataArray`) (`local.Local_CurrentLoopIndex`))))
  (set `local.Local_CurrentLoopIndex` LoopIndex)
  (set `local.Local_NextLoopIndex` (+ LoopIndex 1))
  (set `local.Local_RootElementMesh` RootElementMesh)
  (`|ExecutionSequence`
    (:`then_0`
      (set `local.Local_StartLocation` _location_2)
      (set `local.Local_StartTangent` _tangent_2)
      (set `local.Local_EndLocation` _location)
      (set `local.Local_EndTangent` _tangent)
      (set `local.Local_StartRoll` _output_rootbank_2)
      (set `local.Local_StartScale` (`KismetMathLibrary.MakeVector2D` _output_rootwidth_2 _output_rootthickness_2))
      (set `local.Local_EndRoll` _output_rootbank)
      (set `local.Local_EndScale` (`KismetMathLibrary.MakeVector2D` _output_rootwidth _output_rootthickness)))
    (:`then_1`
      (bind _returnvalue (`AddComponent|NODE_AddSplineMeshComponent-1`))
      (set `local.Local_CurrentSplineMesh` _returnvalue)
      (`StaticMeshComponent.SetStaticMesh` (`local.Local_CurrentSplineMesh`) (`local.Local_RootElementMesh`))
      (`SplineMeshComponent.SetStartAndEnd` (`local.Local_CurrentSplineMesh`) (`local.Local_StartLocation`) (`local.Local_StartTangent`) (`local.Local_EndLocation`) (`local.Local_EndTangent`) true)
      (`SplineMeshComponent.SetStartRoll` (`local.Local_CurrentSplineMesh`) (`local.Local_StartRoll`) true)
      (`SplineMeshComponent.SetEndRoll` (`local.Local_CurrentSplineMesh`) (`local.Local_EndRoll`) true)
      (`SplineMeshComponent.SetStartScale` (`local.Local_CurrentSplineMesh`) (`local.Local_StartScale`) true)
      (`SplineMeshComponent.SetEndScale` (`local.Local_CurrentSplineMesh`) (`local.Local_EndScale`) true)
      (`PrimitiveComponent.SetCollisionEnabled` (`local.Local_CurrentSplineMesh`) (select `bool` (`self.Collisions`) :`false` "NoCollision" :`true` "QueryAndPhysics" :!type "ECollisionEnabled Enum")))))

(fn `UserConstructionScript`
  (bind _rootdataarray (`self.RootDataArray`))
  (`|ExecutionSequence`
    (:`then_0`
      (set `self.Number Of Spline Points` (`SplineComponent.GetNumberOfSplinePoints` (`self.Spline`))))
    (:`then_1`
      (`/Engine/EditorBlueprintResources/StandardMacros.CompareInt` (`KismetArrayLibrary.Array_Length` (`self.RootDataArray`)) (`self.Number Of Spline Points`) :!label _label
        (:`>`
          (`KismetArrayLibrary.Array_Remove` _rootdataarray (`KismetArrayLibrary.Array_LastIndex` _rootdataarray))
          (goto _label))
        (:`<`
          (`KismetArrayLibrary.Array_Add` (`self.RootDataArray`) (`self.RootMeshDefaults`))
          (goto _label))))
    (:`then_2`
      (for _index (range (`self.Number Of Spline Points`))
        (`self.Build Root Element` _index (`self.RootMesh`))))
    (:`then_3`)))