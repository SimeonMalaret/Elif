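; Spawner actor that periodically creates BP_FloatingDraggedActor instances, likely floating platforms for a river.
; Tick drives two chained Delay nodes (Delay, then FireCoolDown), relying on latent retrigger suppression to space out spawns instead of using a timer.
; Each instance spawns at the root component's location and rotation with unit scale, then receives MainRiverManager as its RiverManager.
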(event `self.ReceiveTick`
  (params (DeltaSeconds :type "Float (single-precision)"))
  (bind _defaultsceneroot (`self.DefaultSceneRoot`))
  (`KismetSystemLibrary.Delay` (`self.Delay`))
  (`KismetSystemLibrary.Delay` (`self.FireCoolDown`))
  (bind _returnvalue (`|SpawnActorFromClass` :`Class` "/Game/BP_FloatingDraggedActor.BP_FloatingDraggedActor_C" :`SpawnTransform` (`KismetMathLibrary.MakeTransform` (`SceneComponent.K2_GetComponentLocation` _defaultsceneroot) (`SceneComponent.K2_GetComponentRotation` _defaultsceneroot)) :`CollisionHandlingOverride` "Undefined" :`TransformScaleMethod` "OverrideRootScale" :`Instigator` null))
  (set `/Game/BP_FloatingDraggedActor.RiverManager` (`self.MainRiverManager`) _returnvalue))

(fn `UserConstructionScript`)