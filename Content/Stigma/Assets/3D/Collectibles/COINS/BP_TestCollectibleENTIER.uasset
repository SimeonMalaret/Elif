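; Collectible dog treat pickup that animates its scale and spins from BeginPlay through a timeline.
; When a SecondGameplayCharacter overlaps its Box, it increments that character's dog treat count, updates the treats widget and disables further overlap events.
; The idle timeline then stops and a second timeline spins and shrinks the actor to near zero before destroying it.
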(event `self.ReceiveBeginPlay`
  (bind (_direction _rotate _scale) (`Timeline|Timeline_1` :!label _label)
    (:`Update`
      (`self.SetActorScale3D` (`KismetMathLibrary.VLerp` (`self.LerpScaleStart`) (`self.LerpScableEnd`) _scale))
      (`self.K2_SetActorRotation` (`KismetMathLibrary.RLerp` (struct) (struct :`Yaw` 360.0) _rotate)))))

(event `self.Box.OnComponentBeginOverlap`
  (params (OverlappedComponent :type "PrimitiveComponent Object Reference") (OtherActor :type "Actor Object Reference") (OtherComp :type "PrimitiveComponent Object Reference") (OtherBodyIndex :type Integer) (bFromSweep :type Boolean) (SweepResult :type "HitResult Structure (by ref)"))
  (bind _assecond_gameplay_character (cast `/Game/ThirdPersonCPP/Blueprints/SecondGameplayCharacter` OtherActor))
  (bind _result (`/Engine/EditorBlueprintResources/StandardMacros.IncrementInt` (`/Game/ThirdPersonCPP/Blueprints/SecondGameplayCharacter.NumberDogTreats` _assecond_gameplay_character))
    (:`  `
      (`/Game/Stigma/User_Interface/WBP_NumberTreats.UpdateNumberTreats` (`/Game/ThirdPersonCPP/Blueprints/SecondGameplayCharacter.Widget_Treats` _assecond_gameplay_character) _result)
      (set `PrimitiveComponent.bGenerateOverlapEvents` false (`self.Box`))
      (`|ExecutionSequence`
        (:`then_0`
          (goto _label :!via `Stop`))
        (:`then_1`
          (bind (_direction _scale_2 _rotation_2) (`Timeline|Rotation`)
            (:`Update`
              (`self.SetActorScale3D` (`KismetMathLibrary.VLerp` (`self.LerpScaleStart`) (0.01 0.01 0.01) _scale_2))
              (`self.K2_SetActorRotation` (`KismetMathLibrary.RLerp` (struct) (struct :`Yaw` 360.0) _rotation_2)))
            (:`Finished`
              (`self.K2_DestroyActor`))))))))

(fn `UserConstructionScript`)