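; Test collectible actor that animates in place, then plays a pickup animation and destroys itself when the SecondGameplayCharacter enters its Box.
; Timeline_0 starts on BeginPlay, driving an idle scale pulse and spin, and checks the overlap-set Condition flag on each update.
; Once the flag is set, the Rotation timeline shrinks, spins and raises the actor, with a two-second delay started from its update leading to destruction.
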(event `self.ReceiveBeginPlay`
  (bind (_returnvalue_x _returnvalue_y _returnvalue_z) (`KismetMathLibrary.BreakVector` (`self.K2_GetActorLocation`)))
  (bind (_direction _rotate _scale) (`Timeline|Timeline_0`)
    (:`Update`
      (`self.SetActorScale3D` (`KismetMathLibrary.VLerp` (1.0 1.0 1.0) (0.8 0.8 0.8) _scale))
      (`self.K2_SetActorRotation` (`KismetMathLibrary.RLerp` (struct :`Yaw` 180.0 :`Roll` 90.0) (struct :`Yaw` 360.0 :`Roll` 90.0) _rotate))
      (if (stale `self.Box.OnComponentBeginOverlap` _output_get)
        (bind (_direction_2 _rotate_2 _scale_2 _position) (`Timeline|Rotation`)
          (:`Update`
            (`self.SetActorScale3D` (`KismetMathLibrary.VLerp` (1.0 1.0 1.0) (0.01 0.01 0.01) _scale_2))
            (`self.K2_SetActorRotation` (`KismetMathLibrary.RLerp` (struct :`Yaw` 180.0 :`Roll` 90.0) (struct :`Yaw` 360.0 :`Roll` 90.0) _rotate_2 true))
            (`self.K2_SetActorLocation` (`KismetMathLibrary.MakeVector` _returnvalue_x _returnvalue_y (`KismetMathLibrary.Lerp` _returnvalue_z (+ _returnvalue_z 5.0) _position)))
            (`KismetSystemLibrary.Delay` 2.0)
            (`self.K2_DestroyActor`)))))))

(event `self.Box.OnComponentBeginOverlap`
  (params (OverlappedComponent :type "PrimitiveComponent Object Reference") (OtherActor :type "Actor Object Reference") (OtherComp :type "PrimitiveComponent Object Reference") (OtherBodyIndex :type Integer) (bFromSweep :type Boolean) (SweepResult :type "HitResult Structure (by ref)"))
  (cast `/Game/ThirdPersonCPP/Blueprints/SecondGameplayCharacter` OtherActor)
  (bind _output_get (set `self.Condition` true)))

(fn `UserConstructionScript`)