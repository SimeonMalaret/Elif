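; BP_GamepadPC is a player controller that toggles the game's pause menu.
; On BeginPlay it creates the MenuPAUSE widget and caches the possessed SecondGameplayCharacter.
; The Pause input and the stoppause event share one toggle that sets game pause, shows or removes the widget, and switches input mode and cursor, focusing the Resume button on open.
; Each toggle broadcasts the menu state through OnPause.
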(event `self.ReceiveBeginPlay`
  (bind _returnvalue (`|CreateWidget` "/Game/Stigma/User_Interface/Menu/MenuPAUSE.MenuPAUSE_C"))
  (set `self.Widget Pause` _returnvalue)
  (set `self.PlayerChar` (cast `/Game/ThirdPersonCPP/Blueprints/SecondGameplayCharacter` (`self.K2_GetPawn`) :!pure true)))

(event `InputAction|Pause` :paused true
  (params (Key :type "Key Structure"))
  (bind _widget_pause (`self.Widget Pause`))
  (:`Pressed`
    (`KismetSystemLibrary.PrintString` "Hello")
    (if (`self.isMenuOpen`) :!label _label
      (`GameplayStatics.SetGamePaused` false)
      (`Widget.RemoveFromParent` _widget_pause)
      (set `self.isMenuOpen` false)
      (`WidgetBlueprintLibrary.SetInputMode_GameOnly` self)
      (set `self.bShowMouseCursor` false)
      (`self.OnPause` (`self.isMenuOpen`))
      (else
        (`GameplayStatics.SetGamePaused` true)
        (`UserWidget.AddToViewport` _widget_pause 0)
        (set `self.isMenuOpen` true)
        (`WidgetBlueprintLibrary.SetInputMode_UIOnlyEx` (`GameplayStatics.GetPlayerController` 0) (`/Game/Stigma/User_Interface/Menu/Widgets/Button_Widgets.Button` (`/Game/Stigma/User_Interface/Menu/MenuPAUSE.Button_Widgets_Resume` (`self.Widget Pause`))))
        (set `self.bShowMouseCursor` true)
        (`self.OnPause` (`self.isMenuOpen`))))))

(event `stop pause`
  (goto _label))

(fn `UserConstructionScript`)