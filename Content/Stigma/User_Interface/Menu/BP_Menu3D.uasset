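; BP_Menu3D is a 3D menu actor that hosts a Menu_3DWidgets widget and moves the player's view between linked menu actors.
; On BeginPlay it binds the widget's transition event and disables its own collision.
; A transition index selects an entry in LinkedMenus, then the player controller blends its view target to that actor with easing.
; Collision is off on both menus during the blend and re-enabled on the new one shortly before it ends.
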(event `self.ReceiveBeginPlay`
  (bind _asmenu_3dwidgets (cast `/Game/Stigma/User_Interface/Menu/Widgets/Menu_3DWidgets` (`WidgetComponent.GetUserWidgetObject` (`self.Widget`))))
  (add `/Game/Stigma/User_Interface/Menu/Widgets/Menu_3DWidgets.TransitionToLinkedMenu` _asmenu_3dwidgets (delegate `OnTransitionBetweenMenu`))
  (`self.SetActorEnableCollision` false))

(event `OnTransitionBetweenMenu`
  (params (MenuIndex :type Integer))
  (if (`KismetArrayLibrary.Array_IsValidIndex` (`self.LinkedMenus`) MenuIndex)
    (`self.TransitionTo` (`|GetArrayItem` (`self.LinkedMenus`) MenuIndex))))

(event `TransitionTo`
  (params (`New Menu` :type "/Game/Stigma/User_Interface/Menu/BP_Menu3D Object Reference"))
  (`self.SetActorEnableCollision` false)
  (`self.SetActorEnableCollision` `New Menu` false)
  (`PlayerController.SetViewTargetWithBlend` (`GameplayStatics.GetPlayerController` 0) `New Menu` 2.0 "VTBlend_EaseInOut" 2.0 false)
  (`KismetSystemLibrary.Delay` 1.5)
  (`self.SetActorEnableCollision` `New Menu` true))

(fn `UserConstructionScript`)