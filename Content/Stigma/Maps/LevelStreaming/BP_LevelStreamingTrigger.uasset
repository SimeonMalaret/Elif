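; BP_LevelStreamingTrigger is a trigger actor that streams sublevels in and out as the player character passes through it.
; On overlap with a SecondGameplayCharacter, it loads the level named in LevelToLoad and makes it visible, then unloads the one named in LevelToUnload, skipping either step when the name is None.
; Both the load and the unload block until they finish.
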(event `self.ReceiveActorBeginOverlap`
  (params (OtherActor :type "Actor Object Reference"))
  (cast `/Game/ThirdPersonCPP/Blueprints/SecondGameplayCharacter` OtherActor)
  (if (!= (`self.LevelToLoad`) "None")
    (`GameplayStatics.LoadStreamLevel` (`self.LevelToLoad`) true true))
  (if (!= (`self.LevelToUnload`) "None")
    (`GameplayStatics.UnloadStreamLevel` (`self.LevelToUnload`) true)))

(fn `UserConstructionScript`)