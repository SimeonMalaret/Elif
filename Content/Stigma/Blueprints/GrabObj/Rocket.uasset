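; Rocket is a grabbable-object Blueprint that gives the player a forward boost dash.
; BoostDash, gated by CanDash, launches the player along their forward vector, switches post-process profile, disables input and zeroes braking friction.
; ResetDash restores input, friction and the default profile and clears the dash flags on player and rocket, but does not re-arm CanDash.
; Neither function is called within this graph.
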(event `self.ReceiveBeginPlay`
  (`parent.ReceiveBeginPlay`))

(event `self.ReceiveTick`
  (params (DeltaSeconds :type "Float (single-precision)")))

(fn `BoostDash`
  (params (Actor :type "/Game/ThirdPersonCPP/Blueprints/SecondGameplayCharacter Object Reference"))
  (if (`self.CanDash`)
    (bind _output_get (set `self.Player` Actor))
    (`/Game/ThirdPersonCPP/Blueprints/SecondGameplayCharacter.SwitchProfilePP` _output_get (`|GetArrayItem` (`/Game/ThirdPersonCPP/Blueprints/SecondGameplayCharacter.ProfilesPP` _output_get) 1))
    (set `/Game/ThirdPersonCPP/Blueprints/SecondGameplayCharacter.IsInDash` true _output_get)
    (`self.DisableInput` _output_get (`GameplayStatics.GetPlayerControllerFromID` 0))
    (`Character.LaunchCharacter` _output_get (* (`self.GetActorForwardVector` _output_get) (`self.DashPower`)) false false)
    (set `CharacterMovementComponent.BrakingFrictionFactor` 0.0 (`Character.CharacterMovement` _output_get))
    (set `self.CanDash` false)
    (set `self.Dashing` true))
  (return))

(fn `ResetDash`
  (params (Actor :type "/Game/ThirdPersonCPP/Blueprints/SecondGameplayCharacter Object Reference"))
  (bind _output_get (set `self.Player` Actor))
  (set `/Game/ThirdPersonCPP/Blueprints/SecondGameplayCharacter.IsInDash` false _output_get)
  (set `CharacterMovementComponent.BrakingFrictionFactor` 2.0 (`Character.CharacterMovement` _output_get))
  (`self.EnableInput` _output_get (`GameplayStatics.GetPlayerControllerFromID` 0))
  (`/Game/ThirdPersonCPP/Blueprints/SecondGameplayCharacter.SwitchProfilePP` _output_get (`|GetArrayItem` (`/Game/ThirdPersonCPP/Blueprints/SecondGameplayCharacter.ProfilesPP` _output_get)))
  (set `self.Dashing` false)
  (return))

(fn `UserConstructionScript`
  (`parent.UserConstructionScript`))