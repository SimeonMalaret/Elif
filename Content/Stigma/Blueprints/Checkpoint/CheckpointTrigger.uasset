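; Checkpoint trigger volume that saves the player's respawn point when a SecondGameplayCharacter overlaps it, then stops generating overlaps so it fires only once.
; It records the checkpoint's location as the start point, plus the current camera and, for CameraRail cameras, its distance to the player.
; It then activates its assigned DeadZones and sends a checkpoint reset message to every actor implementing CamTriggerInterface.
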(event `self.TriggerCP.OnComponentBeginOverlap`
  (params (OverlappedComponent :type "PrimitiveComponent Object Reference") (OtherActor :type "Actor Object Reference") (OtherComp :type "PrimitiveComponent Object Reference") (OtherBodyIndex :type Integer) (bFromSweep :type Boolean) (SweepResult :type "HitResult Structure (by ref)"))
  (bind _assecond_gameplay_character (cast `/Game/ThirdPersonCPP/Blueprints/SecondGameplayCharacter` OtherActor))
  (set `/Game/ThirdPersonCPP/Blueprints/SecondGameplayCharacter.StartPoint` (`self.K2_GetActorLocation`) _assecond_gameplay_character)
  (set `PrimitiveComponent.bGenerateOverlapEvents` false (`self.TriggerCP`))
  (`|ExecutionSequence`
    (:`then_0`
      (bind _output_get (set `/Game/ThirdPersonCPP/Blueprints/SecondGameplayCharacter.LastCheckPointCamera` (`/Game/ThirdPersonCPP/Blueprints/SecondGameplayCharacter.CurrentCamera` _assecond_gameplay_character) _assecond_gameplay_character))
      (bind _ascamera_rail (cast `/Game/ThirdPersonCPP/Blueprints/Francois/CameraRail` _output_get))
      (set `/Game/ThirdPersonCPP/Blueprints/SecondGameplayCharacter.LastCheckpointDistance` (`/Game/ThirdPersonCPP/Blueprints/Francois/CameraRail.DistanceToPlayer` _ascamera_rail) _assecond_gameplay_character))
    (:`then_1`
      (for _array_element (`self.DeadZones To Activate`)
        (set `/Game/Stigma/Blueprints/Checkpoint/DeathZone.IsActive` true _array_element)))
    (:`then_2`
      (bind _outactors (`GameplayStatics.GetAllActorsWithInterface` "/Game/Stigma/Blueprints/Camera/CamTriggerInterface.CamTriggerInterface_C"))
      (for _array_element_2 _outactors
        (message `/Game/Stigma/Blueprints/Camera/CamTriggerInterface.CheckPointReset` _array_element_2)))))

(fn `UserConstructionScript`)