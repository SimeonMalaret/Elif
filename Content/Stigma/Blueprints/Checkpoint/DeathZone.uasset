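; DeathZone is a kill volume that sends the player character back through its ResetPosition when overlapped.
; While active, its Death component's overlap with a SecondGameplayCharacter spawns a particle burst and force feedback, hides the mesh and disables input before calling the reset.
; On the first death recorded in Camille_GM, it clears that flag and starts a narration line through the game mode's NarrationManager.
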(event `self.Death.OnComponentBeginOverlap`
  (params (OverlappedComponent :type "PrimitiveComponent Object Reference") (OtherActor :type "Actor Object Reference") (OtherComp :type "PrimitiveComponent Object Reference") (OtherBodyIndex :type Integer) (bFromSweep :type Boolean) (SweepResult :type "HitResult Structure (by ref)"))
  ;[1 1 1] DeadZone (Toggle Character visibility)
  (if (`self.IsActive`)
    (bind _assecond_gameplay_character (cast `/Game/ThirdPersonCPP/Blueprints/SecondGameplayCharacter` OtherActor))
    (`GameplayStatics.SpawnEmitterAtLocation` "/Game/Stigma/FX/Particules/Elif_Spawn/P_Elif_Spawn.P_Elif_Spawn" (`.Location` (`GameplayStatics.BreakHitResult` SweepResult)) (struct) (3.0 3.0 3.0))
    (`GameplayStatics.SpawnForceFeedbackAtLocation` "/Game/Stigma/Feedback/Death.Death" (`self.K2_GetActorLocation` _assecond_gameplay_character) (struct) false 1.0 0.0 null)
    (`SceneComponent.SetVisibility` (`Character.Mesh` _assecond_gameplay_character) false true)
    (`self.DisableInput` _assecond_gameplay_character (`GameplayStatics.GetPlayerController` 0))
    (if (`KismetSystemLibrary.IsValid` _assecond_gameplay_character)
      (`/Game/ThirdPersonCPP/Blueprints/SecondGameplayCharacter.ResetPosition` _assecond_gameplay_character)
      (bind _ascamille_gm (cast `/Game/Stigma/Blueprints/Camille_GM` (`GameplayStatics.GetGameMode`)))
      (if (`/Game/Stigma/Blueprints/Camille_GM.FirstTimeDeath` _ascamille_gm)
        (set `/Game/Stigma/Blueprints/Camille_GM.FirstTimeDeath` false _ascamille_gm)
        (bind _narrationmanager (`/Game/Stigma/Blueprints/Camille_GM.NarrationManager` _ascamille_gm)
          (:`then`
            (`/Game/Stigma/Blueprints/Narration/NarrationManager.StartNarration` _narrationmanager (`self.Index To Play`) null null))
          (:`else`))))))

(fn `UserConstructionScript`)