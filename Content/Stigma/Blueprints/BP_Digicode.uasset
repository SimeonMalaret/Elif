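; BP_Digicode is a code puzzle that is solved when four switched buttons all carry the "true" event name.
; It listens to button activation and deactivation events on Camille_GM, then recounts switched true and false buttons whenever a matching event fires.
; At four switched, after a short delay, it either force-validates and stops every button or resets them all.
; Cables light progressively with the switched count, whether correct or not.
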(event `self.ReceiveBeginPlay`
  (bind _ascamille_gm (cast `/Game/Stigma/Blueprints/Camille_GM` (`GameplayStatics.GetGameMode`) :!pure true))
  (add `/Game/Stigma/Blueprints/Camille_GM.ActivationByButton` _ascamille_gm (delegate `CustomEvent_0`))
  (add `/Game/Stigma/Blueprints/Camille_GM.UnactivationByButton` _ascamille_gm (delegate `CustomEvent_0`)))

(event `CustomEvent_0`
  (params (eventName :type "Array of String (by ref)"))
  (bind _cables (`self.Cables`))
  (bind _returnvalue (+ (`self.nbButtonTrueOn`) (`self.nbButtonFalseOn`)))
  (bind _output (`|GetArrayItem` _cables 1))
  (bind _output_2 (`|GetArrayItem` _cables))
  (if (`KismetArrayLibrary.Array_Contains` eventName (`self.eventNameTrue`))
    (set `self.nbButtonTrueOn` 0 :!label _label)
    (set `self.nbButtonFalseOn` 0)
    (for _array_element (`self.buttons`)
      (if (`/Game/Stigma/Blueprints/BP_Button_SwitchWithCancel.isSwitched` _array_element)
        (if (`KismetArrayLibrary.Array_Contains` (`/Game/Stigma/Blueprints/BP_Button_SwitchWithCancel.eventNameToActive` _array_element) (`self.eventNameTrue`))
          (`/Engine/EditorBlueprintResources/StandardMacros.IncrementInt` (`self.nbButtonTrueOn`))
          (elif (`KismetArrayLibrary.Array_Contains` (`/Game/Stigma/Blueprints/BP_Button_SwitchWithCancel.eventNameToActive` _array_element) (`self.eventNameFalse`))
            (`/Engine/EditorBlueprintResources/StandardMacros.IncrementInt` (`self.nbButtonFalseOn`))))))
    (if (== _returnvalue 4)
      (if (== (`self.nbButtonTrueOn`) 4)
        (`KismetSystemLibrary.Delay` 0.2)
        (for _array_element_2 (`self.buttons`)
          (`/Game/Stigma/Blueprints/BP_Button_SwitchWithCancel.ForceValidateAndStop` _array_element_2)
          (message `/Game/Stigma/Blueprints/Cables/ColorCableInterface.DeactivationColor` _cables :!label _label_2)
          (switch `int` _returnvalue
            (:`1`
              (message `/Game/Stigma/Blueprints/Cables/ColorCableInterface.ActivationColor` _output_2))
            (:`2`
              (message `/Game/Stigma/Blueprints/Cables/ColorCableInterface.ActivationColor` (`|MakeArray` _output_2 _output :!type "Object Object Reference")))
            (:`3`
              (message `/Game/Stigma/Blueprints/Cables/ColorCableInterface.ActivationColor` (`|MakeArray` _output_2 _output (`|GetArrayItem` _cables 2) :!type "Object Object Reference")))
            (:`4`
              (message `/Game/Stigma/Blueprints/Cables/ColorCableInterface.ActivationColor` _cables))))
        (else
          (`KismetSystemLibrary.Delay` 0.2)
          (for _array_element_3 (`self.buttons`)
            (`/Game/Stigma/Blueprints/BP_Button_SwitchWithCancel.Reset` _array_element_3)
            (set `self.nbButtonTrueOn` 0)
            (set `self.nbButtonFalseOn` 0)
            (goto _label_2))))
      (else
        (goto _label_2)))
    (elif (`KismetArrayLibrary.Array_Contains` eventName (`self.eventNameFalse`))
      (goto _label))))

(fn `UserConstructionScript`)