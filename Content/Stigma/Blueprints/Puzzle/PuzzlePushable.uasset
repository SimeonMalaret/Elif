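; Puzzle box that the player pushes onto a designated PuzzlePushTarget, where it locks in place.
; Interaction is handled only while unlocked; overlapping the matching target ends the push, records the start position, sets the lock and notifies the parent puzzle.
; While locked, Tick lerps the box to the target's location, using Speed as the snap duration in seconds.
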(event `self.ReceiveTick`
  (params (DeltaSeconds :type "Float (single-precision)"))
  (bind _elapsed_time (`self.Elapsed Time`))
  (bind _speed (`self.Speed`))
  (if (`self.IsLocked`)
    (set `self.Elapsed Time` (+ (`self.Elapsed Time`) DeltaSeconds))
    (if (< _elapsed_time _speed)
      (`SceneComponent.K2_SetWorldLocation` (`self.Box`) (`KismetMathLibrary.VLerp` (`self.Start Lock Pos`) (`self.K2_GetActorLocation` (`self.Target`)) (/ _elapsed_time _speed)) false false))))

(event `/Game/Stigma/Blueprints/PushObjects/InteractInterface.OnInteracted`
  (params (Player :type "/Game/ThirdPersonCPP/Blueprints/SecondGameplayCharacter Object Reference"))
  (if (not (`self.IsLocked`))
    (`self.HandleInteraction` Player)))

(event `self.Box.OnComponentBeginOverlap`
  (params (OverlappedComponent :type "PrimitiveComponent Object Reference") (OtherActor :type "Actor Object Reference") (OtherComp :type "PrimitiveComponent Object Reference") (OtherBodyIndex :type Integer) (bFromSweep :type Boolean) (SweepResult :type "HitResult Structure (by ref)"))
  (bind _aspuzzle_push_target (cast `/Game/Stigma/Blueprints/Puzzle/PuzzlePushTarget` OtherActor))
  (if (and (== _aspuzzle_push_target (`self.Target`)) (not (`self.IsLocked`)))
    (`/Game/Stigma/Blueprints/PushObjects/PushComponent.EndPush` (`self.PushComponent`))
    (set `self.Start Lock Pos` (`SceneComponent.K2_GetComponentLocation` (`self.Box`)))
    (set `self.IsLocked` true)
    (`/Game/Stigma/Blueprints/Puzzle/PuzzlePush.OnPushableLock` (`self.PuzzleParent`))))

(fn `UserConstructionScript`
  (`parent.UserConstructionScript`))