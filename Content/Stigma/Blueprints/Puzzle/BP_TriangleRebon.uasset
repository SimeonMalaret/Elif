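; BP_TriangleRebon is a puzzle piece that deflects a moving BP_PuzzlCube.
; Entering Dir1 or Dir2 sends the cube from the piece's center toward the other side via SetNextDir, with a one-second lockout against retriggering.
; A cube touching either wall resets the owning Puzzle.
; A dashing SecondGameplayCharacter hitting its cube components spawns an explosion and teleports the piece below the puzzle instead of destroying it.
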(event `self.ReceiveBeginPlay`)

(event `self.dir1.OnComponentBeginOverlap`
  (params (OverlappedComponent :type "PrimitiveComponent Object Reference") (OtherActor :type "Actor Object Reference") (OtherComp :type "PrimitiveComponent Object Reference") (OtherBodyIndex :type Integer) (bFromSweep :type Boolean) (SweepResult :type "HitResult Structure (by ref)"))
  (bind (_returnvalue_x _returnvalue_y) (`KismetMathLibrary.BreakVector` (- (`SceneComponent.K2_GetComponentLocation` (`self.dir2`)) (`SceneComponent.K2_GetComponentLocation` (`self.3DObj`)))))
  (if (`self.passOne`)
    (bind _asbp_puzzl_cube (cast `/Game/Stigma/Blueprints/Puzzle/BP_PuzzlCube` OtherActor))
    (`/Game/Stigma/Blueprints/Puzzle/BP_PuzzlCube.SetNextDir` _asbp_puzzl_cube (`KismetMathLibrary.Normal` (`KismetMathLibrary.MakeVector` _returnvalue_x _returnvalue_y)) (`SceneComponent.K2_GetComponentLocation` (`self.3DObj`)))
    (set `self.passOne` false)
    (`KismetSystemLibrary.Delay` 1.0)
    (set `self.passOne` true)))

(event `self.dir2.OnComponentBeginOverlap`
  (params (OverlappedComponent :type "PrimitiveComponent Object Reference") (OtherActor :type "Actor Object Reference") (OtherComp :type "PrimitiveComponent Object Reference") (OtherBodyIndex :type Integer) (bFromSweep :type Boolean) (SweepResult :type "HitResult Structure (by ref)"))
  (bind (_returnvalue_x _returnvalue_y) (`KismetMathLibrary.BreakVector` (- (`SceneComponent.K2_GetComponentLocation` (`self.dir1`)) (`SceneComponent.K2_GetComponentLocation` (`self.3DObj`)))))
  (if (`self.passOne`)
    (bind _asbp_puzzl_cube (cast `/Game/Stigma/Blueprints/Puzzle/BP_PuzzlCube` OtherActor))
    (`/Game/Stigma/Blueprints/Puzzle/BP_PuzzlCube.SetNextDir` _asbp_puzzl_cube (`KismetMathLibrary.Normal` (`KismetMathLibrary.MakeVector` _returnvalue_x _returnvalue_y)) (`SceneComponent.K2_GetComponentLocation` (`self.3DObj`)))
    (set `self.passOne` false)
    (`KismetSystemLibrary.Delay` 1.0)
    (set `self.passOne` true)))

(event `self.Wall1.OnComponentBeginOverlap`
  (params (OverlappedComponent :type "PrimitiveComponent Object Reference") (OtherActor :type "Actor Object Reference") (OtherComp :type "PrimitiveComponent Object Reference") (OtherBodyIndex :type Integer) (bFromSweep :type Boolean) (SweepResult :type "HitResult Structure (by ref)"))
  (cast `/Game/Stigma/Blueprints/Puzzle/BP_PuzzlCube` OtherActor)
  (`/Game/Stigma/Blueprints/Puzzle/Puzzle.ResetPuzzle` (`self.puzzle`) :!label _label))

(event `self.Wall2.OnComponentBeginOverlap`
  (params (OverlappedComponent :type "PrimitiveComponent Object Reference") (OtherActor :type "Actor Object Reference") (OtherComp :type "PrimitiveComponent Object Reference") (OtherBodyIndex :type Integer) (bFromSweep :type Boolean) (SweepResult :type "HitResult Structure (by ref)"))
  (cast `/Game/Stigma/Blueprints/Puzzle/BP_PuzzlCube` OtherActor)
  (goto _label))

(event `self.Cube1.OnComponentHit`
  (params (HitComponent :type "PrimitiveComponent Object Reference") (OtherActor :type "Actor Object Reference") (OtherComp :type "PrimitiveComponent Object Reference") (NormalImpulse :type "Vector Structure") (Hit :type "HitResult Structure (by ref)"))
  (bind _assecond_gameplay_character (cast `/Game/ThirdPersonCPP/Blueprints/SecondGameplayCharacter` OtherActor))
  (if (`/Game/ThirdPersonCPP/Blueprints/SecondGameplayCharacter.IsInDash` _assecond_gameplay_character)
    (`|SpawnActorFromClass` "/Game/StarterContent/Blueprints/Blueprint_Effect_Explosion.Blueprint_Effect_Explosion_C" (`self.GetTransform`) "Undefined" "OverrideRootScale" null null :!label _label_2)
    (`self.K2_SetActorLocation` (+ (`self.K2_GetActorLocation` (`self.puzzle`)) (0.0 0.0 -1000.0)) false true)))

(event `self.Cube2.OnComponentHit`
  (params (HitComponent :type "PrimitiveComponent Object Reference") (OtherActor :type "Actor Object Reference") (OtherComp :type "PrimitiveComponent Object Reference") (NormalImpulse :type "Vector Structure") (Hit :type "HitResult Structure (by ref)"))
  (bind _assecond_gameplay_character (cast `/Game/ThirdPersonCPP/Blueprints/SecondGameplayCharacter` OtherActor))
  (if (`/Game/ThirdPersonCPP/Blueprints/SecondGameplayCharacter.IsInDash` _assecond_gameplay_character)
    (goto _label_2)))

(event `self.Cube.OnComponentHit`
  (params (HitComponent :type "PrimitiveComponent Object Reference") (OtherActor :type "Actor Object Reference") (OtherComp :type "PrimitiveComponent Object Reference") (NormalImpulse :type "Vector Structure") (Hit :type "HitResult Structure (by ref)"))
  (bind _assecond_gameplay_character (cast `/Game/ThirdPersonCPP/Blueprints/SecondGameplayCharacter` OtherActor))
  (if (`/Game/ThirdPersonCPP/Blueprints/SecondGameplayCharacter.IsInDash` _assecond_gameplay_character)
    (goto _label_2)))

(fn `UserConstructionScript`)