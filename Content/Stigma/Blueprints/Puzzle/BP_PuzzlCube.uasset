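; Puzzle cube that slides in a straight line when the player dashes into one of its four faces.
; Tick moves it with a swept offset; SetNextDir queues a turn, applied by snapping to the switch point once distance to it starts increasing.
; Non-player face overlaps go to HitOther: a BP_CiblePuzzle target spawns an explosion and ends the Puzzle, while anything not tagged IgnorePuzzle resets it.
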(event `self.Face_0.OnComponentBeginOverlap`
  (params (OverlappedComponent :type "PrimitiveComponent Object Reference") (OtherActor :type "Actor Object Reference") (OtherComp :type "PrimitiveComponent Object Reference") (OtherBodyIndex :type Integer) (bFromSweep :type Boolean) (SweepResult :type "HitResult Structure (by ref)"))
  (bind _assecond_gameplay_character (cast `/Game/ThirdPersonCPP/Blueprints/SecondGameplayCharacter` OtherActor)
    (:`then`
      (if (and (`/Game/ThirdPersonCPP/Blueprints/SecondGameplayCharacter.IsInDash` _assecond_gameplay_character) (not (`self.isMoving`)))
        (set `self.direction` (-1.0 0.0 0.0))
        (set `self.isMoving` true :!label _label)))
    (:`CastFailed`
      (`self.HitOther` OtherActor))))

(event `self.Face_1.OnComponentBeginOverlap`
  (params (OverlappedComponent :type "PrimitiveComponent Object Reference") (OtherActor :type "Actor Object Reference") (OtherComp :type "PrimitiveComponent Object Reference") (OtherBodyIndex :type Integer) (bFromSweep :type Boolean) (SweepResult :type "HitResult Structure (by ref)"))
  (bind _assecond_gameplay_character (cast `/Game/ThirdPersonCPP/Blueprints/SecondGameplayCharacter` OtherActor)
    (:`then`
      (if (and (`/Game/ThirdPersonCPP/Blueprints/SecondGameplayCharacter.IsInDash` _assecond_gameplay_character) (not (`self.isMoving`)))
        (set `self.direction` (1.0 0.0 0.0))
        (goto _label)))
    (:`CastFailed`
      (`self.HitOther` OtherActor))))

(event `self.Face_2.OnComponentBeginOverlap`
  (params (OverlappedComponent :type "PrimitiveComponent Object Reference") (OtherActor :type "Actor Object Reference") (OtherComp :type "PrimitiveComponent Object Reference") (OtherBodyIndex :type Integer) (bFromSweep :type Boolean) (SweepResult :type "HitResult Structure (by ref)"))
  (bind _assecond_gameplay_character (cast `/Game/ThirdPersonCPP/Blueprints/SecondGameplayCharacter` OtherActor)
    (:`then`
      (if (and (`/Game/ThirdPersonCPP/Blueprints/SecondGameplayCharacter.IsInDash` _assecond_gameplay_character) (not (`self.isMoving`)))
        (set `self.direction` (0.0 -1.0 0.0))
        (goto _label)))
    (:`CastFailed`
      (`self.HitOther` OtherActor))))

(event `self.Face_3.OnComponentBeginOverlap`
  (params (OverlappedComponent :type "PrimitiveComponent Object Reference") (OtherActor :type "Actor Object Reference") (OtherComp :type "PrimitiveComponent Object Reference") (OtherBodyIndex :type Integer) (bFromSweep :type Boolean) (SweepResult :type "HitResult Structure (by ref)"))
  (bind _assecond_gameplay_character (cast `/Game/ThirdPersonCPP/Blueprints/SecondGameplayCharacter` OtherActor)
    (:`then`
      (if (and (`/Game/ThirdPersonCPP/Blueprints/SecondGameplayCharacter.IsInDash` _assecond_gameplay_character) (not (`self.isMoving`)))
        (set `self.direction` (0.0 1.0 0.0))
        (goto _label)))
    (:`CastFailed`
      (`self.HitOther` OtherActor))))

(event `self.ReceiveTick`
  (params (DeltaSeconds :type "Float (single-precision)"))
  (bind _returnvalue (`KismetMathLibrary.Vector_Distance` (`self.PosNextChange`) (`self.K2_GetActorLocation`)))
  (if (`self.isMoving`)
    (`self.K2_SetActorLocation` (+ (* (* (`self.direction`) DeltaSeconds) (`self.speed`)) (`self.K2_GetActorLocation`)) true)
    (if (`self.isNextPosSet`)
      (if (< (`self.tmpDist`) _returnvalue)
        (set `self.isNextPosSet` false)
        (set `self.direction` (`self.NextDir`))
        (`self.K2_SetActorLocation` (`self.PosNextChange`) false true)
        (else
          (set `self.tmpDist` _returnvalue))))))

(event `SetNextDir`
  (params (Direction :type "Vector Structure") (PositionOfSwitchDir :type "Vector Structure"))
  (bind (_returnvalue_x _returnvalue_y _returnvalue_z) (`KismetMathLibrary.BreakVector` (`self.K2_GetActorLocation`)))
  (set `self.NextDir` Direction)
  (set `self.PosNextChange` (`KismetMathLibrary.MakeVector` PositionOfSwitchDir_X PositionOfSwitchDir_Y _returnvalue_z))
  (set `self.tmpDist` 10000000.0)
  (set `self.isNextPosSet` true))

(fn `HitOther`
  (params (OtherActor :type "Actor Object Reference"))
  (cast `/Game/Stigma/Blueprints/Puzzle/BP_CiblePuzzle` OtherActor
    (:`then`
      (`|SpawnActorFromClass` "/Game/StarterContent/Blueprints/Blueprint_Effect_Explosion.Blueprint_Effect_Explosion_C" (`self.GetTransform`) "Undefined" "OverrideRootScale" null null)
      (`/Game/Stigma/Blueprints/Puzzle/Puzzle.EndPuzzle` (`self.puzzle`)))
    (:`CastFailed`
      (if (not (`self.ActorHasTag` OtherActor "IgnorePuzzle"))
        (`KismetSystemLibrary.PrintString` "RESET")
        (`/Game/Stigma/Blueprints/Puzzle/Puzzle.ResetPuzzle` (`self.puzzle`))))))

(fn `UserConstructionScript`)