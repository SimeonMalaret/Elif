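; PuzzlePush is a puzzle controller that completes when every linked pushable is locked, opening its target bridges.
; It registers itself as PuzzleParent on each pushable at BeginPlay and rechecks all lock states in OnPushableLock.
; On completion it starts DrawBridge_Crocodile targets, then passes the parsed EventName to STIGMA_GM's CallActivationByButton behind a DrawBridge_Lego cast.
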(event `OnPushableLock`
  (for _array_element (`self.Pushables`)
    (if (not (`/Game/Stigma/Blueprints/Puzzle/PuzzlePushable.IsLocked` _array_element))
      (set `self.IsAllDone` false)
      (break)
      (else
        (set `self.IsAllDone` true))))
  (if (`self.IsAllDone`)
    (`self.OnCompleted`)))

(event `self.ReceiveBeginPlay`
  (for _array_element (`self.Pushables`)
    (set `/Game/Stigma/Blueprints/Puzzle/PuzzlePushable.PuzzleParent` self _array_element)))

(event `OnCompleted`
  (for _array_element (`self.TargetToOpen`)
    (bind _asdraw_bridge_crocodile (cast `/Game/Stigma/Blueprints/DrawBridge/DrawBridge_Crocodile` _array_element))
    (`/Game/Stigma/Blueprints/DrawBridge/DrawBridge_Crocodile.StartOpenBridge` _asdraw_bridge_crocodile))
  (cast `/Game/Stigma/Blueprints/DrawBridge/DrawBridge_Lego` _array_element)
  (`/Game/Stigma/Blueprints/STIGMA_GM.ActivationByButton` (cast `/Game/Stigma/Blueprints/STIGMA_GM` (`GameplayStatics.GetGameMode`) :!pure true) (`KismetStringLibrary.ParseIntoArray` (`self.EventName`))))

(fn `UserConstructionScript`)