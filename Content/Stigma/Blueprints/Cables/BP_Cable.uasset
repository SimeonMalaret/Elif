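; BP_Cable is a cable Blueprint whose color shows whether it is powered, optionally passing energy to a linked Activator.
; On BeginPlay it creates a dynamic instance of its second material and caches the original color.
; Activate and deactivate events play or reverse a timeline that blends toward NewColor.
; With a valid Activator they also add or remove energy, with a flag preventing repeated additions.
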(event `self.ReceiveBeginPlay`
  (bind _staticmeshcomponent (`self.StaticMeshComponent`))
  (bind _returnvalue (`PrimitiveComponent.CreateDynamicMaterialInstance` _staticmeshcomponent 1 (`|GetArrayItem` (`MeshComponent.GetMaterials` _staticmeshcomponent) 1) "None"))
  (bind _output_get (set `self.TempMat` _returnvalue))
  (bind _returnvalue_2 (`MaterialInstanceDynamic.K2_GetVectorParameterValue` _output_get "Color"))
  (set `self.OldColor` _returnvalue_2))

(event `SetActiveColor`
  (bind (_newcolor_r _newcolor_g _newcolor_b _newcolor_a) (break `LinearColor` (`self.NewColor`)))
  (set `self.NewColor` (make `LinearColor` _newcolor_r _newcolor_g _newcolor_b _newcolor_a))
  (bind _activator (`self.Activator`)
    (:`then`
      (if (not (`self.energieOn`))
        (set `self.energieOn` true)
        (`/Game/Stigma/Blueprints/Cables/BP_MultiCableAtivator.AddEnergie` _activator)
        (bind (_direction _blend) (`Timeline|LerpColor` :!label _label)
          (:`Update`
            (`MaterialInstanceDynamic.SetVectorParameterValue` (`self.TempMat`) "Color" (`KismetMathLibrary.LinearColorLerp` (`self.OldColor`) (`self.NewColor`) _blend))))))
    (:`else`
      (goto _label))))

(event `SetInactiveColor`
  (bind _activator (`self.Activator`)
    (:`then`
      (set `self.energieOn` false)
      (`/Game/Stigma/Blueprints/Cables/BP_MultiCableAtivator.RemoveEnergie` _activator)
      (goto _label :!via `Reverse`))
    (:`else`
      (goto _label :!via `Reverse`))))

(event `SetActivator`
  (params (NewParam :type "/Game/Stigma/Blueprints/Cables/BP_MultiCableAtivator Object Reference"))
  (set `self.Activator` NewParam))

(fn `UserConstructionScript`)