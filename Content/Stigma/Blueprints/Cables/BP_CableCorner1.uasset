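; BP_CableCorner1 is a corner cable piece that changes color when energized and passes energy to a linked activator.
; On BeginPlay it creates a dynamic material from mesh slot 1 and caches its starting Color.
; SetActiveColor adds energy to the Activator, if valid, and plays a timeline blending to NewColor.
; SetInactiveColor removes that energy and reverses the blend, while SetActivator assigns the linked Activator.
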(event `self.ReceiveBeginPlay`
  (bind _staticmesh (`self.StaticMesh`))
  (bind _returnvalue (`PrimitiveComponent.CreateDynamicMaterialInstance` _staticmesh 1 (`|GetArrayItem` (`MeshComponent.GetMaterials` _staticmesh) 1) "None"))
  (bind _output_get (set `self.TempMat` _returnvalue))
  (bind _returnvalue_2 (`MaterialInstanceDynamic.K2_GetVectorParameterValue` _output_get "Color"))
  (set `self.OldColor` _returnvalue_2))

(event `SetActiveColor`
  (bind (_newcolor_r _newcolor_g _newcolor_b _newcolor_a) (break `LinearColor` (`self.NewColor`)))
  (set `self.NewColor` (make `LinearColor` _newcolor_r _newcolor_g _newcolor_b _newcolor_a))
  (bind _activator (`self.Activator`)
    (:`then`
      (`/Game/Stigma/Blueprints/Cables/BP_MultiCableAtivator.AddEnergie` _activator)
      (bind (_direction _blend) (`Timeline|Timeline_0` :!label _label)
        (:`Update`
          (`MaterialInstanceDynamic.SetVectorParameterValue` (`self.TempMat`) "Color" (`KismetMathLibrary.LinearColorLerp` (`self.OldColor`) (`self.NewColor`) _blend)))))
    (:`else`
      (goto _label))))

(event `SetInactiveColor`
  (bind _activator (`self.Activator`)
    (:`then`
      (`/Game/Stigma/Blueprints/Cables/BP_MultiCableAtivator.RemoveEnergie` _activator)
      (goto _label :!via `Reverse`))
    (:`else`
      (goto _label :!via `Reverse`))))

(event `SetActivator`
  (params (NewParam :type "/Game/Stigma/Blueprints/Cables/BP_MultiCableAtivator Object Reference"))
  (set `self.Activator` NewParam))

(fn `UserConstructionScript`)