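; BP_MultiCableAtivator is a cable puzzle junction that activates once all its input cables supply energy.
; On BeginPlay it registers itself as activator on the Input cables, then counts AddEnergie and RemoveEnergie calls.
; When the count reaches the Input total, a one-time latch sends activation color messages to Input and Output and sets FixEnnergie on their straight and corner cables, so later removal cannot undo activation.
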(event `self.ReceiveBeginPlay`
  (message `/Game/Stigma/Blueprints/Cables/ColorCableInterface.SetActivator` (`self.input`) self))

(event `AddEnergie`
  (bind _input (`self.input`))
  (bind _nbcablein (`self.nbCableIn`))
  (bind _output (`self.output`))
  (`/Engine/EditorBlueprintResources/StandardMacros.IncrementInt` _nbcablein
    (:`  `
      (if (>= _nbcablein (`KismetArrayLibrary.Array_Length` (`self.input`)))
        (if (not (`self.isfinish`))
          (set `self.isfinish` true)
          (message `/Game/Stigma/Blueprints/Cables/ColorCableInterface.ActivationColor` _input)
          (for _array_element _input
            (bind _asbp_cable (cast `/Game/Stigma/Blueprints/Cables/BP_Cable` _array_element)
              (:`then`
                (set `/Game/Stigma/Blueprints/Cables/BP_Cable.fix ennergie` true _asbp_cable))
              (:`CastFailed`
                (bind _asbp_cable_corner (cast `/Game/Stigma/Blueprints/Cables/BP_CableCorner` _array_element)
                  (:`then`
                    (set `/Game/Stigma/Blueprints/Cables/BP_CableCorner.fix ennergie` true _asbp_cable_corner))
                  (:`CastFailed`
                    (bind _asbp_cable_corner_1 (cast `/Game/Stigma/Blueprints/Cables/BP_CableCorner1` _array_element))
                    (set `/Game/Stigma/Blueprints/Cables/BP_CableCorner1.fix ennergie` true _asbp_cable_corner_1))))))
          (message `/Game/Stigma/Blueprints/Cables/ColorCableInterface.ActivationColor` _output)
          (for _array_element_2 _output
            (bind _asbp_cable_2 (cast `/Game/Stigma/Blueprints/Cables/BP_Cable` _array_element_2)
              (:`then`
                (set `/Game/Stigma/Blueprints/Cables/BP_Cable.fix ennergie` true _asbp_cable_2))
              (:`CastFailed`
                (bind _asbp_cable_corner_2 (cast `/Game/Stigma/Blueprints/Cables/BP_CableCorner` _array_element_2)
                  (:`then`
                    (set `/Game/Stigma/Blueprints/Cables/BP_CableCorner.fix ennergie` true _asbp_cable_corner_2))
                  (:`CastFailed`
                    (bind _asbp_cable_corner_1_2 (cast `/Game/Stigma/Blueprints/Cables/BP_CableCorner1` _array_element_2))
                    (set `/Game/Stigma/Blueprints/Cables/BP_CableCorner1.fix ennergie` true _asbp_cable_corner_1_2)))))))))))

(event `RemoveEnergie`
  (`/Engine/EditorBlueprintResources/StandardMacros.DecrementInt` (`self.nbCableIn`)))

(fn `UserConstructionScript`)