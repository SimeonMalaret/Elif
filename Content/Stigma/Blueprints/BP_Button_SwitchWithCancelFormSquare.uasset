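; A floor switch button that toggles on and off each time a tagged object lands on it while empty, with an overlap count tracking occupancy.
; Each toggle calls Camille_GM to activate or lock by event names, or reverse both, then swaps material and plays a Wwise sound.
; Reset forces it off, while ForceValidateAndStop shows the valid material and changes the accepted tag.
; Push animation and timed cancel logic are disconnected.
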(event `self.ReceiveBeginPlay`
  (bind (_returnvalue_x _returnvalue_y _returnvalue_z) (`KismetMathLibrary.BreakVector` (`SceneComponent.K2_GetComponentLocation` (`self.Button`))))
  (set `self.InitPushPosZ` _returnvalue_z)
  (set `self.baseMaterial` (`PrimitiveComponent.GetMaterial` (`self.Button`) 0)))

(event `self.ReceiveTick`
  (params (DeltaSeconds :type "Float (single-precision)")))

(event `Reset`
  (bind _button (`self.Button`))
  (bind _ascamille_gm (cast `/Game/Stigma/Blueprints/Camille_GM` (`GameplayStatics.GetGameMode`) :!pure true))
  (set `self.isSwitched` false)
  (if (stale `self.Box.OnComponentBeginOverlap` _output_get_2) :!label _label
    (`/Game/Stigma/Blueprints/Camille_GM.ActivationByButton` _ascamille_gm (`self.eventNameToActive`))
    (`/Game/Stigma/Blueprints/Camille_GM.LockByButton` _ascamille_gm (`self.eventNameToUnactive`))
    (`PrimitiveComponent.SetMaterial` _button 0 (`self.isValideMaterial`))
    (else
      (`/Game/Stigma/Blueprints/Camille_GM.UnactivationByButton` _ascamille_gm (`self.eventNameToActive`))
      (`/Game/Stigma/Blueprints/Camille_GM.UnLockByButton` _ascamille_gm (`self.eventNameToUnactive`))
      (`PrimitiveComponent.SetMaterial` _button 0 (`self.baseMaterial`))))
  (`AkGameObject.PostAssociatedAkEvent` :`self` (`self.ButtonSound`)))

(event `self.Box.OnComponentBeginOverlap`
  (params (OverlappedComponent :type "PrimitiveComponent Object Reference") (OtherActor :type "Actor Object Reference") (OtherComp :type "PrimitiveComponent Object Reference") (OtherBodyIndex :type Integer) (bFromSweep :type Boolean) (SweepResult :type "HitResult Structure (by ref)"))
  (if (`self.ActorHasTag` OtherActor (`self.InteractibleTag`))
    (bind _output_get (set `self.nbObjOnButton` (+ (`self.nbObjOnButton`) 1)))
    (if (== _output_get 1)
      (set `self.isPush` true)
      (bind _output_get_2 (set `self.isSwitched` (not (`self.isSwitched`))))
      (goto _label))))

(event `self.Box.OnComponentEndOverlap`
  (params (OverlappedComponent :type "PrimitiveComponent Object Reference") (OtherActor :type "Actor Object Reference") (OtherComp :type "PrimitiveComponent Object Reference") (OtherBodyIndex :type Integer))
  (if (`self.ActorHasTag` OtherActor (`self.InteractibleTag`))
    (bind _output_get (set `self.nbObjOnButton` (- (`self.nbObjOnButton`) 1)))
    (if (== _output_get 0)
      (bind _output_get_2 (set `self.isPush` false))
      (if (`self.debug`)
        (`KismetSystemLibrary.PrintString` (`KismetStringLibrary.Conv_BoolToString` _output_get_2))))))

(event `ForceValidateAndStop`
  (set `self.InteractibleTag` "ValideAndStop")
  (`PrimitiveComponent.SetMaterial` (`self.Button`) 0 (`self.isValideMaterial`)))

(fn `UserConstructionScript`)