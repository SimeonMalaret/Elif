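; BP_Cible_Nara is a narration actor that stages a scripted cinematic when its Nara event is called.
; It snaps the game mode's Character to a set position, rotation and fixed scale, then disables input and movement while its level sequence plays.
; A delay matching the sequence length restores walking and input.
; In parallel, after a separate configurable delay, it sends the Companion to a target location.
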(event `self.Nara`
  (bind _ascamille_gm (cast `/Game/Stigma/Blueprints/Camille_GM` (`GameplayStatics.GetGameMode`)))
  (`|ExecutionSequence`
    (:`then_0`
      (`|ExecutionSequence`
        (:`then_0`
          (bind _character (`/Game/Stigma/Blueprints/Camille_GM.character` _ascamille_gm))
          (`self.K2_SetActorTransform` _character (`KismetMathLibrary.MakeTransform` (`self.PositionOnGround`) (`self.RotationForCamera`) (0.8 0.8 0.8)) false false))
        (:`then_1`
          (`self.DisableInput` _character (`GameplayStatics.GetPlayerController` 0))
          (bind _charactermovement (`Character.CharacterMovement` _character))
          (`CharacterMovementComponent.DisableMovement` _charactermovement)
          (bind (_outactor _returnvalue) (`LevelSequencePlayer.CreateLevelSequencePlayer` (`self.Sequence To Play`)))
          (`MovieSceneSequencePlayer.Play` _returnvalue)
          (`KismetSystemLibrary.Delay` (`TimeManagementBlueprintLibrary.Conv_QualifiedFrameTimeToSeconds` (`MovieSceneSequencePlayer.GetDuration` _returnvalue)))
          (`CharacterMovementComponent.SetMovementMode` _charactermovement "MOVE_Walking" 0)
          (`self.EnableInput` _character (`GameplayStatics.GetPlayerController` 0)))))
    (:`then_1`
      (`KismetSystemLibrary.Delay` (`self.Delay`))
      (`/Game/Stigma/Blueprints/Companion/BP_Companion.MoveTo` (`/Game/Stigma/Blueprints/Camille_GM.companion` _ascamille_gm) (`self.Location`)))))

(fn `UserConstructionScript`
  (`parent.UserConstructionScript`))