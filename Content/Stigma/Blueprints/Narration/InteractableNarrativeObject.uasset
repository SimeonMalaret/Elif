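; Interactable narrative object that displays a timed sequence of dialogue text on screen when interacted with.
; Interact turns off the Sphere's overlap events and adds a TextBp widget to the viewport.
; A hand-built latent loop shows each Dialogue entry for its matching TimeDialogues delay, resetting the display between lines.
; After a final Duration delay the widget fades; the AudioDialogues lookup is left unconnected.
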(event `Interact`
  (set `PrimitiveComponent.bGenerateOverlapEvents` false (`self.Sphere`))
  (bind _returnvalue (`|CreateWidget` "/Game/ThirdPersonCPP/Blueprints/Francois/TextBp.TextBp_C"))
  (`UserWidget.AddToViewport` _returnvalue 0)
  (set `self.Index Loop` 0)
  (if (< (`self.Index Loop`) (`KismetArrayLibrary.Array_Length` (`self.Dialogue`))) :!label _label
    (`/Game/Stigma/Blueprints/Narration/NarrationFunction.DisplayMessage` (`|GetArrayItem` (`self.Dialogue`) (`self.Index Loop`)) (`|GetArrayItem` (`self.TimeDialogues`) (`self.Index Loop`)) _returnvalue)
    (`KismetSystemLibrary.Delay` (`|GetArrayItem` (`self.TimeDialogues`) (`self.Index Loop`)))
    (`/Engine/EditorBlueprintResources/StandardMacros.IncrementInt` (`self.Index Loop`)
      (:`  `
        (`/Game/Stigma/Blueprints/Narration/NarrationFunction.ResetDisplay` _returnvalue)
        (goto _label)))
    (else
      (`KismetSystemLibrary.Delay` (`self.Duration`))
      (`/Game/ThirdPersonCPP/Blueprints/Francois/TextBp.Fade` _returnvalue))))

(fn `UserConstructionScript`)