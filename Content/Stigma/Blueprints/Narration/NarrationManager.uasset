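; NarrationManager plays a sequence of narration lines, showing text on screen with matching Wwise audio.
; StartNarration creates or resets a TextBp widget, stopping current audio on reuse, then walks the given indices into Narrations.
; Each entry fades out the previous text, displays its own, fades in and waits its timing.
; After the last, a final fade runs, then optional clouds are removed and an optional item is destroyed.
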(event `StartNarration`
  (params (IndexToPlay :type "Array of Integer") (Cloud :type "/Game/ThirdPersonCPP/Blueprints/Francois/Cloud Object Reference") (`Item To Destroy` :type "Actor Object Reference"))
  (bind (_narrative_instance_texte _narrative_instance_timing _narrative_instance_playaudio _narrative_instance_stopaudio) (break `/Game/Stigma/Blueprints/Narration/Struct_Dialogue` (`self.Narrative Instance`)))
  (bind _ak (`self.Ak`))
  (bind _ak_2 (`self.Ak`))
  (bind _widgettext (`self.WidgetText`))
  (set `self.Index to Play` IndexToPlay)
  (bind _widgettext_2 (`self.WidgetText`)
    (:`then`
      (`/Game/Stigma/Blueprints/Narration/NarrationFunction.ResetDisplay` _widgettext_2)
      (set `AkGameObject.AkAudioEvent` _narrative_instance_stopaudio _ak)
      (`AkGameObject.PostAssociatedAkEvent` :`self` _ak))
    (:`else`
      (bind _returnvalue (`|CreateWidget` "/Game/ThirdPersonCPP/Blueprints/Francois/TextBp.TextBp_C"))
      (bind _output_get (set `self.WidgetText` _returnvalue))
      (`UserWidget.AddToViewport` _returnvalue 0)
      (`UserWidget.AddToViewport` _output_get 0)))
  (set `self.Index Loop` 0)
  (if (< (`self.Index Loop`) (`KismetArrayLibrary.Array_Length` (`self.Index to Play`))) :!label _label
    (bind (_direction _fade) (`Timeline|FadeOut` :!via `PlayFromStart`)
      (:`Update`
        (`Widget.SetRenderOpacity` _widgettext _fade))
      (:`Finished`
        (`/Game/Stigma/Blueprints/Narration/NarrationFunction.ResetDisplay` _widgettext)
        (bind _output_get_2 (set `self.Narrative Instance` (`|GetArrayItem` (`self.Narrations`) (`|GetArrayItem` (`self.Index to Play`) (`self.Index Loop`)))))
        (`/Game/Stigma/Blueprints/Narration/NarrationFunction.DisplayMessage` (break `/Game/Stigma/Blueprints/Narration/Struct_Dialogue` _output_get_2) 1.0 _widgettext)
        (set `AkGameObject.AkAudioEvent` (`.PlayAudio_10_4C7DD743448E433043D39DA3A834BD3B` (break `/Game/Stigma/Blueprints/Narration/Struct_Dialogue` _output_get_2)) _ak_2)
        (`AkGameObject.PostAssociatedAkEvent` :`self` _ak_2)
        (bind (_direction_2 _fade_2) (`Timeline|FadeIn` :!via `PlayFromStart`)
          (:`Update`
            (`Widget.SetRenderOpacity` _widgettext _fade_2))
          (:`Finished`
            (`KismetSystemLibrary.Delay` (`.Timing_5_CB85ADC54E882F9E7758D9B3EF6F9EB2` (break `/Game/Stigma/Blueprints/Narration/Struct_Dialogue` _output_get_2)))
            (if (> (`KismetArrayLibrary.Array_Length` (`self.Index After Delay`)) 0)
              (if (not (`KismetArrayLibrary.Array_Identical` (`self.Index After Delay`) (`self.Index to Play`)))
                (set `self.Index After Delay` (`self.Index to Play`)))
              (else
                (set `self.Index After Delay` (`self.Index to Play`))))
            (`/Engine/EditorBlueprintResources/StandardMacros.IncrementInt` (`self.Index Loop`)
              (:`  `
                (goto _label)))))))
    (else
      (bind (_direction_3 _fade_3) (`Timeline|Timeline_0` :!via `PlayFromStart`)
        (:`Update`
          (`Widget.SetRenderOpacity` _widgettext _fade_3))
        (:`Finished`
          (`/Engine/EditorBlueprintResources/StandardMacros.IsValid` Cloud
            (:`Is Valid`
              (`/Game/ThirdPersonCPP/Blueprints/Francois/Cloud.RemoveClouds` Cloud))
            (:`Is Not Valid`
              _))
          (`/Engine/EditorBlueprintResources/StandardMacros.IsValid` `Item To Destroy`
            (:`Is Valid`
              (`self.K2_DestroyActor` `Item To Destroy`)
              (set `self.Narrative Instance` (struct)))))))))

(fn `UserConstructionScript`)