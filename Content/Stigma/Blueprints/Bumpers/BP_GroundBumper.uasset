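; BP_GroundBumper is a frog-shaped ground bumper prop that bounces the player's SecondGameplayCharacter straight up into the air.
; Overlapping its Box launches the character with a fixed upward velocity that overrides only Z, so horizontal momentum is kept.
; Each bounce also posts a Wwise bounce sound, plays the bumper's skeletal animation once, and starts narration at IndexToPlay through the STIGMA_GM NarrationManager when that manager is valid.
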(event `self.Box.OnComponentBeginOverlap`
  (params (OverlappedComponent :type "PrimitiveComponent Object Reference") (OtherActor :type "Actor Object Reference") (OtherComp :type "PrimitiveComponent Object Reference") (OtherBodyIndex :type Integer) (bFromSweep :type Boolean) (SweepResult :type "HitResult Structure (by ref)"))
  ;[1 1 1] Bump
  (bind _assecond_gameplay_character (cast `/Game/ThirdPersonCPP/Blueprints/SecondGameplayCharacter` OtherActor))
  (`Character.LaunchCharacter` _assecond_gameplay_character (0.0 0.0 1900.0) false true)
  (`AkGameObject.PostAssociatedAkEvent` :`self` (`self.Bounce Sound`))
  (`SkeletalMeshComponent.PlayAnimation` (`self.SkeletalMeshComponent`) "/Game/Stigma/Assets/3D/Bumper/Bumper_Anim/PROD_PRPS_Frog_Bumper_Ground_04.PROD_PRPS_Frog_Bumper_Ground_04_Animation" false)
  (bind _narrationmanager (`/Game/Stigma/Blueprints/STIGMA_GM.NarrationManager` (cast `/Game/Stigma/Blueprints/STIGMA_GM` (`GameplayStatics.GetGameMode`) :!pure true))
    (:`then`
      (`/Game/Stigma/Blueprints/Narration/NarrationManager.StartNarration` _narrationmanager (`self.Index To Play`) null null null))
    (:`else`)))

(fn `UserConstructionScript`)