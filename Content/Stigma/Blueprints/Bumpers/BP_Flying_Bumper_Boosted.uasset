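; Flying frog bumper that launches a SecondGameplayCharacter straight up when it overlaps the trigger box.
; BeginPlay starts two timelines, one lerping four blade rotations toward a 360-degree yaw offset, the other bobbing the skeletal mesh vertically.
; Each bump overrides Z velocity, plays a Wwise bounce sound and a one-shot animation, and starts indexed narration through the game mode's NarrationManager.
; The bottom-left blade's initial rotation is never stored, as BottomRight's variable is assigned twice.
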(event `self.ReceiveBeginPlay`
  (bind _initialposition (`self.InitialPosition`))
  (bind (_initialupleft_rotation_roll _initialupleft_rotation_pitch _initialupleft_rotation_yaw) (`KismetMathLibrary.BreakRotator` (`self.InitialUpLeft Rotation`)))
  (bind (_initialupright_rotation_roll _initialupright_rotation_pitch _initialupright_rotation_yaw) (`KismetMathLibrary.BreakRotator` (`self.InitialUpRight Rotation`)))
  (bind (_initialbotright_rotation_roll _initialbotright_rotation_pitch _initialbotright_rotation_yaw) (`KismetMathLibrary.BreakRotator` (`self.InitialBotRight Rotation`)))
  (bind (_initialbotleft_rotation_roll _initialbotleft_rotation_pitch _initialbotleft_rotation_yaw) (`KismetMathLibrary.BreakRotator` (`self.InitialBotLeft Rotation`)))
  (bind (_returnvalue_x _returnvalue_y _returnvalue_z) (`KismetMathLibrary.BreakVector` (+ (`KismetMathLibrary.MakeVector` _initialbotleft_rotation_roll _initialbotleft_rotation_pitch _initialbotleft_rotation_yaw) (0.0 0.0 360.0))))
  (bind (_returnvalue_x_2 _returnvalue_y_2 _returnvalue_z_2) (`KismetMathLibrary.BreakVector` (+ (`KismetMathLibrary.MakeVector` _initialupleft_rotation_roll _initialupleft_rotation_pitch _initialupleft_rotation_yaw) (0.0 0.0 360.0))))
  (bind (_returnvalue_x_3 _returnvalue_y_3 _returnvalue_z_3) (`KismetMathLibrary.BreakVector` (+ (`KismetMathLibrary.MakeVector` _initialupright_rotation_roll _initialupright_rotation_pitch _initialupright_rotation_yaw) (0.0 0.0 360.0))))
  (bind (_returnvalue_x_4 _returnvalue_y_4 _returnvalue_z_4) (`KismetMathLibrary.BreakVector` (+ (`KismetMathLibrary.MakeVector` _initialbotright_rotation_roll _initialbotright_rotation_pitch _initialbotright_rotation_yaw) (0.0 0.0 360.0))))
  (set `self.InitialPosition` (`self.K2_GetActorLocation`))
  (set `self.InitialUpLeft Rotation` (`SceneComponent.RelativeRotation` (`self.BladeUpLeft`)))
  (set `self.InitialUpRight Rotation` (`SceneComponent.RelativeRotation` (`self.BladeUpRight`)))
  (set `self.InitialBotRight Rotation` (`SceneComponent.RelativeRotation` (`self.BladeBottomLeft`)))
  (set `self.InitialBotRight Rotation` (`SceneComponent.RelativeRotation` (`self.BladeBottomRight`)))
  (set `self.EndUpLeft` (`KismetMathLibrary.MakeRotator` _returnvalue_x_2 _returnvalue_y_2 _returnvalue_z_2))
  (set `self.EndUpRight` (`KismetMathLibrary.MakeRotator` _returnvalue_x_3 _returnvalue_y_3 _returnvalue_z_3))
  (set `self.EndBotRight` (`KismetMathLibrary.MakeRotator` _returnvalue_x_4 _returnvalue_y_4 _returnvalue_z_4))
  (set `self.EndBotLeft` (`KismetMathLibrary.MakeRotator` _returnvalue_x _returnvalue_y _returnvalue_z))
  (`|ExecutionSequence`
    (:`then_0`
      (bind (_direction _movementblades) (`Timeline|Blades`)
        (:`Update`
          (`SceneComponent.K2_SetRelativeRotation` (`self.BladeUpLeft`) (`KismetMathLibrary.RLerp` (`self.InitialUpLeft Rotation`) (`self.EndUpLeft`) _movementblades) false false)
          (`SceneComponent.K2_SetRelativeRotation` (`self.BladeUpRight`) (`KismetMathLibrary.RLerp` (`self.InitialUpRight Rotation`) (`self.EndUpRight`) _movementblades) false false)
          (`SceneComponent.K2_SetRelativeRotation` (`self.BladeBottomRight`) (`KismetMathLibrary.RLerp` (`self.InitialBotRight Rotation`) (`self.EndBotRight`) _movementblades) false false)
          (`SceneComponent.K2_SetRelativeRotation` (`self.BladeBottomLeft`) (`KismetMathLibrary.RLerp` (`self.InitialBotLeft Rotation`) (`self.EndBotLeft`) _movementblades) false false))))
    (:`then_1`
      (bind (_direction_2 _verticalmovement) (`Timeline|Bumper`)
        (:`Update`
          (`SceneComponent.K2_SetRelativeLocation` (`self.SkeletalMeshComponent`) (`KismetMathLibrary.VLerp` _initialposition (+ _initialposition (0.0 0.0 15.0)) _verticalmovement) false false))))))

(event `self.Box.OnComponentBeginOverlap`
  (params (OverlappedComponent :type "PrimitiveComponent Object Reference") (OtherActor :type "Actor Object Reference") (OtherComp :type "PrimitiveComponent Object Reference") (OtherBodyIndex :type Integer) (bFromSweep :type Boolean) (SweepResult :type "HitResult Structure (by ref)"))
  ;[1 1 1] Bump
  (bind _assecond_gameplay_character (cast `/Game/ThirdPersonCPP/Blueprints/SecondGameplayCharacter` OtherActor))
  (`Character.LaunchCharacter` _assecond_gameplay_character (0.0 0.0 2100.0) false true)
  (`AkGameObject.PostAssociatedAkEvent` :`self` (`self.Bounce Sound`))
  (`SkeletalMeshComponent.PlayAnimation` (`self.SkeletalMeshComponent`) "/Game/Stigma/Assets/3D/Bumper/Bumper_Anim/PROD_PRPS_Frog_Bumper_Fly_04.PROD_PRPS_Frog_Bumper_Fly_04_Animation" false)
  (bind _narrationmanager (`/Game/Stigma/Blueprints/STIGMA_GM.NarrationManager` (cast `/Game/Stigma/Blueprints/STIGMA_GM` (`GameplayStatics.GetGameMode`) :!pure true))
    (:`then`
      (`/Game/Stigma/Blueprints/Narration/NarrationManager.StartNarration` _narrationmanager (`self.Index To Play`) null null null))
    (:`else`)))

(fn `UserConstructionScript`)