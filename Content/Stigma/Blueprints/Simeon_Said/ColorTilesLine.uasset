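; ColorTilesLine is a line of color tiles for the Simeon Said minigame, controlled as a group.
; When given its manager, it stores the reference and sets each tile to a random color from the manager's color list, falling back to blue if the list is empty.
; It also exposes events that set every tile in the line to one color or reset them all.
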(event `SetManager`
  (params (manager :type "/Game/Stigma/Blueprints/Simeon_Said/SimeonManager Object Reference"))
  (bind _output_get (set `self.SimeonManager` manager))
  (for _array_element (`self.Tiless`)
    (bind _colorlist (`/Game/Stigma/Blueprints/Simeon_Said/SimeonManager.colorList` _output_get))
    (bind _returnvalue (`KismetArrayLibrary.Array_Length` _colorlist))
    (if (> _returnvalue 0)
      (`/Game/Stigma/Blueprints/Simeon_Said/ColorTile.SetColor` _array_element (`|GetArrayItem` _colorlist (`KismetMathLibrary.RandomInteger` _returnvalue)))
      (else
        (`/Game/Stigma/Blueprints/Simeon_Said/ColorTile.SetColor` _array_element "/Game/Stigma/Material/Blue.Blue")))))

(event `SetLineColor`
  (params (colorMat :type "Material Object Reference"))
  (for _array_element (`self.Tiless`)
    (`/Game/Stigma/Blueprints/Simeon_Said/ColorTile.SetColor` _array_element colorMat)))

(event `ResetLineColor`
  (for _array_element (`self.Tiless`)
    (`/Game/Stigma/Blueprints/Simeon_Said/ColorTile.ResetColor` _array_element)))

(fn `UserConstructionScript`)