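; ColorTile is a floor tile for the Simeon Said color minigame that reports its current color when a player touches it.
; It keeps a base material and a current material, with events to set either on the Color component or reset to the base.
; When a SecondGameplayCharacter begins overlapping its Box, it passes the current material and that character to its TileLine's CheckColor for evaluation.
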(event `SetBaseColor`
  (params (material :type "Material Object Reference"))
  (set `self.BaseMat` material)
  (`self.SetColor` material))

(event `SetColor`
  (params (material :type "Material Object Reference"))
  (`PrimitiveComponent.SetMaterial` (`self.Color`) 0 material)
  (set `self.Material` material))

(event `ResetColor`
  (bind _basemat (`self.BaseMat`))
  (`PrimitiveComponent.SetMaterial` (`self.Color`) 0 _basemat)
  (set `self.Material` _basemat))

(event `self.Box.OnComponentBeginOverlap`
  (params (OverlappedComponent :type "PrimitiveComponent Object Reference") (OtherActor :type "Actor Object Reference") (OtherComp :type "PrimitiveComponent Object Reference") (OtherBodyIndex :type Integer) (bFromSweep :type Boolean) (SweepResult :type "HitResult Structure (by ref)"))
  (bind _assecond_gameplay_character (cast `/Game/ThirdPersonCPP/Blueprints/SecondGameplayCharacter` OtherActor))
  (`/Game/Stigma/Blueprints/Simeon_Said/ColorTilesLine.CheckColor` (`self.tileLine`) (`self.Material`) _assecond_gameplay_character))

(fn `UserConstructionScript`)