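; Manager for a Simon Says-style color game that periodically changes the color shown on an indicator.
; On BeginPlay it blacks out the indicator, starts an initial countdown and registers itself as manager on each of its Lines.
; A Tick-driven timer then picks a random material from ColorList, falling back to Blue when empty, applies it to the indicator and prints a debug message.
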(event `self.ReceiveBeginPlay`
  (`PrimitiveComponent.SetMaterial` (`self.colorIndicator`) 0 "/Game/Stigma/Player/Black.Black")
  (set `self.timer` 5.0)
  (for _array_element (`self.Lines`)
    (`/Game/Stigma/Blueprints/Simeon_Said/ColorTilesLine.SetManager` _array_element self)))

(event `self.ReceiveTick`
  (params (DeltaSeconds :type "Float (single-precision)"))
  (bind _colorlist (`self.colorList`))
  (bind _returnvalue (`KismetArrayLibrary.Array_Length` _colorlist))
  (bind _output_get (set `self.timer` (- (`self.timer`) DeltaSeconds)))
  (if (<= _output_get 0.0)
    (if (> _returnvalue 0)
      (set `self.CurentColor` (`|GetArrayItem` _colorlist (`KismetMathLibrary.RandomInteger` _returnvalue)))
      (else
        (bind _output_get_2 (set `self.CurentColor` "/Game/Stigma/Material/Blue.Blue"))))
    (`PrimitiveComponent.SetMaterial` (`self.colorIndicator`) 0 (`self.CurentColor`))
    (`KismetSystemLibrary.PrintString` (`KismetStringLibrary.Concat_StrStr` "change color to " (`KismetSystemLibrary.GetObjectName` _output_get_2)))
    (set `self.timer` (+ (`self.timer`) (`self.switchColorInterval`)))))

(fn `UserConstructionScript`)