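; BP_DecoPaperPlane is a decorative paper plane actor, by its name, that bobs vertically around the level.
; On BeginPlay it stores its start location, picks a random bob height and waits a random delay so instances desynchronize.
; A Movement timeline then lerps the actor upward from that location, flipping a boolean on each finish to play or reverse in an endless ping-pong.
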(event `self.ReceiveBeginPlay`
  (bind _initialposition (`self.InitialPosition`))
  (set `self.InitialPosition` (`self.K2_GetActorLocation`))
  (set `self.SizeMovement` (`KismetMathLibrary.RandomFloatInRange` 50.0 80.0))
  (`KismetSystemLibrary.Delay` (`KismetMathLibrary.RandomFloatInRange` 0.0 2.5))
  (bind (_direction _lerpdeltatime) (`Timeline|Movement` :!label _label)
    (:`Update`
      (`self.K2_SetActorLocation` (`KismetMathLibrary.VLerp` _initialposition (+ _initialposition (`KismetMathLibrary.MakeVector` 0.0 0.0 (`self.SizeMovement`))) _lerpdeltatime)))
    (:`Finished`
      (bind _output_get (set `self.ForwardTime` (not (`self.ForwardTime`))))
      (if _output_get
        (goto _label)
        (else
          (goto _label :!via `Reverse`))))))

(fn `UserConstructionScript`)