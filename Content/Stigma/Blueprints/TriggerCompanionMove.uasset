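; Trigger actor that sends the level's companion to a set location when a tagged actor enters it.
; On BeginPlay it finds and caches the BP_Companion instance as its target.
; An overlap from an actor with the configured tag waits a configurable delay, calls MoveTo on the companion, then calls Unactive on it if the UnactiveCompanion flag is set.
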(event `self.ReceiveBeginPlay`
  (bind _returnvalue (`GameplayStatics.GetActorOfClass` "/Game/Stigma/Blueprints/Companion/BP_Companion.BP_Companion_C"))
  (set `self.Target` _returnvalue))

(event `self.trigger.OnComponentBeginOverlap`
  (params (OverlappedComponent :type "PrimitiveComponent Object Reference") (OtherActor :type "Actor Object Reference") (OtherComp :type "PrimitiveComponent Object Reference") (OtherBodyIndex :type Integer) (bFromSweep :type Boolean) (SweepResult :type "HitResult Structure (by ref)"))
  (if (`self.ActorHasTag` OtherActor (`self.Tag`))
    (`KismetSystemLibrary.Delay` (`self.Delay`))
    (`/Game/Stigma/Blueprints/Companion/BP_Companion.MoveTo` (`self.Target`) (`self.Location`))
    (if (`self.UnactiveCompanion`)
      (`/Game/Stigma/Blueprints/Companion/BP_Companion.Unactive` (`self.Target`)))))

(fn `UserConstructionScript`)