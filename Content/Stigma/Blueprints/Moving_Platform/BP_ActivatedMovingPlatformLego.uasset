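; Lego moving platform that opens and closes like a bridge in response to button events broadcast by STIGMA_GM.
; Matching activation events raise a counter that opens it at a threshold; deactivation lowers it to close.
; Lock forces closing and blocks opening until unlock events bring that shared counter to zero.
; A speed-adjusted timeline lerps the actor between two transforms with Wwise audio, and the mesh gets a random material.
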(event `OpenBrodgeByButton`
  (params (eventName :type "Array of String (by ref)"))
  (if (`KismetArrayLibrary.Array_Contains` eventName (`self.Event Name`))
    (bind _output_get (set `self.nbActors` (+ (`self.nbActors`) 1)))
    (if (and (>= _output_get (`self.Nb Actor to Open`)) (not (`self.Is Lock`)))
      (set `self.IsOpen` true)
      (`self.StartOpenBridge`)
      (if (`self.debug`)
        (`KismetSystemLibrary.PrintString` "Open")))))

(event `Lock`
  (params (eventName :type "Array of String (by ref)"))
  (if (`KismetArrayLibrary.Array_Contains` eventName (`self.Event Name`))
    (if (`self.debug`)
      (`KismetSystemLibrary.PrintString` "Lock"))
    (set `self.Is Lock` true)
    (set `self.nbLock` (+ (`self.nbActors`) 1))
    (set `self.IsOpen` false)
    (`self.StartCloseBridge`)))

(event `self.ReceiveBeginPlay`
  (bind _asstigma_gm (cast `/Game/Stigma/Blueprints/STIGMA_GM` (`GameplayStatics.GetGameMode`) :!pure true))
  (`PrimitiveComponent.SetMaterial` (`self.Mesh`) 0 (`|GetArrayItem` (`self.MaterialsList`) (`KismetMathLibrary.RandomInteger` (`KismetArrayLibrary.Array_Length` (`self.MaterialsList`)))))
  (add `/Game/Stigma/Blueprints/STIGMA_GM.ActivationByButton` _asstigma_gm (delegate `OpenBrodgeByButton`))
  (add `/Game/Stigma/Blueprints/STIGMA_GM.UnactivationByButton` _asstigma_gm (delegate `CloseBridgeByButton`))
  (add `/Game/Stigma/Blueprints/STIGMA_GM.LockByButton` _asstigma_gm (delegate `Lock`))
  (add `/Game/Stigma/Blueprints/STIGMA_GM.UnLockByButton` _asstigma_gm (delegate `Unlock`)))

(event `Unlock`
  (params (eventName :type "Array of String (by ref)"))
  (if (`KismetArrayLibrary.Array_Contains` eventName (`self.Event Name`))
    (if (`self.debug`)
      (`KismetSystemLibrary.PrintString` "unlock"))
    (bind _output_get (set `self.nbActors` (- (`self.nbActors`) 1)))
    (if (<= _output_get 0)
      (set `self.Is Lock` false)
      (if (>= (`self.nbActors`) (`self.Nb Actor to Open`))
        (set `self.IsOpen` true)
        (`self.StartOpenBridge`)))))

(event `CloseBridgeByButton`
  (params (eventName :type "Array of String (by ref)"))
  (if (`KismetArrayLibrary.Array_Contains` eventName (`self.Event Name`))
    (bind _output_get (set `self.nbActors` (- (`self.nbActors`) 1)))
    (if (< _output_get (`self.Nb Actor to Open`))
      (set `self.IsOpen` false)
      (`self.StartCloseBridge`)
      (if (`self.debug`)
        (`KismetSystemLibrary.PrintString` "Close")))))

(event `StartOpenBridge`
  (`TimelineComponent.SetPlayRate` (`self.Timeline_0`) (`self.Opening Speed`))
  (if (`self.isMoving`)
    (bind (_direction _opening) (`Timeline|Timeline_0` :!label _label)
      (:`Update`
        (bind _output_get (set `self.Alpha` _opening))
        (`self.K2_SetActorTransform` (`KismetMathLibrary.TLerp` (`self.PositionStart`) (`self.PositionEnd`) _output_get) false true)
        (set `self.isMoving` true))
      (:`Finished`
        (set `self.isMoving` false)
        (`AkGameObject.Stop` (`self.BridgeDownSound1`))))
    (elif (< (`self.Alpha`) 2.0)
      (`AkGameObject.PostAssociatedAkEvent` :`self` (`self.BridgeDownSound1`))
      (goto _label))))

(event `StartCloseBridge`
  (`TimelineComponent.SetPlayRate` (`self.Timeline_0`) (`self.ClosingSpeed`))
  (if (`self.isMoving`)
    (goto _label :!via `Reverse`)
    (elif (> (`self.Alpha`) 0.0)
      (`AkGameObject.PostAssociatedAkEvent` :`self` (`self.BridgeDownSound1`))
      (goto _label :!via `Reverse`))))

(fn `UserConstructionScript`
  (`PrimitiveComponent.SetMaterial` (`self.Mesh`) 0 (`|GetArrayItem` (`self.MaterialsList`) (`KismetMathLibrary.RandomInteger` (`KismetArrayLibrary.Array_Length` (`self.MaterialsList`))))))