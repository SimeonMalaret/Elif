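; BP_MovingPlatformLego is a moving platform that travels between a start and end location and shows a random material.
; The construction script feeds StartLocation and EndLocation to InterpToMovement as relative control points and sets its travel Duration.
; It also gives the mesh a random entry from MaterialsList, and BeginPlay picks again, so the in-game look can differ from the editor.
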(event `self.ReceiveBeginPlay`
  (`PrimitiveComponent.SetMaterial` (`self.Mesh`) 0 (`|GetArrayItem` (`self.MaterialsList`) (`KismetMathLibrary.RandomInteger` (`KismetArrayLibrary.Array_Length` (`self.MaterialsList`))))))

(fn `UserConstructionScript`
  (bind _interptomovement (`self.InterpToMovement`))
  (set `InterpToMovementComponent.ControlPoints` (`|MakeArray` (make `InterpControlPoint` (`self.StartLocation`)) (make `InterpControlPoint` (`self.EndLocation`))) _interptomovement)
  (set `InterpToMovementComponent.Duration` (`self.Duration`) _interptomovement)
  (`PrimitiveComponent.SetMaterial` (`self.Mesh`) 0 (`|GetArrayItem` (`self.MaterialsList`) (`KismetMathLibrary.RandomInteger` (`KismetArrayLibrary.Array_Length` (`self.MaterialsList`))))))