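; BP_Cart is a cart actor with a configurable body mesh and two animated eyes.
; On BeginPlay it applies MeshToShow to the Body and starts the Eyes timeline, which lerps the pitch of both eyes in unison between two angles.
; When the timeline finishes, it flips SwitchMovement to choose Play or Reverse, keeping the eyes swinging back and forth.
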(event `self.ReceiveBeginPlay`
  (`StaticMeshComponent.SetStaticMesh` (`self.Body`) (`self.Mesh To Show`))
  (bind (_direction _movementeyes) (`Timeline|Eyes` :!label _label)
    (:`Update`
      (bind _returnvalue (`KismetMathLibrary.Lerp` 20.0 35.0 _movementeyes))
      (`SceneComponent.K2_SetRelativeRotation` (`self.LeftEye`) (`KismetMathLibrary.MakeRotator` 0.0 _returnvalue) false false)
      (`SceneComponent.K2_SetRelativeRotation` (`self.RightEye`) (`KismetMathLibrary.MakeRotator` 0.0 _returnvalue) false false))
    (:`Finished`
      (bind _output_get (set `self.SwitchMovement` (not (`self.SwitchMovement`))))
      (if _output_get
        (goto _label)
        (else
          (goto _label :!via `Reverse`))))))

(fn `UserConstructionScript`)