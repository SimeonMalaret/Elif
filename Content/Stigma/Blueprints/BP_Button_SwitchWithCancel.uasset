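; Floor toggle switch that flips each time a tagged actor first steps on it, activating or cancelling named events through STIGMA_GM.
; An overlap count drives the Tick-lerped button press, while each flip swaps material, plays sound and runs a paw-and-head timeline forward or backward.
; Switching on also locks a second event and may trigger a random shout.
; Reset forces it off; ForceValidateAndStop shows it validated and changes the accepted tag.
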(event `self.ReceiveBeginPlay`
  (bind (_returnvalue_x _returnvalue_y _returnvalue_z) (`KismetMathLibrary.BreakVector` (`SceneComponent.K2_GetComponentLocation` (`self.Button`))))
  (set `self.InitPushPosZ` _returnvalue_z)
  (set `self.baseMaterial` (`PrimitiveComponent.GetMaterial` (`self.Button`) 0))
  (set `self.InitialURP` (`SceneComponent.RelativeRotation` (`self.UpRightPaw`)))
  (set `self.InitialULP` (`SceneComponent.RelativeRotation` (`self.UpLeftPaw`)))
  (set `self.InitialDRP` (`SceneComponent.RelativeRotation` (`self.DownRightPaw`)))
  (set `self.InitialDLP` (`SceneComponent.RelativeRotation` (`self.DownLeftPaw`)))
  (set `self.InitialHead` (`SceneComponent.RelativeLocation` (`self.Head`))))

(event `self.ReceiveTick`
  (params (DeltaSeconds :type "Float (single-precision)"))
  (bind _button (`self.Button`))
  (bind _lerpbuttonpush (`self.lerpButtonPush`))
  (bind (_returnvalue_x _returnvalue_y _returnvalue_z) (`KismetMathLibrary.BreakVector` (`SceneComponent.K2_GetComponentLocation` (`self.Base`))))
  (bind (_returnvalue_x_2 _returnvalue_y_2) (`KismetMathLibrary.BreakVector` (`SceneComponent.K2_GetComponentLocation` _button)))
  (bind _returnvalue (* DeltaSeconds (`self.speedPush`)))
  (if (`self.isPush`)
    (set `self.lerpButtonPush` (+ _returnvalue _lerpbuttonpush))
    (else
      (set `self.lerpButtonPush` (- _lerpbuttonpush _returnvalue))))
  (if true
    _
    (else
      _))
  (if (and (<= (`self.lerpButtonPush`) 1.0) (>= (`self.lerpButtonPush`) 0.0))
    _
    (elif (`self.isPush`)
      (set `self.lerpButtonPush` 1.0)
      (else
        (set `self.lerpButtonPush` 0.0))))
  (`SceneComponent.K2_SetWorldLocation` _button (`KismetMathLibrary.MakeVector` _returnvalue_x_2 _returnvalue_y_2 (`KismetMathLibrary.Lerp` (`self.InitPushPosZ`) _returnvalue_z (`self.lerpButtonPush`))) false false))

(event `Reset`
  (bind _button (`self.Button`))
  (bind _asstigma_gm (cast `/Game/Stigma/Blueprints/STIGMA_GM` (`GameplayStatics.GetGameMode`) :!pure true))
  (set `self.isSwitched` false)
  (if (stale `self.Box.OnComponentBeginOverlap` _output_get_2) :!label _label
    (`/Game/Stigma/Blueprints/STIGMA_GM.ActivationByButton` _asstigma_gm (`self.eventNameToActive`))
    (`|ExecutionSequence`
      (:`then_0`
        (if (>= (/ (`self.RandomClick`) 100.0) (`KismetMathLibrary.RandomFloat`))
          (`AkGameObject.PostAssociatedAkEvent` :`self` (`self.Elif_Shout_137`)))
        (`/Game/Stigma/Blueprints/STIGMA_GM.LockByButton` _asstigma_gm (`self.eventNameToUnactive`))
        (`PrimitiveComponent.SetMaterial` _button 0 (`self.isValideMaterial`))
        (if (not (`self.isNoSound`)) :!label _label_2
          (`AkGameObject.PostAssociatedAkEvent` :`self` (`self.ButtonSound`))))
      (:`then_1`
        (bind (_direction _rotate) (`Timeline|PawRotation` :!label _label_3)
          (:`Update`
            (`self.PawRotate` _rotate)))))
    (else
      (`/Game/Stigma/Blueprints/STIGMA_GM.UnactivationByButton` _asstigma_gm (`self.eventNameToActive`))
      (`|ExecutionSequence`
        (:`then_0`
          (goto _label_3 :!via `Reverse`))
        (:`then_1`
          (`/Game/Stigma/Blueprints/STIGMA_GM.UnLockByButton` _asstigma_gm (`self.eventNameToUnactive`))
          (`PrimitiveComponent.SetMaterial` _button 0 (`self.baseMaterial`))
          (goto _label_2))))))

(event `self.Box.OnComponentBeginOverlap`
  (params (OverlappedComponent :type "PrimitiveComponent Object Reference") (OtherActor :type "Actor Object Reference") (OtherComp :type "PrimitiveComponent Object Reference") (OtherBodyIndex :type Integer) (bFromSweep :type Boolean) (SweepResult :type "HitResult Structure (by ref)"))
  (if (`self.ActorHasTag` OtherActor (`self.InteractibleTag`))
    (bind _output_get (set `self.nbObjOnButton` (+ (`self.nbObjOnButton`) 1)))
    (if (== _output_get 1)
      (set `self.isPush` true)
      (bind _output_get_2 (set `self.isSwitched` (not (`self.isSwitched`))))
      (goto _label))))

(event `self.Box.OnComponentEndOverlap`
  (params (OverlappedComponent :type "PrimitiveComponent Object Reference") (OtherActor :type "Actor Object Reference") (OtherComp :type "PrimitiveComponent Object Reference") (OtherBodyIndex :type Integer))
  (if (`self.ActorHasTag` OtherActor (`self.InteractibleTag`))
    (bind _output_get (set `self.nbObjOnButton` (- (`self.nbObjOnButton`) 1)))
    (if (== _output_get 0)
      (set `self.isPush` false))))

(event `ForceValidateAndStop`
  (set `self.InteractibleTag` "ValideAndStop")
  (`PrimitiveComponent.SetMaterial` (`self.Button`) 0 (`self.isValideMaterial`)))

(fn `PawRotate`
  (params (Speed :type "Float (double-precision) (by ref)"))
  (bind _initialhead (`self.InitialHead`))
  (`SceneComponent.K2_SetRelativeRotation` (`self.UpRightPaw`) (`KismetMathLibrary.RLerp` (`self.InitialURP`) (struct :`Yaw` 50.0) Speed) false false)
  (`SceneComponent.K2_SetRelativeRotation` (`self.UpLeftPaw`) (`KismetMathLibrary.RLerp` (`self.InitialULP`) (struct :`Yaw` -40.0) Speed) false false)
  (`SceneComponent.K2_SetRelativeRotation` (`self.DownRightPaw`) (`KismetMathLibrary.RLerp` (`self.InitialDRP`) (struct :`Yaw` 55.0) Speed) false false)
  (`SceneComponent.K2_SetRelativeRotation` (`self.DownLeftPaw`) (`KismetMathLibrary.RLerp` (`self.InitialDLP`) (struct :`Yaw` -50.0) Speed) false false)
  (`SceneComponent.K2_SetRelativeLocation` (`self.Head`) (`KismetMathLibrary.VLerp` _initialhead (- _initialhead (20.0 0.0 0.0)) Speed) false false)
  (return))

(fn `UserConstructionScript`)