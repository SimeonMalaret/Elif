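; AI controller for a companion character that drives its behaviour through the BT_Companion behavior tree.
; On BeginPlay it runs the tree and uses the BB_Companion blackboard.
; Custom events act as setters that write the companion state enum, follow actor and target location into blackboard keys, so callers can change behaviour without touching the blackboard directly.
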(event `self.ReceiveBeginPlay`
  (`self.RunBehaviorTree` "/Game/Stigma/Blueprints/Companion/BT_Companion.BT_Companion")
  (`self.UseBlackboard` "/Game/Stigma/Blueprints/Companion/BB_Companion.BB_Companion"))

(event `SetCompanionState`
  (params (CompanionState :type "/Game/Stigma/Blueprints/Companion/E_CompanionState Enum" :default "NewEnumerator0"))
  (`BlackboardComponent.SetValueAsEnum` (`self.Blackboard`) "CompanionState" CompanionState))

(event `SetFollowActor`
  (params (FollowActor :type "Actor Object Reference"))
  (`BlackboardComponent.SetValueAsObject` (`self.Blackboard`) "FollowActor" FollowActor))

(event `SetTargetLocation`
  (params (TargetLocation :type "Vector Structure"))
  (`BlackboardComponent.SetValueAsVector` (`self.Blackboard`) "TargetLocation" TargetLocation))

(fn `UserConstructionScript`)