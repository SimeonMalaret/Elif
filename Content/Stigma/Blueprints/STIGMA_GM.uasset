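; STIGMA_GM is the game mode for Stigma, running setup logic when play begins.
; It finds and stores the level's NarrationManager actor.
; On levels listed in MapToBeginBallWith, it waits briefly, then forces the SecondGameplayCharacter to pick up and activates that character's whistle widget, so those maps start with the ball in hand.
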(event `self.ReceiveBeginPlay`
  (`|ExecutionSequence`
    (:`then_0`
      (bind _returnvalue (`GameplayStatics.GetActorOfClass` "/Game/Stigma/Blueprints/Narration/NarrationManager.NarrationManager_C"))
      (set `self.NarrationManager` _returnvalue))
    (:`then_1`
      (bind _returnvalue_2 (`GameplayStatics.GetCurrentLevelName` true))
      (if (`KismetArrayLibrary.Array_Contains` (`self.Map to Begin Ball With`) _returnvalue_2)
        (`KismetSystemLibrary.PrintString` "Hello")
        (bind _assecond_gameplay_character (cast `/Game/ThirdPersonCPP/Blueprints/SecondGameplayCharacter` (`GameplayStatics.GetPlayerPawn` 0)))
        (`KismetSystemLibrary.Delay` 0.2)
        (`/Game/ThirdPersonCPP/Blueprints/SecondGameplayCharacter.ForcedPickUp` _assecond_gameplay_character)
        (`/Game/Stigma/User_Interface/WBP_Whistle.ActivateWhistle` (`/Game/ThirdPersonCPP/Blueprints/SecondGameplayCharacter.Widget_Whistle` _assecond_gameplay_character) 1.0)))))

(fn `UserConstructionScript`)