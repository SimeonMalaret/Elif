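; BP_EditableButton is a pressure button that triggers named events when an actor with the interactible tag enters or leaves its box.
; Overlap begin and end pass EventName to the Camille_GM game mode's activation and unactivation calls and toggle IsPush.
; Tick ramps a clamped alpha at SpeedPush, lerping MoveObject's world Z between its starting height and the Cube's height to animate the press.
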(event `self.ReceiveBeginPlay`
  (bind (_returnvalue_x _returnvalue_y _returnvalue_z) (`KismetMathLibrary.BreakVector` (`SceneComponent.K2_GetComponentLocation` (`self.moveObject`))))
  (set `self.InitPushPosZ` _returnvalue_z))

(event `self.Box.OnComponentBeginOverlap`
  (params (OverlappedComponent :type "PrimitiveComponent Object Reference") (OtherActor :type "Actor Object Reference") (OtherComp :type "PrimitiveComponent Object Reference") (OtherBodyIndex :type Integer) (bFromSweep :type Boolean) (SweepResult :type "HitResult Structure (by ref)"))
  (if (`self.ActorHasTag` OtherActor (`self.InteractibleTag`))
    (bind _ascamille_gm (cast `/Game/Stigma/Blueprints/Camille_GM` (`GameplayStatics.GetGameMode`)))
    (`/Game/Stigma/Blueprints/Camille_GM.ActivationByButton` _ascamille_gm (`self.eventName`) null)
    (set `self.isPush` true)))

(event `self.ReceiveTick`
  (params (DeltaSeconds :type "Float (single-precision)"))
  (bind _lerpbuttonpush (`self.lerpButtonPush`))
  (bind _moveobject (`self.moveObject`))
  (bind _lerpbuttonpush_2 (`self.lerpButtonPush`))
  (bind (_returnvalue_x _returnvalue_y _returnvalue_z) (`KismetMathLibrary.BreakVector` (`SceneComponent.K2_GetComponentLocation` (`self.Cube`))))
  (bind (_returnvalue_x_2 _returnvalue_y_2) (`KismetMathLibrary.BreakVector` (`SceneComponent.K2_GetComponentLocation` _moveobject)))
  (bind _returnvalue (* DeltaSeconds (`self.speedPush`)))
  (if (`self.isPush`)
    (set `self.lerpButtonPush` (+ _returnvalue _lerpbuttonpush_2))
    (else
      (set `self.lerpButtonPush` (- _lerpbuttonpush_2 _returnvalue))))
  (if (`self.debug`)
    (`KismetSystemLibrary.PrintString` (`KismetStringLibrary.Conv_DoubleToString` _lerpbuttonpush) true true (struct :`G` 0.66 :`B` 1.0 :`A` 1.0) 0.0))
  (if (and (<= _lerpbuttonpush 1.0) (>= (`self.lerpButtonPush`) 0.0))
    _
    (elif (`self.isPush`)
      (set `self.lerpButtonPush` 1.0)
      (else
        (set `self.lerpButtonPush` 0.0))))
  (`SceneComponent.K2_SetWorldLocation` _moveobject (`KismetMathLibrary.MakeVector` _returnvalue_x_2 _returnvalue_y_2 (`KismetMathLibrary.Lerp` (`self.InitPushPosZ`) _returnvalue_z (`self.lerpButtonPush`))) false false))

(event `self.Box.OnComponentEndOverlap`
  (params (OverlappedComponent :type "PrimitiveComponent Object Reference") (OtherActor :type "Actor Object Reference") (OtherComp :type "PrimitiveComponent Object Reference") (OtherBodyIndex :type Integer))
  (if (`self.ActorHasTag` OtherActor (`self.InteractibleTag`))
    (bind _ascamille_gm (cast `/Game/Stigma/Blueprints/Camille_GM` (`GameplayStatics.GetGameMode`)))
    (`/Game/Stigma/Blueprints/Camille_GM.UnactivationByButton` _ascamille_gm (`self.eventName`) self)
    (set `self.isPush` false)))

(fn `UserConstructionScript`)