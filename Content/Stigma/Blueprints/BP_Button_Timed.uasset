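; Timed pressure button that activates one named event and locks another through Camille_GM when a first tagged object overlaps its box.
; After a delay it reverses both calls and restores the button material, even if the object remains.
; Both changes play a Wwise sound on the game mode's SoundGhost, or on itself as fallback.
; The button-sinking animation logic is disconnected, so only the material shows the state.
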(event `self.ReceiveBeginPlay`
  (bind (_returnvalue_x _returnvalue_y _returnvalue_z) (`KismetMathLibrary.BreakVector` (`SceneComponent.K2_GetComponentLocation` (`self.Button`))))
  (set `self.InitPushPosZ` _returnvalue_z)
  (set `self.baseMaterial` (`PrimitiveComponent.GetMaterial` (`self.Button`) 0)))

(event `self.ReceiveTick`
  (params (DeltaSeconds :type "Float (single-precision)")))

(event `self.Box.OnComponentBeginOverlap`
  (params (OverlappedComponent :type "PrimitiveComponent Object Reference") (OtherActor :type "Actor Object Reference") (OtherComp :type "PrimitiveComponent Object Reference") (OtherBodyIndex :type Integer) (bFromSweep :type Boolean) (SweepResult :type "HitResult Structure (by ref)"))
  (if (`self.ActorHasTag` OtherActor (`self.InteractibleTag`))
    (bind _output_get (set `self.nbObjOnButton` (+ (`self.nbObjOnButton`) 1)))
    (if (== _output_get 1)
      (set `self.isPush` true)
      (bind _ascamille_gm (cast `/Game/Stigma/Blueprints/Camille_GM` (`GameplayStatics.GetGameMode`)))
      (`KismetSystemLibrary.PrintString` "on")
      (`/Game/Stigma/Blueprints/Camille_GM.ActivationByButton` _ascamille_gm (`self.eventNameToActive`))
      (`/Game/Stigma/Blueprints/Camille_GM.LockByButton` _ascamille_gm (`self.eventNameToUnactive`))
      (`PrimitiveComponent.SetMaterial` (`self.Button`) 0 (`self.isValideMaterial`))
      (bind _ascamille_gm_2 (cast `/Game/Stigma/Blueprints/Camille_GM` (`GameplayStatics.GetGameMode`))
        (:`then`
          (bind _soundghost (`/Game/Stigma/Blueprints/Camille_GM.SoundGhost` _ascamille_gm_2)
            (:`then`
              (`AkGameplayStatics.PostEvent` "/Game/Stigma/Sound/Event/LEVELEVENT_WU/PROPS/Button/Play_Button.Play_Button" _soundghost))
            (:`else`
              (`AkGameplayStatics.PostEvent` "/Game/Stigma/Sound/Event/LEVELEVENT_WU/PROPS/Button/Play_Button.Play_Button" self :!label _label))))
        (:`CastFailed`
          (goto _label)))
      (`|ExecutionSequence`
        (:`then_0`
          (`KismetSystemLibrary.Delay` (`self.timeUnvalide`))
          (`/Game/Stigma/Blueprints/Camille_GM.UnactivationByButton` _ascamille_gm (`self.eventNameToActive`))
          (`/Game/Stigma/Blueprints/Camille_GM.UnLockByButton` _ascamille_gm (`self.eventNameToUnactive`))
          (`PrimitiveComponent.SetMaterial` (`self.Button`) 0 (`self.baseMaterial`))
          (bind _ascamille_gm_3 (cast `/Game/Stigma/Blueprints/Camille_GM` (`GameplayStatics.GetGameMode`))
            (:`then`
              (bind _soundghost_2 (`/Game/Stigma/Blueprints/Camille_GM.SoundGhost` _ascamille_gm_3)
                (:`then`
                  (`AkGameplayStatics.PostEvent` "/Game/Stigma/Sound/Event/LEVELEVENT_WU/PROPS/Button/Play_Button.Play_Button" _soundghost_2))
                (:`else`
                  (`AkGameplayStatics.PostEvent` "/Game/Stigma/Sound/Event/LEVELEVENT_WU/PROPS/Button/Play_Button.Play_Button" self :!label _label_2))))
            (:`CastFailed`
              (goto _label_2)))
          (if (`self.debug`)
            (`KismetSystemLibrary.PrintString` (`KismetStringLibrary.Conv_BoolToString` (`self.isPush`)))))
        (:`then_1`
          (if (`self.debug`)
            (`KismetSystemLibrary.PrintString` (`KismetStringLibrary.Conv_BoolToString` (`self.isPush`)))))))))

(event `self.Box.OnComponentEndOverlap`
  (params (OverlappedComponent :type "PrimitiveComponent Object Reference") (OtherActor :type "Actor Object Reference") (OtherComp :type "PrimitiveComponent Object Reference") (OtherBodyIndex :type Integer))
  (if (`self.ActorHasTag` OtherActor (`self.InteractibleTag`))
    (bind _output_get (set `self.nbObjOnButton` (- (`self.nbObjOnButton`) 1)))
    (if (== _output_get 0)
      (bind _output_get_2 (set `self.isPush` false))
      (if (`self.debug`)
        (`KismetSystemLibrary.PrintString` (`KismetStringLibrary.Conv_BoolToString` _output_get_2))))))

(fn `UserConstructionScript`)