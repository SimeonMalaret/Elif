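; Breakable wall actor that assigns its Apex destructible mesh from a soft reference at BeginPlay, async loading it if needed.
; On first fracture it changes collision responses, opens an optional linked bridge and destroys itself after a delay.
; It also damages the wall at a Z offset above, found in its WallProtector's list, so destruction can chain upward.
; It then calls the protector's Destruction and shortly resets that protector's destroyed flag.
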(event `self.ReceiveBeginPlay`
  (bind _destructiblemeshsoftref (`self.DestructibleMeshSoftRef`))
  (bind _output (`|ConvertAsset` _destructiblemeshsoftref))
  ;[1 1 1] PERSONNE NE TOUCHE À ÇA !!!!!
  (`/Engine/EditorBlueprintResources/StandardMacros.IsValid` _output
    (:`Is Valid`
      (`DestructibleComponent.SetDestructibleMesh` (`self.Destructible`) _output))
    (:`Is Not Valid`
      (bind _object (`|LoadAsset` _destructiblemeshsoftref)
        (:`Completed`
          (bind _asdestructible_mesh (cast `DestructibleMesh` _object))
          (`DestructibleComponent.SetDestructibleMesh` (`self.Destructible`) _asdestructible_mesh))))))

(event `self.Destructible.OnComponentFracture`
  (params (HitPoint :type "Vector Structure (by ref)") (HitDirection :type "Vector Structure (by ref)"))
  (bind _cube (`self.Cube`))
  (bind _wallprotector (`self.WallProtector`))
  (bind _destructible (`self.Destructible`))
  ;[1 1 1] OnFracture
  (if (not (`self.IsAlreadyDestroyed`))
    (set `self.IsAlreadyDestroyed` true)
    (`|ExecutionSequence`
      (:`then_0`
        (`PrimitiveComponent.SetCollisionResponseToChannel` _cube "ECC_GameTraceChannel5" "ECR_Ignore")
        (`PrimitiveComponent.SetCollisionResponseToChannel` _cube "ECC_Pawn" "ECR_Ignore")
        (`PrimitiveComponent.SetCollisionResponseToChannel` _cube "ECC_GameTraceChannel3" "ECR_Ignore")
        (`PrimitiveComponent.SetCollisionResponseToChannel` _destructible "ECC_GameTraceChannel6" "ECR_Ignore")
        (`PrimitiveComponent.SetCollisionResponseToChannel` _destructible "ECC_WorldStatic" "ECR_Block")
        (bind _bridgetoopen (`self.BridgeToOpen`)
          (:`then`
            (`/Game/Stigma/Blueprints/DrawBridge/DrawbridgePlatform.StartOpenBridge` _bridgetoopen))
          (:`else`
            _))
        (`KismetSystemLibrary.Delay` 5.0)
        (`self.K2_DestroyActor`))
      (:`then_1`
        (`self.Find Object In UpwardPosition`))
      (:`then_2`
        (`/Game/Stigma/Blueprints/DestructionWall/DestructibleWall.Destruction` _wallprotector)
        (`KismetSystemLibrary.Delay` 0.5)
        (set `/Game/Stigma/Blueprints/DestructionWall/DestructibleWall.Has Destroyed` false _wallprotector)))))

(fn `Find Object In UpwardPosition`
  (locals (`Element to Activate` :type "/Game/Stigma/Blueprints/DestructiblWall Object Reference"))
  (for _array_element (`/Game/Stigma/Blueprints/DestructionWall/DestructibleWall.DestructibleWalls` (`self.WallProtector`))
    (if (`KismetSystemLibrary.IsValid` _array_element)
      (if (== (`self.K2_GetActorLocation` _array_element) (+ (`self.K2_GetActorLocation`) (`KismetMathLibrary.MakeVector` 0.0 0.0 (`self.Z Offset`))) :`ErrorTolerance` 1.0)
        (set `local.Element to Activate` _array_element)
        (break))))
  (bind _element_to_activate (`local.Element to Activate`)
    (:`then`
      (`DestructibleComponent.ApplyDamage` (`/Game/Stigma/Blueprints/DestructiblWall.Destructible` _element_to_activate) 100.0 (`self.K2_GetActorLocation` _element_to_activate) (`KismetMathLibrary.MakeVector` 0.0) 0.0))
    (:`else`)))

(fn `UserConstructionScript`)