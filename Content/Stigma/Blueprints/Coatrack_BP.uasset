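; Coatrack actor that animates an upper and lower beak piece (BecUp, BecBot) from BeginPlay.
; The Bec timeline lerps both relative transforms between cached bases and end poses.
; Each finish flips MovementSwitch, alternating a slow reverse with a second timeline toward "Super" poses.
; That timeline makes the Super poses the new base and replays Bec at a faster rate, chaining the motion into a cycle.
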(event `self.ReceiveBeginPlay`
  (`TimelineComponent.SetPlayRate` (`self.Timeline_1`) 2.0)
  (bind _output_get (set `self.Start Transform Up` (`SceneComponent.GetRelativeTransform` (`self.BecUp`))))
  (set `self.Transform Local Up` _output_get)
  (bind _output_get_2 (set `self.Start Transform Bot` (`SceneComponent.GetRelativeTransform` (`self.BecBot`))))
  (set `self.Transform Local Bot` _output_get_2)
  (bind (_direction _movementbec) (`Timeline|Bec` :!label _label)
    (:`Update`
      (`SceneComponent.K2_SetRelativeTransform` (`self.BecUp`) (`KismetMathLibrary.TLerp` (`self.Transform Local Up`) (`self.End Transform Up`) _movementbec) false false)
      (`SceneComponent.K2_SetRelativeTransform` (`self.BecBot`) (`KismetMathLibrary.TLerp` (`self.Transform Local Bot`) (`self.End Transform Bot`) _movementbec) false false))
    (:`Finished`
      (bind _output_get_3 (set `self.MovementSwitch` (not (`self.MovementSwitch`))))
      (if _output_get_3
        (`TimelineComponent.SetPlayRate` (`self.Bec`) 4.5)
        (bind (_direction_2 _newtrack_0) (`Timeline|Timeline_1` :!via `PlayFromStart`)
          (:`Update`
            (`SceneComponent.K2_SetRelativeTransform` (`self.BecUp`) (`KismetMathLibrary.TLerp` (`self.Transform Local Up`) (`self.Super Up Transform`) _newtrack_0) false false)
            (`SceneComponent.K2_SetRelativeTransform` (`self.BecBot`) (`KismetMathLibrary.TLerp` (`self.Transform Local Bot`) (`self.Super Bot Transform`) _newtrack_0) false false))
          (:`Finished`
            (set `self.Transform Local Up` (`self.Super Up Transform`))
            (set `self.Transform Local Bot` (`self.Super Bot Transform`))
            (goto _label)))
        (else
          (`TimelineComponent.SetPlayRate` (`self.Bec`) 0.5)
          (set `self.Transform Local Up` (`self.Start Transform Up`))
          (set `self.Transform Local Bot` (`self.Start Transform Bot`))
          (goto _label :!via `Reverse`))))))

(fn `UserConstructionScript`)