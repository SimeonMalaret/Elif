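; BP_PenWall is a wall actor that animates its vertical scale to stretch and shrink.
; On BeginPlay it picks a random peak height and waits a random short delay, so instances vary in size and timing.
; The ScaleZ timeline interpolates Z scale toward that peak while X and Y stay fixed.
; A flag toggled on each finish chooses between playing and reversing the timeline for a ping-pong loop.
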(event `self.ReceiveBeginPlay`
  (set `self.MaxScale` (`KismetMathLibrary.RandomFloatInRange` 0.6 0.7))
  (`KismetSystemLibrary.Delay` (`KismetMathLibrary.RandomFloatInRange` 0.0 1.0))
  (bind (_direction _scalevertical) (`Timeline|ScaleZ` :!label _label)
    (:`Update`
      (`self.SetActorScale3D` (`KismetMathLibrary.MakeVector` 0.5 0.5 (`KismetMathLibrary.Lerp` 0.5 (`self.MaxScale`) _scalevertical))))
    (:`Finished`
      (bind _output_get (set `self.SwitchLoop` (not (`self.SwitchLoop`))))
      (if _output_get
        (goto _label)
        (else
          (goto _label :!via `Reverse`))))))

(fn `UserConstructionScript`)