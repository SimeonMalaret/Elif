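; Destructible wall that, on its first fracture, can open a linked drawbridge and bring down the wall above it.
; BeginPlay resolves a soft-referenced destructible mesh, async loading it if needed, and applies a random material.
; Fracturing adjusts collision, triggers the WallProtector, spawns random particles and destroys the actor after a delay.
; The chain reaction damages the protector-listed wall found at a Z offset above this one.
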(event `self.ReceiveBeginPlay`
  (bind _destructible (`self.Destructible`))
  (bind _destructiblemeshsoftref (`self.DestructibleMeshSoftRef`))
  (bind _destructible_2 (`self.Destructible`))
  (bind _output (`|ConvertAsset` _destructiblemeshsoftref))
  ;[1 1 1] PERSONNE NE TOUCHE À ÇA !!!!!
  (`/Engine/EditorBlueprintResources/StandardMacros.IsValid` _output
    (:`Is Valid`
      (`DestructibleComponent.SetDestructibleMesh` (`self.Destructible`) _output)
      (bind _output_get (set `self.IndexMaterial` (`KismetMathLibrary.RandomInteger` (`KismetArrayLibrary.Array_Length` (`self.MaterialsList`)))))
      (bind _output_2 (`|GetArrayItem` (`self.MaterialsList`) _output_get))
      (`PrimitiveComponent.SetMaterial` _destructible_2 0 _output_2)
      (`PrimitiveComponent.SetMaterial` _destructible_2 4 _output_2))
    (:`Is Not Valid`
      (bind _object (`|LoadAsset` _destructiblemeshsoftref)
        (:`Completed`
          (bind _asdestructible_mesh (cast `DestructibleMesh` _object))
          (`DestructibleComponent.SetDestructibleMesh` (`self.Destructible`) _asdestructible_mesh)
          (bind _output_get_2 (set `self.IndexMaterial` (`KismetMathLibrary.RandomInteger` (`KismetArrayLibrary.Array_Length` (`self.MaterialsList`)))))
          (bind _output_3 (`|GetArrayItem` (`self.MaterialsList`) _output_get_2))
          (`PrimitiveComponent.SetMaterial` _destructible 0 _output_3)
          (`PrimitiveComponent.SetMaterial` _destructible 4 _output_3))))))

(event `self.Destructible.OnComponentFracture`
  (params (HitPoint :type "Vector Structure (by ref)") (HitDirection :type "Vector Structure (by ref)"))
  (bind (_returnvalue_location _returnvalue_rotation _returnvalue_scale) (`KismetMathLibrary.BreakTransform` (`self.GetTransform`)))
  (bind _destructible (`self.Destructible`))
  ;[1 1 1] OnFracture
  (if (not (`self.IsAlreadyDestroyed`))
    (set `self.IsAlreadyDestroyed` true)
    (`|ExecutionSequence`
      (:`then_0`
        (`PrimitiveComponent.SetCollisionResponseToAllChannels` (`self.Cube`) "ECR_Ignore")
        (`PrimitiveComponent.SetCollisionResponseToChannel` _destructible "ECC_GameTraceChannel6" "ECR_Ignore")
        (`PrimitiveComponent.SetCollisionResponseToChannel` _destructible "ECC_WorldStatic" "ECR_Block")
        (bind _bridgetoopen (`self.BridgeToOpen`)
          (:`then`
            (bind _asdraw_bridge_crocodile (cast `/Game/Stigma/Blueprints/DrawBridge/DrawBridge_Crocodile` _bridgetoopen)
              (:`then`
                (`/Game/Stigma/Blueprints/DrawBridge/DrawBridge_Crocodile.StartOpenBridge` _asdraw_bridge_crocodile))
              (:`CastFailed`
                (bind _asdraw_bridge_folder (cast `/Game/Stigma/Blueprints/DrawBridge/DrawBridge_Folder` _bridgetoopen)
                  (:`then`
                    (`/Game/Stigma/Blueprints/DrawBridge/DrawBridge_Folder.StartOpenBridge` _asdraw_bridge_folder))
                  (:`CastFailed`
                    (bind _asdrawbridge_platform (cast `/Game/Stigma/Blueprints/DrawBridge/DrawbridgePlatform` _bridgetoopen)
                      (:`then`
                        (`/Game/Stigma/Blueprints/DrawBridge/DrawbridgePlatform.StartOpenBridge` _asdrawbridge_platform))
                      (:`CastFailed`
                        (bind _asdraw_bridge_emergency_exit (cast `/Game/Stigma/Blueprints/DrawBridge/DrawBridge_EmergencyExit` _bridgetoopen))
                        (`/Game/Stigma/Blueprints/DrawBridge/DrawBridge_EmergencyExit.StartOpenBridge` _asdraw_bridge_emergency_exit))))))))
          (:`else`
            _))
        (`KismetSystemLibrary.Delay` 5.0)
        (`self.K2_DestroyActor`))
      (:`then_1`
        (`self.Find Object In UpwardPosition`))
      (:`then_2`
        (bind _wallprotector (`self.WallProtector`)
          (:`then`
            (`/Game/Stigma/Blueprints/DestructionWall/DestructibleWall.Destruction` _wallprotector)
            (`KismetSystemLibrary.Delay` 0.5)
            (set `/Game/Stigma/Blueprints/DestructionWall/DestructibleWall.Has Destroyed` false _wallprotector))
          (:`else`)))
      (:`then_3`
        (`GameplayStatics.SpawnEmitterAtLocation` (`|GetArrayItem` (`self.Emitter Template`) (`KismetMathLibrary.RandomIntegerInRange` 0 3)) (+ _returnvalue_location (0.0 0.0 250.0)) (struct) (* _returnvalue_scale 3.0))))))

(fn `Find Object In UpwardPosition`
  (locals (`Element to Activate` :type "/Game/Stigma/Blueprints/DestructionWall/DestructiblWall Object Reference"))
  (bind _wallprotector (`self.WallProtector`)
    (:`then`
      (bind _destructiblewalls (`/Game/Stigma/Blueprints/DestructionWall/DestructibleWall.DestructibleWalls` _wallprotector))
      (if (> (`KismetArrayLibrary.Array_Length` _destructiblewalls) 0)
        (for _array_element _destructiblewalls
          (if (`KismetSystemLibrary.IsValid` _array_element)
            (if (== (`self.K2_GetActorLocation` _array_element) (+ (`self.K2_GetActorLocation`) (`KismetMathLibrary.MakeVector` 0.0 0.0 (`self.Z Offset`))) :`ErrorTolerance` 1.0)
              (set `local.Element to Activate` _array_element)
              (break))))
        (bind _element_to_activate (`local.Element to Activate`)
          (:`then`
            (bind _destructible (`/Game/Stigma/Blueprints/DestructionWall/DestructiblWall.Destructible` _element_to_activate)
              (:`then`
                (`DestructibleComponent.ApplyDamage` _destructible 100.0 (`self.K2_GetActorLocation` _element_to_activate) (`KismetMathLibrary.MakeVector` 0.0) 0.0))
              (:`else`)))
          (:`else`))
        (else
          (`KismetSystemLibrary.PrintString` "liste vide"))))
    (:`else`)))

(fn `UserConstructionScript`)