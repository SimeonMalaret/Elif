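; Parent actor for a group of destructible walls that plays shared, one-time feedback when destruction is triggered.
; On BeginPlay it registers itself as each wall's WallProtector and attaches the walls to itself, keeping world transforms.
; Its Destruction event is guarded by HasDestroyed, then starts a strong camera shake through the player character's CameraShakeSource and posts the Wwise wall destruction sound.
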(event `self.ReceiveBeginPlay`
  (for _array_element (`self.DestructibleWalls`)
    (set `/Game/Stigma/Blueprints/DestructiblWall.WallProtector` self _array_element)
    (`self.K2_AttachToActor` _array_element self "None" "KeepWorld" "KeepWorld" "KeepWorld" true)))

(event `Destruction`
  (if (not (`self.Has Destroyed`))
    (set `self.Has Destroyed` true)
    (bind _assecond_gameplay_character (cast `/Game/ThirdPersonCPP/Blueprints/SecondGameplayCharacter` (`GameplayStatics.GetPlayerPawn` 0)))
    (`CameraShakeSourceComponent.StartCameraShake` :`self` (`/Game/ThirdPersonCPP/Blueprints/SecondGameplayCharacter.CameraShakeSource` _assecond_gameplay_character) :`InCameraShake` "/Game/Stigma/Blueprints/CamShake.CamShake_C" :`Scale` 7.0)
    (`AkGameplayStatics.PostEvent` "/Game/Stigma/Sound/Event/LEVELEVENT_WU/Walls/Play_Wall_Destruction.Play_Wall_Destruction" self)))

(fn `UserConstructionScript`)