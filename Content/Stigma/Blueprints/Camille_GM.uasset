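; Camille_GM is a game manager Blueprint that runs level-start setup for Stigma.
; On BeginPlay it finds and stores the level's NarrationManager actor and prints a debug warning about launching in the menu.
; It then checks whether the current level name is in MapToBeginBallWith.
; On those maps it casts the player pawn to SecondGameplayCharacter and, after a short delay, forces a pickup, presumably so play begins holding the ball.
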(event `self.ReceiveBeginPlay`
  (`|ExecutionSequence`
    (:`then_0`
      (bind _returnvalue (`GameplayStatics.GetActorOfClass` "/Game/Stigma/Blueprints/Narration/NarrationManager.NarrationManager_C"))
      (set `self.NarrationManager` _returnvalue)
      (`KismetSystemLibrary.PrintString` "Gamemanager Begin, si lancement dans le menu appeler camille car c'est la merde" true true (struct :`R` 0.838719 :`G` 1.0 :`A` 1.0)))
    (:`then_1`
      (bind _returnvalue_2 (`GameplayStatics.GetCurrentLevelName` true))
      (if (`KismetArrayLibrary.Array_Contains` (`self.Map to Begin Ball With`) _returnvalue_2)
        (`KismetSystemLibrary.PrintString` "Hello")
        (bind _assecond_gameplay_character (cast `/Game/ThirdPersonCPP/Blueprints/SecondGameplayCharacter` (`GameplayStatics.GetPlayerPawn` 0)))
        (`KismetSystemLibrary.Delay` 0.2)
        (`/Game/ThirdPersonCPP/Blueprints/SecondGameplayCharacter.ForcedPickUp` _assecond_gameplay_character)))))

(fn `UserConstructionScript`)