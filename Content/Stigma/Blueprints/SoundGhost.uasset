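; SoundGhost is an actor that carries a Wwise sound along with the player's character.
; On BeginPlay it caches player pawn 0 as a SecondGameplayCharacter and posts the event associated with its Ak component.
; Every Tick it teleports to that character's location without sweep.
; Disconnected leftover nodes would register it with the Camille_GM game mode and print debug strings, but never run.
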(event `self.ReceiveTick`
  (params (DeltaSeconds :type "Float (single-precision)"))
  (bind _player_ (`self.player'`)
    (:`then`
      (`self.K2_SetActorLocation` (`self.K2_GetActorLocation` _player_) false true))
    (:`else`)))

(event `self.ReceiveBeginPlay`
  (bind _assecond_gameplay_character (cast `/Game/ThirdPersonCPP/Blueprints/SecondGameplayCharacter` (`GameplayStatics.GetPlayerPawn` 0))
    (:`then`
      (set `self.player'` _assecond_gameplay_character))
    (:`CastFailed`
      _))
  (`AkGameObject.PostAssociatedAkEvent` :`self` (`self.Ak`)))

(fn `UserConstructionScript`)