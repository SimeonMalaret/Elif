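; BP_DogHouse is a dog house Blueprint that serves as a destination and teleport point for the player's companion.
; Calling the companion changes its controller state and targets this house's Entrance, projected onto the navmesh.
; Teleporting moves the companion, fetched from STIGMA_GM, to the associated dog house's entrance, using a tall navmesh projection extent to find valid ground.
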(event `TeleportToAssociatedDogHouse`
  (`self.K2_SetActorLocation` (`/Game/Stigma/Blueprints/STIGMA_GM.companion` (cast `/Game/Stigma/Blueprints/STIGMA_GM` (`GameplayStatics.GetGameMode`) :!pure true)) (`NavigationSystemV1.K2_ProjectPointToNavigation` (`SceneComponent.K2_GetComponentLocation` (`/Game/Stigma/Blueprints/Niche/BP_DogHouse.Entrance` (`self.Associated DogHouse`))) null null (400.0 400.0 3000.0)) false true))

(event `CallCompanionToDogHouse`
  (bind _companioncontroller (`/Game/Stigma/Blueprints/Companion/BP_Companion.CompanionController` (`/Game/Stigma/Blueprints/STIGMA_GM.companion` (cast `/Game/Stigma/Blueprints/STIGMA_GM` (`GameplayStatics.GetGameMode`) :!pure true))))
  (`/Game/Stigma/Blueprints/Companion/BP_CompanionController.SetCompanionState` _companioncontroller "NewEnumerator5")
  (`/Game/Stigma/Blueprints/Companion/BP_CompanionController.SetTargetLocation` _companioncontroller (`NavigationSystemV1.K2_ProjectPointToNavigation` (`SceneComponent.K2_GetComponentLocation` (`self.Entrance`)))))

(fn `UserConstructionScript`)