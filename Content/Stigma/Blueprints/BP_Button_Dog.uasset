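; BP_Button_Dog is a pressure button that activates game events while actors with the interactible tag rest on it.
; A box overlap counter makes only the first arrival and last departure notify STIGMA_GM with EventName, swap material and message linked cables.
; Tick lerps the button's height toward its base while pressed and back on release.
; IsCableFixOn keeps cables lit; each overlap plays Wwise audio, with click effects on entry.
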(event `self.ReceiveBeginPlay`
  (bind (_returnvalue_x _returnvalue_y _returnvalue_z) (`KismetMathLibrary.BreakVector` (`SceneComponent.K2_GetComponentLocation` (`self.Button`))))
  (set `self.InitPushPosZ` _returnvalue_z)
  (set `self.BaseMat` (`|GetArrayItem` (`MeshComponent.GetMaterials` (`self.Button`)))))

(event `self.Box.OnComponentBeginOverlap`
  (params (OverlappedComponent :type "PrimitiveComponent Object Reference") (OtherActor :type "Actor Object Reference") (OtherComp :type "PrimitiveComponent Object Reference") (OtherBodyIndex :type Integer) (bFromSweep :type Boolean) (SweepResult :type "HitResult Structure (by ref)"))
  (if (`self.ActorHasTag` OtherActor (`self.InteractibleTag`))
    (`AkGameObject.PostAssociatedAkEvent` :`self` (`self.ButtonSoundOn`))
    (bind _returnvalue (`NiagaraFunctionLibrary.SpawnSystemAtLocation` "/Game/Stigma/FX/Particules/Marcus/ClickDog/FX_ClickDog_System.FX_ClickDog_System"))
    (`PrimitiveComponent.SetRenderCustomDepth` _returnvalue true)
    (bind _output_get (set `self.nbObjOnButton` (+ (`self.nbObjOnButton`) 1)))
    (if (== _output_get 1)
      (`/Game/Stigma/Blueprints/STIGMA_GM.ActivationByButton` (cast `/Game/Stigma/Blueprints/STIGMA_GM` (`GameplayStatics.GetGameMode`) :!pure true) (`KismetStringLibrary.ParseIntoArray` (`self.eventName`)))
      (`|ExecutionSequence`
        (:`then_0`
          (bind _output_get_2 (set `self.isPush` true))
          (`PrimitiveComponent.SetMaterial` (`self.Button`) 0 (`self.ValidationMat`))
          (if (`self.debug`)
            (`KismetSystemLibrary.PrintString` (`KismetStringLibrary.Conv_BoolToString` _output_get_2))))
        (:`then_1`
          (if (!= (`KismetArrayLibrary.Array_Length` (`self.Cables`)) 0)
            (message `/Game/Stigma/Blueprints/Cables/ColorCableInterface.ActivationColor` (`self.Cables`))))))))

(event `self.ReceiveTick`
  (params (DeltaSeconds :type "Float (single-precision)"))
  (bind _lerpbuttonpush (`self.lerpButtonPush`))
  (bind _button (`self.Button`))
  (bind _lerpbuttonpush_2 (`self.lerpButtonPush`))
  (bind (_returnvalue_x _returnvalue_y _returnvalue_z) (`KismetMathLibrary.BreakVector` (`SceneComponent.K2_GetComponentLocation` (`self.Base`))))
  (bind (_returnvalue_x_2 _returnvalue_y_2) (`KismetMathLibrary.BreakVector` (`SceneComponent.K2_GetComponentLocation` _button)))
  (bind _returnvalue (* DeltaSeconds (`self.speedPush`)))
  (if (`self.isPush`)
    (set `self.lerpButtonPush` (+ _returnvalue _lerpbuttonpush_2))
    (else
      (set `self.lerpButtonPush` (- _lerpbuttonpush_2 _returnvalue))))
  (if (`self.debug`)
    (`KismetSystemLibrary.PrintString` (`KismetStringLibrary.Conv_DoubleToString` _lerpbuttonpush) true true (struct :`G` 0.66 :`B` 1.0 :`A` 1.0) 0.0))
  (if (and (<= _lerpbuttonpush 1.0) (>= (`self.lerpButtonPush`) 0.0))
    _
    (elif (`self.isPush`)
      (set `self.lerpButtonPush` 1.0)
      (else
        (set `self.lerpButtonPush` 0.0))))
  (`SceneComponent.K2_SetWorldLocation` _button (`KismetMathLibrary.MakeVector` _returnvalue_x_2 _returnvalue_y_2 (`KismetMathLibrary.Lerp` (`self.InitPushPosZ`) _returnvalue_z (`self.lerpButtonPush`))) false false))

(event `self.Box.OnComponentEndOverlap`
  (params (OverlappedComponent :type "PrimitiveComponent Object Reference") (OtherActor :type "Actor Object Reference") (OtherComp :type "PrimitiveComponent Object Reference") (OtherBodyIndex :type Integer))
  (if (`self.ActorHasTag` OtherActor (`self.InteractibleTag`))
    (`AkGameObject.PostAssociatedAkEvent` :`self` (`self.ButtonSoundOut`))
    (bind _output_get (set `self.nbObjOnButton` (- (`self.nbObjOnButton`) 1)))
    (if (== _output_get 0)
      (`/Game/Stigma/Blueprints/STIGMA_GM.UnactivationByButton` (cast `/Game/Stigma/Blueprints/STIGMA_GM` (`GameplayStatics.GetGameMode`) :!pure true) (`KismetStringLibrary.ParseIntoArray` (`self.eventName`)))
      (`|ExecutionSequence`
        (:`then_0`
          (bind _output_get_2 (set `self.isPush` false))
          (`PrimitiveComponent.SetMaterial` (`self.Button`) 0 (`self.BaseMat`))
          (if (`self.debug`)
            (`KismetSystemLibrary.PrintString` (`KismetStringLibrary.Conv_BoolToString` _output_get_2))))
        (:`then_1`
          (if (not (`self.isCableFixOn`))
            (if (!= (`KismetArrayLibrary.Array_Length` (`self.Cables`)) 0)
              (message `/Game/Stigma/Blueprints/Cables/ColorCableInterface.DeactivationColor` (`self.Cables`)))))))))

(fn `UserConstructionScript`)