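; ButtonTrigger is a grabbable Blueprint actor whose Cube component toggles between physics simulation and being held.
; Grabbed disables physics on the Cube and Dropped restores it, with both calling the parent implementation and updating the IsGrab flag.
; While IsGrab is set, Tick teleports the Cube to the DefaultSceneRoot location every frame without sweeping, leaving its rotation untouched.
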(event `self.ReceiveTick`
  (params (DeltaSeconds :type "Float (single-precision)"))
  (if (`self.isGrab`)
    (`SceneComponent.K2_SetWorldLocation` (`self.Cube`) (`SceneComponent.K2_GetComponentLocation` (`self.DefaultSceneRoot`)) false true)))

(fn `Dropped`
  (`PrimitiveComponent.SetSimulatePhysics` (`self.Cube`) true)
  (`parent.Dropped`)
  (set `self.isGrab` false))

(fn `Grabbed`
  (`PrimitiveComponent.SetSimulatePhysics` (`self.Cube`) false)
  (`parent.Grabbed`)
  (set `self.isGrab` true))

(fn `UserConstructionScript`
  (`parent.UserConstructionScript`))