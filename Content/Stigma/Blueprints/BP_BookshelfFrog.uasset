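; BP_BookshelfFrog is a frog prop, presumably bookshelf decor, whose two eyes slide back and forth continuously.
; On BeginPlay it caches both eyes' relative locations and waits a short random delay, so instances can move out of sync.
; The EyesMovement timeline lerps an offset along each eye's local parent X axis, and a toggle on Finished chooses Play or Reverse to keep the motion looping.
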(event `self.ReceiveBeginPlay`
  (set `self.Relative Location EyeR` (`SceneComponent.RelativeLocation` (`self.RightEye`)))
  (set `self.Relative Location EyeL` (`SceneComponent.RelativeLocation` (`self.LeftEye`)))
  (`KismetSystemLibrary.Delay` (`KismetMathLibrary.RandomFloatInRange` 0.0 0.75))
  (bind (_direction _alphalerpeyes) (`Timeline|EyesMovement` :!label _label)
    (:`Update`
      (bind _returnvalue (`KismetMathLibrary.Lerp` 0.0 60.0 _alphalerpeyes))
      (`SceneComponent.K2_SetRelativeLocation` (`self.RightEye`) (- (`self.Relative Location EyeR`) (`KismetMathLibrary.MakeVector` _returnvalue)) false false)
      (`SceneComponent.K2_SetRelativeLocation` (`self.LeftEye`) (- (`self.Relative Location EyeL`) (`KismetMathLibrary.MakeVector` _returnvalue)) false false))
    (:`Finished`
      (bind _output_get (set `self.SwitchMovement` (not (`self.SwitchMovement`))))
      (if _output_get
        (goto _label)
        (else
          (goto _label :!via `Reverse`))))))

(fn `UserConstructionScript`)