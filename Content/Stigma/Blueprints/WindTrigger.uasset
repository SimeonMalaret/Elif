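; WindTrigger is a one-shot trigger that changes the wind when a SecondGameplayCharacter overlaps it.
; A timeline lerps MPC_Wind direction and intensity toward end values, with direction at double alpha.
; A second timeline yaws every BP_FlowerBell to EndRotation, saves that as their OriginalRotation, then destroys the trigger.
; It also sets Interact_Col stationary wind on or off, though that check reads an unset parameter.
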(event `self.ReceiveActorBeginOverlap`
  (params (OtherActor :type "Actor Object Reference"))
  (cast `/Game/ThirdPersonCPP/Blueprints/SecondGameplayCharacter` OtherActor)
  (`|ExecutionSequence`
    (:`then_0`
      ;[1 1 1] SetDirectionnal wind intensity
      (bind _returnvalue (`KismetMaterialLibrary.GetVectorParameterValue` "/Game/Stigma/Foliage_Grass/MPC_Wind.MPC_Wind" "Wind Direction"))
      (bind _returnvalue_2 (`KismetMaterialLibrary.GetScalarParameterValue` "/Game/Stigma/Foliage_Grass/MPC_Wind.MPC_Wind" "Wind Intensity"))
      (bind (_direction _windlerp) (`Timeline|Wind Transition` :!via `PlayFromStart`)
        (:`Update`
          (`KismetMaterialLibrary.SetVectorParameterValue` "/Game/Stigma/Foliage_Grass/MPC_Wind.MPC_Wind" "Wind Direction" (`KismetMathLibrary.LinearColorLerp` _returnvalue (`self.WindEndDirection`) (* _windlerp 2.0)))
          (`KismetMaterialLibrary.SetScalarParameterValue` "/Game/Stigma/Foliage_Grass/MPC_Wind.MPC_Wind" "Wind Intensity" (`KismetMathLibrary.Lerp` _returnvalue_2 (`self.WindEndIntensity`) _windlerp)))))
    (:`then_1`
      ;[1 1 1] Rotate Every FlowerBells
      (bind (_direction_2 _flowerrotation) (`Timeline|Flower Rotation`)
        (:`Update`
          (bind _outactors (`GameplayStatics.GetAllActorsOfClass` "/Game/Stigma/FlowerBell/BP_FlowerBell.BP_FlowerBell_C"))
          (for _array_element _outactors
            (bind (_returnvalue_roll _returnvalue_pitch) (`KismetMathLibrary.BreakRotator` (`self.K2_GetActorRotation` _array_element)))
            (`self.K2_SetActorRotation` _array_element (`KismetMathLibrary.MakeRotator` _returnvalue_roll _returnvalue_pitch (`KismetMathLibrary.Lerp` (`/Game/Stigma/FlowerBell/BP_FlowerBell.OriginalRotation` _array_element) (`self.EndRotation`) _flowerrotation)) true)))
        (:`Finished`
          (bind _outactors_2 (`GameplayStatics.GetAllActorsOfClass` "/Game/Stigma/FlowerBell/BP_FlowerBell.BP_FlowerBell_C"))
          (for _array_element_2 _outactors_2
            (bind (_returnvalue_roll_2 _returnvalue_pitch_2 _returnvalue_yaw) (`KismetMathLibrary.BreakRotator` (`self.K2_GetActorRotation` _array_element_2)))
            (set `/Game/Stigma/FlowerBell/BP_FlowerBell.OriginalRotation` _returnvalue_yaw _array_element_2))
          (`self.K2_DestroyActor`))))
    (:`then_2`
      ;[1 1 1] Stationnary Wind
      (bind _returnvalue_3 (`KismetMaterialLibrary.GetScalarParameterValue` null))
      (if (== _returnvalue_3 0.0)
        (`KismetMaterialLibrary.SetScalarParameterValue` "/Game/Stigma/Foliage_Grass/Interact_Col.Interact_Col" "Wind_Intensity" 0.5)
        (`KismetMaterialLibrary.SetScalarParameterValue` "/Game/Stigma/Foliage_Grass/Interact_Col.Interact_Col" "Wind_Weight" 0.5)
        (else
          (`KismetMaterialLibrary.SetScalarParameterValue` "/Game/Stigma/Foliage_Grass/Interact_Col.Interact_Col" "Wind_Intensity")
          (`KismetMaterialLibrary.SetScalarParameterValue` "/Game/Stigma/Foliage_Grass/Interact_Col.Interact_Col" "Wind_Weight"))))))

(fn `UserConstructionScript`)