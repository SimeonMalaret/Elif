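; Target actor that reacts to being hit by a Ball, optionally patrolling back and forth between two reference actors at distance-normalized speed until activated.
; Each Ball overlap sends its EventName to Camille_GM's button activation and plays a timeline easing it toward ActivePosition.
; The first hit also stops the patrol, forces the character to retrieve the ball, plays the FlowerBell Wwise event, starts narration and spins the target's pitch.
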(event `self.ReceiveBeginPlay`
  (set `self.InitRotation` (`self.K2_GetActorRotation`))
  (if (`self.canMove`)
    (set `self.speed` (/ (* 100 (`self.speed`)) (`KismetMathLibrary.Vector_Distance` (`self.K2_GetActorLocation` (`self.moveFrom`)) (`self.K2_GetActorLocation` (`self.moveTo`)))))))

(event `self.ReceiveActorBeginOverlap`
  (params (OtherActor :type "Actor Object Reference"))
  (bind (_initrotation_roll _initrotation_pitch _initrotation_yaw) (`KismetMathLibrary.BreakRotator` (`self.InitRotation`)))
  (cast `/Game/Stigma/Blueprints/Ball` OtherActor)
  (bind _ascamille_gm (cast `/Game/Stigma/Blueprints/Camille_GM` (`GameplayStatics.GetGameMode`)))
  (`/Game/Stigma/Blueprints/Camille_GM.ActivationByButton` _ascamille_gm (`KismetStringLibrary.ParseIntoArray` (`self.eventName`)))
  (`|ExecutionSequence`
    (:`then_0`
      (bind (_direction _position) (`Timeline|Activation`)
        (:`Update`
          (`self.K2_SetActorLocation` (`KismetMathLibrary.VLerp` (`self.K2_GetActorLocation`) (`self.activePosition`) _position)))))
    (:`then_1`
      (if (not (`self.isActivate`))
        (bind _character (`/Game/Stigma/Blueprints/Camille_GM.character` _ascamille_gm)
          (:`then`
            (`/Game/ThirdPersonCPP/Blueprints/SecondGameplayCharacter.ForceGetBackBall` _character true))
          (:`else`
            _))
        (`AkGameplayStatics.PostEvent` "/Game/Stigma/Sound/flowerBell.flowerBell" self)
        (set `self.isActivate` true)
        (`|ExecutionSequence`
          (:`then_0`
            (bind _ascamille_gm_2 (cast `/Game/Stigma/Blueprints/Camille_GM` (`GameplayStatics.GetGameMode`)))
            (bind _narrationmanager (`/Game/Stigma/Blueprints/Camille_GM.NarrationManager` _ascamille_gm_2)
              (:`then`
                (`/Game/Stigma/Blueprints/Narration/NarrationManager.StartNarration` _narrationmanager (`self.Index To Play`) null))
              (:`else`)))
          (:`then_1`
            ;[1 1 1] debug
            (if (`self.debug`)
              (`KismetSystemLibrary.PrintString` "cible toucher")))
          (:`then_2`
            (bind (_direction_2 _position_2) (`Timeline|Timeline_0`)
              (:`Update`
                (`self.K2_SetActorRelativeRotation` (`KismetMathLibrary.MakeRotator` _initrotation_roll (+ _initrotation_pitch (* 360 _position_2)) _initrotation_yaw))))))))))

(event `self.ReceiveTick`
  (params (DeltaSeconds :type "Float (single-precision)"))
  (bind _returnvalue (* DeltaSeconds (`self.speed`)))
  (if (not (`self.isActivate`))
    (if (`self.canMove`)
      (if (`self.moveRight`)
        (bind _output_get (set `self.lerpPos` (+ (`self.lerpPos`) _returnvalue)))
        (if (>= _output_get 1.0)
          (set `self.lerpPos` 1.0)
          (set `self.moveRight` (not (`self.moveRight`)) :!label _label))
        (else
          (bind _output_get_2 (set `self.lerpPos` (- (`self.lerpPos`) _returnvalue)))
          (if (<= _output_get_2 0.0)
            (set `self.lerpPos` 0.0)
            (goto _label)
            (else
              _))))
      (`self.K2_SetActorLocation` (`KismetMathLibrary.VLerp` (`self.K2_GetActorLocation` (`self.moveFrom`)) (`self.K2_GetActorLocation` (`self.moveTo`)) (`self.lerpPos`)) false true))))

(fn `UserConstructionScript`)