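; Death zone that teleports a SecondGameplayCharacter to a respawn point when it enters the box.
; On overlap it hides the character's mesh, spawns a scaled-up explosion at its location, moves it to the LocationRespawn actor and shows the mesh again.
; All steps run in the same frame: the DelayRespawn delay node has no incoming execution, so it never runs.
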(event `self.Box.OnComponentBeginOverlap`
  (params (OverlappedComponent :type "PrimitiveComponent Object Reference") (OtherActor :type "Actor Object Reference") (OtherComp :type "PrimitiveComponent Object Reference") (OtherBodyIndex :type Integer) (bFromSweep :type Boolean) (SweepResult :type "HitResult Structure (by ref)"))
  (bind _assecond_gameplay_character (cast `/Game/ThirdPersonCPP/Blueprints/SecondGameplayCharacter` OtherActor))
  (`SceneComponent.SetVisibility` (`Character.Mesh` _assecond_gameplay_character) false false)
  (`GameplayStatics.SpawnEmitterAtLocation` "/Game/StarterContent/Particles/P_Explosion.P_Explosion" (`self.K2_GetActorLocation` _assecond_gameplay_character) (struct) (3.0 3.0 3.0))
  (`self.K2_SetActorLocation` _assecond_gameplay_character (`self.K2_GetActorLocation` (`self.Location respawn`)) false true)
  (`SceneComponent.SetVisibility` (`Character.Mesh` _assecond_gameplay_character) true true))

(fn `UserConstructionScript`)