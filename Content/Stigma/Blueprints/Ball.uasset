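; Thrown ball actor that draws the companion to where it bounces.
; On each sphere hit above a minimum projectile speed, it prints the speed and projects its location onto the navmesh.
; If that succeeds and a BP_Companion exists, it sends the companion to the projected point and posts a Wwise bounce event, so the sound depends on both checks.
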(event `self.Sphere.OnComponentHit`
  (params (HitComponent :type "PrimitiveComponent Object Reference") (OtherActor :type "Actor Object Reference") (OtherComp :type "PrimitiveComponent Object Reference") (NormalImpulse :type "Vector Structure") (Hit :type "HitResult Structure (by ref)"))
  (bind (_projectedlocation _returnvalue) (`NavigationSystemV1.K2_ProjectPointToNavigation` (`self.K2_GetActorLocation`) null null (100.0 100.0 100.0)))
  (bind _returnvalue_2 (`KismetMathLibrary.VSize` (`MovementComponent.Velocity` (`self.ProjectileMovement`))))
  (`|ExecutionSequence`
    (:`then_0`
      (if (> _returnvalue_2 200.0)
        (`KismetSystemLibrary.PrintString` (`KismetStringLibrary.Conv_DoubleToString` _returnvalue_2))
        (if _returnvalue
          (bind _returnvalue_3 (`GameplayStatics.GetActorOfClass` "/Game/Stigma/Blueprints/Companion/BP_Companion.BP_Companion_C"))
          (if (`KismetSystemLibrary.IsValid` _returnvalue_3)
            (`/Game/Stigma/Blueprints/Companion/BP_Companion.MoveTo` _returnvalue_3 _projectedlocation)
            (`AkGameplayStatics.PostEvent` "/Game/Stigma/Sound/Event/Marrec_Events_WU/LEVEL/PROPS/ThrowBall/Play_ThrowBall_Bounce.Play_ThrowBall_Bounce" self)))))))

(fn `UserConstructionScript`)