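; Moving cushion platform that shuttles between two points and sinks while the SecondGameplayCharacter stands on it.
; BeginPlay converts both offsets to world space, then a duration-scaled timeline lerps the actor between them, reversing whenever it finishes.
; A second timeline lowers the mesh relative to the actor when the character overlaps the Cylinder, and reverses when it leaves.
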(event `self.ReceiveBeginPlay`
  (bind _returnvalue_location (`KismetMathLibrary.BreakTransform` (`KismetMathLibrary.ComposeTransforms` (`KismetMathLibrary.Conv_VectorToTransform` (`self.Location_1`)) (`self.GetTransform`))))
  (bind _returnvalue_location_2 (`KismetMathLibrary.BreakTransform` (`KismetMathLibrary.ComposeTransforms` (`KismetMathLibrary.Conv_VectorToTransform` (`self.Location_2`)) (`self.GetTransform`))))
  (set `self.StartPosition` (`SceneComponent.RelativeLocation` (`self.StaticMesh`)))
  (set `self.Location_1` _returnvalue_location)
  (set `self.Location_2` _returnvalue_location_2)
  (`TimelineComponent.SetPlayRate` (`self.Timeline_1`) (/ 1.0 (`self.Duration`)))
  (bind (_direction _lerpdeltatime) (`Timeline|Timeline_1` :!label _label)
    (:`Update`
      (`self.K2_SetActorLocation` (`KismetMathLibrary.VLerp` (`self.Location_1`) (`self.Location_2`) _lerpdeltatime)))
    (:`Finished`
      (bind _output_get (set `self.ForwardTime` (not (`self.ForwardTime`))))
      (if _output_get
        (goto _label)
        (else
          (goto _label :!via `Reverse`))))))

(event `self.Cylinder.OnComponentBeginOverlap`
  (params (OverlappedComponent :type "PrimitiveComponent Object Reference") (OtherActor :type "Actor Object Reference") (OtherComp :type "PrimitiveComponent Object Reference") (OtherBodyIndex :type Integer) (bFromSweep :type Boolean) (SweepResult :type "HitResult Structure (by ref)"))
  (bind _startposition (`self.StartPosition`))
  (cast `/Game/ThirdPersonCPP/Blueprints/SecondGameplayCharacter` OtherActor)
  (bind (_direction _newtrack_0) (`Timeline|Timeline_0` :!label _label_2)
    (:`Update`
      (`SceneComponent.K2_SetRelativeLocation` (`self.StaticMesh`) (`KismetMathLibrary.VLerp` _startposition (- _startposition (0.0 0.0 30.0)) _newtrack_0) false false))))

(event `self.Cylinder.OnComponentEndOverlap`
  (params (OverlappedComponent :type "PrimitiveComponent Object Reference") (OtherActor :type "Actor Object Reference") (OtherComp :type "PrimitiveComponent Object Reference") (OtherBodyIndex :type Integer))
  (cast `/Game/ThirdPersonCPP/Blueprints/SecondGameplayCharacter` OtherActor)
  (goto _label_2 :!via `Reverse`))

(fn `UserConstructionScript`)