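; Trigger volume that changes the player's gameplay camera when the SecondGameplayCharacter overlaps it.
; Boolean flags enable four actions: switch to an assigned camera, retarget, toggle a rail camera's lock, or change its follow distance.
; Each action toggles on re-entry, restoring the stored previous camera, player target or previous distance.
; Switches carry the target point's location over and flag the incoming camera as in transit.
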(event `self.ReceiveActorBeginOverlap`
  (params (OtherActor :type "Actor Object Reference"))
  (bind _assecond_gameplay_character (cast `/Game/ThirdPersonCPP/Blueprints/SecondGameplayCharacter` OtherActor))
  (if (`self.switch`)
    (`self.SwicthCam` _assecond_gameplay_character))
  (`|ExecutionSequence`
    (:`then_0`
      (if (`self.target`)
        (`self.TargetCam` _assecond_gameplay_character)
        (bind _ascamera_static (cast `/Game/ThirdPersonCPP/Blueprints/Francois/CameraStatic` (`/Game/ThirdPersonCPP/Blueprints/SecondGameplayCharacter.CurrentCamera` _assecond_gameplay_character)))))
    (:`then_1`
      (if (`self.lock`)
        (`self.LockCam` _assecond_gameplay_character)))
    (:`then_2`
      (if (`self.distCam`)
        (`self.DistanceCam` _assecond_gameplay_character)))))

(event `self.ReceiveBeginPlay`
  (set `self.DistanceVar` (`self.New Distance To Player`)))

(event `/Game/Stigma/Blueprints/Camera/CamTriggerInterface.Reset`
  (if (`self.switch`)
    (set `self.PreviousCam` null)
    (set `self.DistanceVar` (`self.New Distance To Player`))))

(event `LockCam`
  (params (caracter :type "/Game/ThirdPersonCPP/Blueprints/SecondGameplayCharacter Object Reference"))
  ;[1 1 1] lock
  (bind _ascamera_rail (cast `/Game/ThirdPersonCPP/Blueprints/Francois/CameraRail` (`/Game/ThirdPersonCPP/Blueprints/SecondGameplayCharacter.CurrentCamera` caracter)))
  (if (`/Game/ThirdPersonCPP/Blueprints/Francois/CameraRail.IsLock` _ascamera_rail)
    (set `/Game/ThirdPersonCPP/Blueprints/Francois/CameraRail.IsLock` false _ascamera_rail)
    (else
      (set `/Game/ThirdPersonCPP/Blueprints/Francois/CameraRail.IsLock` true _ascamera_rail))))

(event `SwicthCam`
  (params (caracter :type "/Game/ThirdPersonCPP/Blueprints/SecondGameplayCharacter Object Reference"))
  (bind _previouscam (`self.PreviousCam`))
  (bind _currentcamera (`/Game/ThirdPersonCPP/Blueprints/SecondGameplayCharacter.CurrentCamera` caracter))
  (bind _camera_for_switch (`self.Camera for switch`))
  (bind _followcamera (`DreamHuntersCharacter.FollowCamera` caracter))
  (bind _returnvalue (`SceneComponent.K2_GetComponentLocation` (`/Game/ThirdPersonCPP/Blueprints/Francois/CameraStatic.TargetPoint` _previouscam)))
  ;[1 1 1] switch
  (if (!= _currentcamera _camera_for_switch)
    (bind _ascamera_static (cast `/Game/ThirdPersonCPP/Blueprints/Francois/CameraStatic` _currentcamera))
    (bind _output_get (set `self.PreviousCam` _ascamera_static))
    (message `/Game/ThirdPersonCPP/Blueprints/Francois/CameraInterface.Deactivate Camera` _currentcamera)
    (bind _output_get_2 (set `/Game/ThirdPersonCPP/Blueprints/SecondGameplayCharacter.CurrentCamera` _camera_for_switch caracter))
    (bind _ascamera_static_2 (cast `/Game/ThirdPersonCPP/Blueprints/Francois/CameraStatic` _output_get_2))
    (`SceneComponent.K2_SetWorldLocation` (`/Game/ThirdPersonCPP/Blueprints/Francois/CameraStatic.TargetPoint` _ascamera_static_2) (`SceneComponent.K2_GetComponentLocation` (`/Game/ThirdPersonCPP/Blueprints/Francois/CameraStatic.TargetPoint` _output_get)) false false)
    (set `/Game/ThirdPersonCPP/Blueprints/Francois/CameraStatic.isInTransit` true _camera_for_switch)
    (message `/Game/ThirdPersonCPP/Blueprints/Francois/CameraInterface.Activate Camera` _camera_for_switch _followcamera caracter)
    (elif (`self.target`)
      (message `/Game/ThirdPersonCPP/Blueprints/Francois/CameraInterface.Deactivate Camera` _currentcamera)
      (bind _output_get_3 (set `/Game/ThirdPersonCPP/Blueprints/SecondGameplayCharacter.CurrentCamera` _previouscam caracter))
      (bind _ascamera_static_3 (cast `/Game/ThirdPersonCPP/Blueprints/Francois/CameraStatic` _output_get_3))
      (`SceneComponent.K2_SetWorldLocation` (`/Game/ThirdPersonCPP/Blueprints/Francois/CameraStatic.TargetPoint` _ascamera_static_3) _returnvalue false false)
      (set `/Game/ThirdPersonCPP/Blueprints/Francois/CameraStatic.isInTransit` true _previouscam)
      (message `/Game/ThirdPersonCPP/Blueprints/Francois/CameraInterface.Activate Camera` _previouscam _followcamera (`self.NewTarget for camera`))
      (else
        (message `/Game/ThirdPersonCPP/Blueprints/Francois/CameraInterface.Deactivate Camera` _currentcamera)
        (bind _output_get_4 (set `/Game/ThirdPersonCPP/Blueprints/SecondGameplayCharacter.CurrentCamera` _previouscam caracter))
        (bind _ascamera_static_4 (cast `/Game/ThirdPersonCPP/Blueprints/Francois/CameraStatic` _output_get_4))
        (`SceneComponent.K2_SetWorldLocation` (`/Game/ThirdPersonCPP/Blueprints/Francois/CameraStatic.TargetPoint` _ascamera_static_4) _returnvalue false false)
        (set `/Game/ThirdPersonCPP/Blueprints/Francois/CameraStatic.isInTransit` true _previouscam)
        (message `/Game/ThirdPersonCPP/Blueprints/Francois/CameraInterface.Activate Camera` _previouscam _followcamera caracter)))))

(event `TargetCam`
  (params (caracter :type "/Game/ThirdPersonCPP/Blueprints/SecondGameplayCharacter Object Reference"))
  (bind _newtarget_for_camera (`self.NewTarget for camera`))
  ;[1 1 1] target
  (bind _ascamera_static (cast `/Game/ThirdPersonCPP/Blueprints/Francois/CameraStatic` (`/Game/ThirdPersonCPP/Blueprints/SecondGameplayCharacter.CurrentCamera` caracter)))
  (if (`KismetSystemLibrary.IsValid` _newtarget_for_camera)
    (if (!= (`/Game/ThirdPersonCPP/Blueprints/Francois/CameraStatic.Target` _ascamera_static) (`self.NewTarget for camera`))
      (set `/Game/ThirdPersonCPP/Blueprints/Francois/CameraStatic.Target` _newtarget_for_camera _ascamera_static)
      (else
        (set `/Game/ThirdPersonCPP/Blueprints/Francois/CameraStatic.Target` (`GameplayStatics.GetPlayerCharacter` 0) _ascamera_static :!label _label)))
    (else
      (goto _label))))

(event `DistanceCam`
  (params (caracter :type "/Game/ThirdPersonCPP/Blueprints/SecondGameplayCharacter Object Reference"))
  ;[1 1 1] distance trigger
  (bind _ascamera_rail (cast `/Game/ThirdPersonCPP/Blueprints/Francois/CameraRail` (`/Game/ThirdPersonCPP/Blueprints/SecondGameplayCharacter.CurrentCamera` caracter)))
  (`/Game/ThirdPersonCPP/Blueprints/Francois/CameraRail.ChangeDistance` _ascamera_rail (`self.DistanceVar`))
  (set `self.DistanceVar` (`/Game/ThirdPersonCPP/Blueprints/Francois/CameraRail.DistanceToPlayer` _ascamera_rail)))

(fn `UserConstructionScript`)