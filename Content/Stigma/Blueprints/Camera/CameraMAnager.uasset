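; CameraMAnager is a manager Blueprint that centralizes tuning for the game's static cameras.
; On BeginPlay it gathers every actor implementing CameraInterface, casts each to CameraStatic and copies in its own speed, offset and no-move radius settings.
; The loop body exits for any actor that fails the cast, and the manager does nothing after this initial push.
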(event `self.ReceiveBeginPlay`
  (bind _outactors (`GameplayStatics.GetAllActorsWithInterface` "/Game/ThirdPersonCPP/Blueprints/Francois/CameraInterface.CameraInterface_C"))
  (for _array_element _outactors
    (bind _ascamera_static (cast `/Game/ThirdPersonCPP/Blueprints/Francois/CameraStatic` _array_element))
    (set `/Game/ThirdPersonCPP/Blueprints/Francois/CameraStatic.CameraSpeedMove` (`self.CameraSpeedMove`) _ascamera_static)
    (set `/Game/ThirdPersonCPP/Blueprints/Francois/CameraStatic.CameraSpeedImmobile` (`self.CameraSpeedImmobile`) _ascamera_static)
    (set `/Game/ThirdPersonCPP/Blueprints/Francois/CameraStatic.CameraSpeedOrientation` (`self.CameraSpeedOrientation`) _ascamera_static)
    (set `/Game/ThirdPersonCPP/Blueprints/Francois/CameraStatic.CameraOffsetMove` (`self.CameraOffsetMove`) _ascamera_static)
    (set `/Game/ThirdPersonCPP/Blueprints/Francois/CameraStatic.CameraOffsetImmobile` (`self.CameraOffsetImmobile`) _ascamera_static)
    (set `/Game/ThirdPersonCPP/Blueprints/Francois/CameraStatic.CameraOffsetUp` (`self.CameraOffsetUp`) _ascamera_static)
    (set `/Game/ThirdPersonCPP/Blueprints/Francois/CameraStatic.radiusNoMove` (`self.RadiusNoMove`) _ascamera_static)))

(fn `UserConstructionScript`)