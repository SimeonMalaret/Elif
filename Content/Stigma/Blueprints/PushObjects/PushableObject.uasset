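; Pushable object actor that, on interact, snaps the character to a push spot and starts a push through the character's PushComponent.
; The construction script previews each PushTransforms entry as an arrow.
; Interaction picks the nearest transform within PushRange, then rejects it if capsule and line traces find an overlap, unwalkable floor or blocked path.
; Failures print a red reason, and debug shapes show the checks.
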(event `/Game/Stigma/Blueprints/PushObjects/InteractInterface.OnInteract`
  (params (Player :type "/Game/ThirdPersonCPP/Blueprints/SecondGameplayCharacter Object Reference"))
  (`self.HandleInteraction` Player))

(fn `FindClosestPushTransformIndex`
  (params (CharacterLocation :type "Vector2D Structure") (PushRange :type "Float (double-precision)"))
  (returns (BestIndex :type Integer))
  (locals (`Current Transform Index` :type Integer) (`Closest Transform Index` :type Integer :default -1) (`Current DistanceSq` :type "Float (double-precision)" :default 0.0) (`Closest DistanceSq` :type "Float (double-precision)"))
  (for (_array_element _array_index) (`self.Push Transforms`)
    (set `local.Current Transform Index` _array_index)
    (bind _output_get (set `local.Current DistanceSq` (`KismetMathLibrary.DistanceSquared2D` (`KismetMathLibrary.Conv_VectorToVector2D` (`KismetMathLibrary.TransformLocation` (`self.GetTransform`) (.location _array_element))) (`local.CharacterLocation`))))
    (if (< _output_get (`KismetMathLibrary.Square` (`local.PushRange`)))
      (if (or (< (`local.Current DistanceSq`) (`local.Closest DistanceSq`)) (< (`local.Closest Transform Index`) 0))
        (set `local.Closest Transform Index` (`local.Current Transform Index`))
        (set `local.Closest DistanceSq` (`local.Current DistanceSq`)))))
  (return (`local.Closest Transform Index`)))

(fn `HandleInteraction`
  (params (Character :type "/Game/ThirdPersonCPP/Blueprints/SecondGameplayCharacter Object Reference"))
  (locals (PushComponent :type "/Game/Stigma/Blueprints/PushObjects/PushComponent Object Reference") (`Character New Transform` :type "Transform Structure"))
  (bind _character (`local.Character`))
  (bind _character_new_transform_location (`KismetMathLibrary.BreakTransform` (`local.Character New Transform`)))
  (bind _character_new_transform_location_2 (`KismetMathLibrary.BreakTransform` (`local.Character New Transform`)))
  (bind _capsulecomponent (`Character.CapsuleComponent` (`local.Character`)))
  (`/Engine/EditorBlueprintResources/StandardMacros.IsValid` Character
    (:`Is Valid`
      (bind _output_get (set `local.PushComponent` (`self.GetComponentByClass` Character "/Game/Stigma/Blueprints/PushObjects/PushComponent.PushComponent_C")))
      (`/Engine/EditorBlueprintResources/StandardMacros.IsValid` _output_get
        (:`Is Valid`
          (bind _bestindex (`self.FindClosestPushTransformIndex` (`KismetMathLibrary.Conv_VectorToVector2D` (`self.K2_GetActorLocation` (`local.Character`))) (`/Game/Stigma/Blueprints/PushObjects/PushComponent.PushRange` (`local.PushComponent`))))
          (if (>= _bestindex 0)
            (bind (_returnvalue_location _returnvalue_rotation) (`KismetMathLibrary.BreakTransform` (`KismetMathLibrary.ComposeTransforms` (`|GetArrayItem` (`self.Push Transforms`) _bestindex) (`self.GetTransform`))))
            (bind _returnvalue (+ _returnvalue_location (`KismetMathLibrary.MakeVector` 0.0 0.0 (`CapsuleComponent.GetScaledCapsuleHalfHeight` (`Character.CapsuleComponent` _character)))))
            (set `local.Character New Transform` (`KismetMathLibrary.MakeTransform` _returnvalue _returnvalue_rotation (`self.GetActorScale3D` _character)))
            (`KismetSystemLibrary.DrawDebugSphere` _returnvalue 20.0 12 (struct :`R` 1.0 :`G` 1.0 :`A` 1.0) 2.0 1.0)
            (bind _outhit (`KismetSystemLibrary.CapsuleTraceSingle` :`Start` (+ _character_new_transform_location_2 (0.0 0.0 70.0)) :`End` (- _character_new_transform_location_2 (0.0 0.0 100.0)) :`Radius` (`CapsuleComponent.GetScaledCapsuleRadius` _capsulecomponent) :`HalfHeight` (`CapsuleComponent.GetScaledCapsuleHalfHeight` _capsulecomponent) :`TraceChannel` "TraceTypeQuery1" :`DrawDebugType` "ForDuration" :`DrawTime` 2.0))
            (bind (_bblockinghit _binitialoverlap _time _distance _location _impactpoint _normal _impactnormal) (`GameplayStatics.BreakHitResult` _outhit))
            (if (not _binitialoverlap)
              (if (< (`CharacterMovementComponent.K2_GetWalkableFloorZ` (`Character.CharacterMovement` (`local.Character`))) (.z _impactnormal))
                (bind (_outhit_2 _returnvalue_2) (`KismetSystemLibrary.LineTraceSingle` (`self.K2_GetActorLocation`) _character_new_transform_location "TraceTypeQuery1" false (`|MakeArray` (`local.Character`) :!type "Actor Object Reference") "ForDuration" true (struct :`R` 1.0 :`A` 1.0) (struct :`G` 1.0 :`A` 1.0) 2.0))
                (if (not _returnvalue_2)
                  (`self.K2_SetActorTransform` (`local.Character`) (`local.Character New Transform`) false false)
                  (`/Game/Stigma/Blueprints/PushObjects/PushComponent.BeginPush` (`local.PushComponent`) self)
                  (else
                    (`self.PushFailedInfo` "Object between player and push object")))
                (else
                  (`self.PushFailedInfo` "Floor not walkable")))
              (else
                (`self.PushFailedInfo` "Something in the way")))
            (else
              (`self.PushFailedInfo` "No push transform bound"))))
        (:`Is Not Valid`
          (`self.PushFailedInfo` "Character does not have push component"))))
    (:`Is Not Valid`
      (`self.PushFailedInfo` "Character not valid"))))

(fn `UserConstructionScript`
  (for _array_element (`self.Push Transforms`)
    (`AddComponent|NODE_AddArrowComponent-0` :`RelativeTransform` _array_element)))