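; Pushable object actor that snaps an interacting character to one of its predefined push points and starts a push.
; The construction script adds an arrow for each push transform.
; On interaction it picks the nearest point within the character's PushComponent range, validates space, walkable floor and no wall via capsule and line traces.
; It then teleports the character there and calls BeginPush, or prints the failure reason.
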(event `/Game/Stigma/Blueprints/PushObjects/InteractInterface.OnInteracted`
  (params (Player :type "/Game/ThirdPersonCPP/Blueprints/SecondGameplayCharacter Object Reference"))
  (`self.HandleInteraction` Player))

(fn `FindClosestPushTransformIndex`
  (params (CharacterPosition :type "Vector2D Structure") (PushRange :type "Float (double-precision)"))
  (returns (ClosestIndex :type Integer))
  (locals (CurrentTransformIndex :type Integer) (CurrentDistanceSqr :type "Float (double-precision)" :default 0.0) (ClosestDistanceSqr :type "Float (double-precision)" :default 1000000.0) (ClosestTransformIndex :type Integer :default -1))
  (for (_array_element _array_index) (`self.PushTranform`)
    (set `local.CurrentTransformIndex` _array_index)
    (bind _output_get (set `local.CurrentDistanceSqr` (`KismetMathLibrary.DistanceSquared2D` (`KismetMathLibrary.Conv_VectorToVector2D` (`KismetMathLibrary.TransformLocation` (`self.GetTransform`) (.location _array_element))) (`local.CharacterPosition`))))
    (if (< _output_get (`KismetMathLibrary.Square` (`local.PushRange`)))
      (if (< (`local.CurrentDistanceSqr`) (`local.ClosestDistanceSqr`))
        (set `local.ClosestTransformIndex` (`local.CurrentTransformIndex`))
        (set `local.ClosestDistanceSqr` (`local.CurrentDistanceSqr`)))))
  (return (`local.ClosestTransformIndex`)))

(fn `HandleInteraction`
  (params (Character :type "/Game/ThirdPersonCPP/Blueprints/SecondGameplayCharacter Object Reference"))
  (locals (PlayerPreviousTransform :type "Transform Structure") (PlayerNewTransform :type "Transform Structure") (IndexTransform :type Integer :default 0))
  (bind _playernewtransform_location (`KismetMathLibrary.BreakTransform` (`local.PlayerNewTransform`)))
  (bind _character (`local.Character`))
  (bind _playernewtransform_location_2 (`KismetMathLibrary.BreakTransform` (`local.PlayerNewTransform`)))
  (bind _character_2 (`local.Character`))
  (bind _character_3 (`local.Character`))
  (bind _output_location (`KismetMathLibrary.BreakTransform` (`|GetArrayItem` (`self.PushTranform`) (`local.IndexTransform`))))
  (bind _capsulecomponent (`Character.CapsuleComponent` _character))
  (`/Engine/EditorBlueprintResources/StandardMacros.IsValid` Character
    (:`Is Valid`
      (bind _output_get (set `self.PushComponent` (`self.GetComponentByClass` Character "/Game/Stigma/Blueprints/PushObjects/PushComponent.PushComponent_C")))
      (`/Engine/EditorBlueprintResources/StandardMacros.IsValid` _output_get
        (:`Is Valid`
          (set `local.PlayerPreviousTransform` (`self.GetTransform` (`local.Character`)))
          (bind _closestindex (`self.FindClosestPushTransformIndex` (`KismetMathLibrary.Conv_VectorToVector2D` (`self.K2_GetActorLocation` (`local.Character`))) (`/Game/Stigma/Blueprints/PushObjects/PushComponent.PushRange` (`self.PushComponent`))))
          (bind _output_get_2 (set `local.IndexTransform` _closestindex))
          (if (>= _output_get_2 0)
            (bind (_returnvalue_location _returnvalue_rotation) (`KismetMathLibrary.BreakTransform` (`KismetMathLibrary.ComposeTransforms` (`|GetArrayItem` (`self.PushTranform`) _output_get_2) (`self.GetTransform`))))
            (bind _returnvalue (+ _returnvalue_location (`KismetMathLibrary.MakeVector` 0.0 0.0 (`CapsuleComponent.GetScaledCapsuleHalfHeight` (`Character.CapsuleComponent` (`local.Character`))))))
            (set `local.PlayerNewTransform` (`KismetMathLibrary.MakeTransform` _returnvalue _returnvalue_rotation (`SceneComponent.K2_GetComponentScale` (`Character.CapsuleComponent` _character_3))))
            (if (not (not (`/Game/ThirdPersonCPP/Blueprints/SecondGameplayCharacter.DEBUG` _character_3)))
              (`KismetSystemLibrary.DrawDebugSphere` _returnvalue 20.0 12 (struct :`B` 1.0 :`A` 1.0) 2.0 1.0))
            (bind _outhit (`KismetSystemLibrary.CapsuleTraceSingle` (+ _playernewtransform_location (0.0 0.0 70.0)) (- _playernewtransform_location (0.0 0.0 100.0)) (`CapsuleComponent.GetScaledCapsuleRadius` _capsulecomponent) (`CapsuleComponent.GetScaledCapsuleHalfHeight` _capsulecomponent) "TraceTypeQuery1" false (`|MakeArray` _character :!type "Actor Object Reference")))
            (bind (_bblockinghit _binitialoverlap _time _distance _location _impactpoint _normal _impactnormal) (`GameplayStatics.BreakHitResult` _outhit))
            (if (not _binitialoverlap)
              (if (> (.z _impactnormal) (`CharacterMovementComponent.K2_GetWalkableFloorZ` (`Character.CharacterMovement` (`local.Character`))))
                (bind (_outhit_2 _returnvalue_2) (`KismetSystemLibrary.LineTraceSingle` (`self.K2_GetActorLocation`) _playernewtransform_location_2 "TraceTypeQuery1" false (`|MakeArray` (`local.Character`) :!type "Actor Object Reference")))
                (if (not _returnvalue_2)
                  (`self.K2_SetActorTransform` _character_2 (`local.PlayerNewTransform`) false true)
                  (`/Game/Stigma/Blueprints/PushObjects/PushComponent.BeginPush` (`/Game/ThirdPersonCPP/Blueprints/SecondGameplayCharacter.PushComponent` _character_2) self (`KismetMathLibrary.Conv_VectorToVector2D` _output_location))
                  (else
                    (`self.FailInformation` "Wall between player and object")))
                (else
                  (`self.FailInformation` "Floor Not Walkable")))
              (else
                (`self.FailInformation` "No room for player to be")))
            (else
              (`self.FailInformation` "No Transform found"))))
        (:`Is Not Valid`
          (`self.FailInformation` "Character does not have Component"))))
    (:`Is Not Valid`
      (`self.FailInformation` "Character is enabled"))))

(fn `UserConstructionScript`
  (for _array_element (`self.PushTranform`)
    (`AddComponent|NODE_AddArrowComponent-0` :`RelativeTransform` _array_element)))