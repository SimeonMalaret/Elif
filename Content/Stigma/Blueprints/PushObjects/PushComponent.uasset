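; Character component that lets its owner push objects in the world.
; BeginPush attaches the character to the pushable, constrains movement to a plane along its facing, stops rotate-to-movement and enables tick.
; Tick sweeps the pushable along the owner's forward vector at PushSpeed, carrying the attached character with it.
; EndPush detaches, restores movement settings and disables tick; IsPushingObject reports whether a pushable is held.
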(event `self.ReceiveBeginPlay`
  (`self.SetComponentTickEnabled` false))

(event `self.ReceiveTick`
  (params (DeltaSeconds :type "Float (single-precision)"))
  (bind _currentpushable (`self.CurrentPushable`)
    (:`then`
      (bind _sweephitresult (`Actor.K2_AddActorWorldOffset` _currentpushable (* (`Actor.GetActorForwardVector` (`self.GetOwner`)) (* DeltaSeconds (`self.PushSpeed`))) true false)))
    (:`else`)))

(fn `BeginPush`
  (params (PushObject :type "/Game/Stigma/Blueprints/PushObjects/PushableObject Object Reference"))
  (locals (OwningCharacter :type "Character Object Reference"))
  (bind _owningcharacter (`local.OwningCharacter`))
  (bind _charactermovement (`Character.CharacterMovement` _owningcharacter))
  (if (not (`KismetSystemLibrary.IsValid` (`self.CurrentPushable`)))
    (bind _ascharacter (cast `Character` (`self.GetOwner`)))
    (set `local.OwningCharacter` _ascharacter)
    (bind _output_get (set `self.CurrentPushable` (`local.PushObject`)))
    (`Actor.K2_AttachToActor` (`local.OwningCharacter`) _output_get "None" "KeepWorld" "KeepWorld" "KeepWorld" true)
    (`MovementComponent.SetPlaneConstraintEnabled` _charactermovement true)
    (`MovementComponent.SetPlaneConstraintNormal` _charactermovement (`Actor.GetActorRightVector` _owningcharacter))
    (set `CharacterMovementComponent.bOrientRotationToMovement` false _charactermovement)
    (`self.SetComponentTickEnabled` true)))

(fn `EndPush`
  (locals (`Owning Character` :type "Character Object Reference"))
  (bind _charactermovement (`Character.CharacterMovement` (`local.Owning Character`)))
  (`self.CurrentPushable`
    (:`then`
      (set `self.CurrentPushable` null)
      (bind _ascharacter (cast `Character` (`self.GetOwner`)))
      (bind _output_get (set `local.Owning Character` _ascharacter))
      (`Actor.K2_DetachFromActor` _output_get "KeepWorld" "KeepWorld" "KeepWorld")
      (`MovementComponent.SetPlaneConstraintEnabled` _charactermovement false)
      (set `CharacterMovementComponent.bOrientRotationToMovement` true _charactermovement)
      (`self.SetComponentTickEnabled` false))
    (:`else`)))

(fn `IsPushingObject`
  (returns (ReturnValue :type Boolean))
  (return (`KismetSystemLibrary.IsValid` (`self.CurrentPushable`))))