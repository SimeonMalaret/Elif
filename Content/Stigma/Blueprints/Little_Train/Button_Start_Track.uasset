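; Pressure-plate button, filed under Little_Train, that notifies the game mode when SecondGameplayCharacter steps on or off it.
; Collision overlap start plays the MovementButton timeline to lerp the button mesh down, and overlap end reverses it.
; Each overlap also parses the EventName string into an array and passes it to STIGMA_GM through CallActivationByButton or CallUnactivationByButton.
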(event `MovementDown`
  (bind (_direction _updown) (`Timeline|MovementButton` :!label _label)
    (:`Update`
      (`SceneComponent.K2_SetRelativeLocation` (`self.Button`) (`KismetMathLibrary.VLerp` (0.0 0.0 14.0) (0.0 0.0 3.0) _updown) false false))))

(event `MovementUp`
  (goto _label :!via `Reverse`))

(event `self.Collision.OnComponentBeginOverlap`
  (params (OverlappedComponent :type "PrimitiveComponent Object Reference") (OtherActor :type "Actor Object Reference") (OtherComp :type "PrimitiveComponent Object Reference") (OtherBodyIndex :type Integer) (bFromSweep :type Boolean) (SweepResult :type "HitResult Structure (by ref)"))
  (cast `/Game/ThirdPersonCPP/Blueprints/SecondGameplayCharacter` OtherActor)
  (`|ExecutionSequence`
    (:`then_0`
      (`self.MovementDown`))
    (:`then_1`
      (`/Game/Stigma/Blueprints/STIGMA_GM.ActivationByButton` (cast `/Game/Stigma/Blueprints/STIGMA_GM` (`GameplayStatics.GetGameMode`) :!pure true) (`KismetStringLibrary.ParseIntoArray` (`self.eventName`))))))

(event `self.Collision.OnComponentEndOverlap`
  (params (OverlappedComponent :type "PrimitiveComponent Object Reference") (OtherActor :type "Actor Object Reference") (OtherComp :type "PrimitiveComponent Object Reference") (OtherBodyIndex :type Integer))
  (cast `/Game/ThirdPersonCPP/Blueprints/SecondGameplayCharacter` OtherActor)
  (`|ExecutionSequence`
    (:`then_0`
      (`self.MovementUp`))
    (:`then_1`
      (`/Game/Stigma/Blueprints/STIGMA_GM.UnactivationByButton` (cast `/Game/Stigma/Blueprints/STIGMA_GM` (`GameplayStatics.GetGameMode`) :!pure true) (`KismetStringLibrary.ParseIntoArray` (`self.eventName`))))))

(fn `UserConstructionScript`)