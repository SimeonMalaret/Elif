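; Manager for a toy train puzzle that runs once enough matching button events are active.
; On start, it chains track pieces from StartTrack by matching spline endpoints and merges them into one spawned Rail spline for the train.
; CheckEnd compares that spline's end to EndTrack's, firing game mode activation events on success.
; Otherwise it hides the train with effects and respawns it at the start after a delay.
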(event `FailMovement`
  (bind _train (`self.Train`))
  (bind _returnvalue (`SplineComponent.GetLocationAtSplinePoint` (`/Game/Stigma/Blueprints/Little_Train/Rail.Spline` (`self.StartTrack`)) 0 "World"))
  ;[1 1 1] Ending movement train
  ;;[1 1 1] Fail reset
  (`SceneComponent.SetVisibility` (`/Game/Stigma/Blueprints/Little_Train/MovingTrain.Train` _train) false false)
  (`GameplayStatics.SpawnEmitterAtLocation` "/Game/Stigma/FX/Particules/Doggo_SoundWave/P_Doggo_SoundWave.P_Doggo_SoundWave" (`self.K2_GetActorLocation` _train))
  (`KismetSystemLibrary.Delay` (`self.timeRespawn`))
  (`self.K2_SetActorLocation` (`self.Train`) _returnvalue false false)
  (`GameplayStatics.SpawnEmitterAtLocation` "/Game/Stigma/FX/Particules/Dog_Toy_Pop/P_Dog_Toy_Pop_Depop.P_Dog_Toy_Pop_Depop" _returnvalue)
  (`SceneComponent.SetVisibility` (`/Game/Stigma/Blueprints/Little_Train/MovingTrain.Train` (`self.Train`)) true false)
  (set `self.hasStart` false))

(event `self.ReceiveBeginPlay`
  (bind _train (`self.Train`))
  (bind _asstigma_gm (cast `/Game/Stigma/Blueprints/STIGMA_GM` (`GameplayStatics.GetGameMode`) :!pure true))
  (set `/Game/Stigma/Blueprints/Little_Train/MovingTrain.Manager` self _train)
  (set `/Game/Stigma/Blueprints/Little_Train/MovingTrain.TrackSpline` (`self.StartTrack`) _train)
  (`self.K2_SetActorLocation` (`self.Train`) (`SplineComponent.GetLocationAtSplinePoint` (`/Game/Stigma/Blueprints/Little_Train/Rail.Spline` (`self.StartTrack`)) 0 "World") false false)
  (`KismetArrayLibrary.Array_Add` (`self.TracksList`) (`self.StartTrack`))
  (for _array_element (`self.Tracks`)
    (set `/Game/Stigma/Blueprints/Little_Train/Rail.managerTrain` self _array_element))
  (add `/Game/Stigma/Blueprints/STIGMA_GM.ActivationByButton` _asstigma_gm (delegate `StartTrain`))
  (add `/Game/Stigma/Blueprints/STIGMA_GM.UnactivationByButton` _asstigma_gm (delegate `LooseButton`)))

(event `LooseButton`
  (params (eventName :type "Array of String (by ref)"))
  ;[1 1 1] ButtonLeft
  (if (`KismetArrayLibrary.Array_Contains` eventName (`self.event`))
    (`/Engine/EditorBlueprintResources/StandardMacros.DecrementInt` (`self.numberActors`))))

(event `SuccessMovement`
  ;[1 1 1] Ending movement train
  ;;[1 1 1] Success
  (`/Game/Stigma/Blueprints/STIGMA_GM.ActivationByButton` (cast `/Game/Stigma/Blueprints/STIGMA_GM` (`GameplayStatics.GetGameMode`) :!pure true) (`KismetStringLibrary.ParseIntoArray` (`self.eventToActivate`))))

(event `CheckEnd`
  (bind _endtrack (`self.EndTrack`))
  (bind _spline (`/Game/Stigma/Blueprints/Little_Train/Rail.Spline` (`self.CompleteTrack`)))
  (bind _spline_2 (`/Game/Stigma/Blueprints/Little_Train/Rail.Spline` _endtrack))
  ;[1 1 1] Ending movement train
  ;;[1 1 1] CheckEnd
  (`/Engine/EditorBlueprintResources/StandardMacros.IsValid` _endtrack
    (:`Is Valid`
      (if (== (`SplineComponent.GetLocationAtSplinePoint` _spline (- (`SplineComponent.GetNumberOfSplinePoints` _spline) 1) "World") (`SplineComponent.GetLocationAtSplinePoint` _spline_2 (- (`SplineComponent.GetNumberOfSplinePoints` _spline_2) 1) "World"))
        (`self.SuccessMovement`)
        (else
          (`self.FailMovement` :!label _label))))
    (:`Is Not Valid`
      (goto _label))))

(event `StartTrain`
  (params (eventName :type "Array of String (by ref)"))
  ;[1 1 1] StartTrain
  (if (`KismetArrayLibrary.Array_Contains` eventName (`self.event`))
    (bind _result (`/Engine/EditorBlueprintResources/StandardMacros.IncrementInt` (`self.numberActors`))
      (:`  `
        (if (== _result (`self.numberActorsToStart`))
          (if (not (`self.hasStart`))
            (`self.CalculateMovement`)
            (set `self.hasStart` true)
            (`/Game/Stigma/Blueprints/Little_Train/MovingTrain.Movement` (`self.Train`))))))))

(event `CalculateMovement`
  ;[1 1 1] Calcul track
  (for _array_element (`self.Tracks`)
    (for _array_element_2 (`self.Tracks`)
      (bind _spline (`/Game/Stigma/Blueprints/Little_Train/Rail.Spline` _array_element))
      (if (!= _array_element_2 _spline)
        (if (== (`SplineComponent.GetLocationAtSplinePoint` (`/Game/Stigma/Blueprints/Little_Train/Rail.Spline` _array_element_2) 0 "World") (`SplineComponent.GetLocationAtSplinePoint` _spline (- (`SplineComponent.GetNumberOfSplinePoints` _spline) 1) "World") :`ErrorTolerance` 3.0)
          (set `/Game/Stigma/Blueprints/Little_Train/Rail.nextSpline` _array_element_2 _array_element)
          (if (`KismetArrayLibrary.Array_Contains` (`self.TracksList`) _array_element)
            (`KismetArrayLibrary.Array_Add` (`self.TracksList`) _array_element_2)
            (break)
            (else
              (break)))))))
  (`self.CreateTrack`))

(event `CreateTrack`
  ;[1 1 1] Creation of unique spline
  (bind _returnvalue (`|SpawnActorFromClass` "/Game/Stigma/Blueprints/Little_Train/Rail.Rail_C" (`KismetMathLibrary.MakeTransform` (0.0 0.0 0.0)) "Undefined" "OverrideRootScale" null null))
  (bind _output_get (set `self.CompleteTrack` _returnvalue))
  (`self.K2_SetActorLocation` _output_get (`self.K2_GetActorLocation` (`|GetArrayItem` (`self.TracksList`))) false false)
  (`SplineComponent.ClearSplinePoints` (`/Game/Stigma/Blueprints/Little_Train/Rail.Spline` _output_get) true)
  (`self.AddSplinePoint` 0)
  (for _index (range 1 (`KismetArrayLibrary.Array_Length` (`self.TracksList`)))
    (`self.AddSplinePoint` _index 1))
  (set `/Game/Stigma/Blueprints/Little_Train/MovingTrain.TrackSpline` (`self.CompleteTrack`) (`self.Train`)))

(fn `AddSplinePoint`
  (params (IndexTrack :type Integer) (FirstIndexLoop :type Integer))
  (bind _completetrack (`self.CompleteTrack`))
  (bind _spline (`/Game/Stigma/Blueprints/Little_Train/Rail.Spline` _completetrack))
  (bind _spline_2 (`/Game/Stigma/Blueprints/Little_Train/Rail.Spline` (`|GetArrayItem` (`self.TracksList`) IndexTrack)))
  (for _index (range (`local.FirstIndexLoop`) (`SplineComponent.GetNumberOfSplinePoints` _spline_2))
    (bind _returnvalue (`SplineComponent.GetTransformAtSplinePoint` _spline_2 _index "World" false))
    (bind _returnvalue_location (`KismetMathLibrary.BreakTransform` (`KismetMathLibrary.MakeRelativeTransform` _returnvalue (`self.GetTransform` _completetrack))))
    (`SplineComponent.AddPoint` _spline (make `SplinePoint` (`KismetMathLibrary.Conv_IntToDouble` (`SplineComponent.GetNumberOfSplinePoints` _spline)) _returnvalue_location (0.0 0.0 0.0) (0.0 0.0 0.0) (.rotation _returnvalue) (.scale _returnvalue) (`SplineComponent.GetSplinePointType` _spline_2 _index)) true)))

(fn `UserConstructionScript`)