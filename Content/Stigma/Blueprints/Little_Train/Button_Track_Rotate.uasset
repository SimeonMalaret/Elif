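; Pressure button for the little train gameplay that rotates its linked track while a SecondGameplayCharacter stands on it.
; Collision overlaps set the active flag and drive a timeline that lowers or raises the button.
; Pressing starts a second timeline that turns the track toward a 90-degree yaw step in RotationDirection, feeding its curve into RInterpTo as DeltaTime.
; Each finished turn repeats while the button stays active and the track's train manager has not started.
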(event `MovementDown`
  (bind (_direction _updown) (`Timeline|ButtonMovement` :!label _label)
    (:`Update`
      (`SceneComponent.K2_SetRelativeLocation` (`self.Button`) (`KismetMathLibrary.VLerp` (0.0 0.0 14.0) (0.0 0.0 3.0) _updown) false false))))

(event `MovementUp`
  (goto _label :!via `Reverse`))

(event `RotationTrack`
  (bind _currentrotation (`self.currentRotation`))
  (if (not (`/Game/Stigma/Blueprints/Little_Train/Manager_Train.hasStart` (`/Game/Stigma/Blueprints/Little_Train/Rail.managerTrain` (`self.Track`)))) :!label _label_2
    (if (`self.isActive`)
      (set `self.currentRotation` (`self.K2_GetActorRotation` (`self.Track`)))
      (bind (_direction _rotationtrack) (`Timeline|TimelineRotation` :!via `PlayFromStart`)
        (:`Update`
          (`self.K2_SetActorRotation` (`self.Track`) (`KismetMathLibrary.RInterpTo` _currentrotation (`KismetMathLibrary.MakeRotator` (.roll _currentrotation) (.pitch _currentrotation) (+ (.yaw _currentrotation) (* 90.0 (`self.rotationDirection`)))) _rotationtrack 2.0) false))
        (:`Finished`
          (goto _label_2))))))

(event `self.Collision.OnComponentBeginOverlap`
  (params (OverlappedComponent :type "PrimitiveComponent Object Reference") (OtherActor :type "Actor Object Reference") (OtherComp :type "PrimitiveComponent Object Reference") (OtherBodyIndex :type Integer) (bFromSweep :type Boolean) (SweepResult :type "HitResult Structure (by ref)"))
  (cast `/Game/ThirdPersonCPP/Blueprints/SecondGameplayCharacter` OtherActor)
  (set `self.isActive` true)
  (`|ExecutionSequence`
    (:`then_0`
      (`self.MovementDown`))
    (:`then_1`
      (`self.RotationTrack`))))

(event `self.Collision.OnComponentEndOverlap`
  (params (OverlappedComponent :type "PrimitiveComponent Object Reference") (OtherActor :type "Actor Object Reference") (OtherComp :type "PrimitiveComponent Object Reference") (OtherBodyIndex :type Integer))
  (cast `/Game/ThirdPersonCPP/Blueprints/SecondGameplayCharacter` OtherActor)
  (set `self.isActive` false)
  (`self.MovementUp`))

(fn `UserConstructionScript`)