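; MovingTrain is an actor, a little train that rides along a chain of spline track pieces.
; The Movement event plays a timeline that lerps distance over the current track's spline length, setting world location and rotation each update.
; When the timeline finishes, it stops with a debug print if the track is the Manager's end track; otherwise it switches to the next spline and replays, or prints that none follows.
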(event `Movement`
  (bind _spline (`/Game/Stigma/Blueprints/Little_Train/Rail.Spline` (`self.TrackSpline`)))
  (bind _nextspline (`/Game/Stigma/Blueprints/Little_Train/Rail.nextSpline` (`self.TrackSpline`)))
  (bind (_direction _movementonrail) (`Timeline|TrainMovement` :!via `PlayFromStart` :!label _label)
    (:`Update`
      (bind _returnvalue (`KismetMathLibrary.Lerp` 0.0 (`SplineComponent.GetSplineLength` _spline) _movementonrail))
      (`self.K2_SetActorLocationAndRotation` (`SplineComponent.GetLocationAtDistanceAlongSpline` _spline _returnvalue "World") (`SplineComponent.GetRotationAtDistanceAlongSpline` _spline _returnvalue "World")))
    (:`Finished`
      (if (== (`/Game/Stigma/Blueprints/Little_Train/Manager_Train.EndTrack` (`self.Manager`)) (`self.TrackSpline`))
        (`KismetSystemLibrary.PrintString` "La fin")
        (elif (`KismetSystemLibrary.IsValid` _nextspline)
          (set `self.TrackSpline` _nextspline)
          (goto _label :!via `PlayFromStart`)
          (else
            (`KismetSystemLibrary.PrintString` "Il y a pas de suite")))))))

(fn `UserConstructionScript`)