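; Destructible wall actor that, when its destructible mesh fractures, stops blocking the player and can open a linked bridge.
; On fracture, both the cube and destructible mesh ignore Pawn and two custom trace channels, and an optional BridgeToOpen reference starts opening.
; The same event triggers a camera shake on the SecondGameplayCharacter player pawn and posts a Wwise wall destruction sound.
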(event `self.Cube_DM.OnComponentFracture`
  (params (HitPoint :type "Vector Structure (by ref)") (HitDirection :type "Vector Structure (by ref)"))
  (`|ExecutionSequence`
    (:`then_0`
      (`PrimitiveComponent.SetCollisionResponseToChannel` (`self.Cube`) "ECC_GameTraceChannel5" "ECR_Ignore")
      (`PrimitiveComponent.SetCollisionResponseToChannel` (`self.Cube`) "ECC_Pawn" "ECR_Ignore")
      (`PrimitiveComponent.SetCollisionResponseToChannel` (`self.Cube_DM`) "ECC_GameTraceChannel5" "ECR_Ignore")
      (`PrimitiveComponent.SetCollisionResponseToChannel` (`self.Cube_DM`) "ECC_Pawn" "ECR_Ignore")
      (`PrimitiveComponent.SetCollisionResponseToChannel` (`self.Cube`) "ECC_GameTraceChannel3" "ECR_Ignore")
      (`PrimitiveComponent.SetCollisionResponseToChannel` (`self.Cube_DM`) "ECC_GameTraceChannel3" "ECR_Ignore")
      (bind _bridgetoopen (`self.BridgeToOpen`)
        (:`then`
          (`/Game/Stigma/Blueprints/DrawBridge/DrawbridgePlatform.StartOpenBridge` _bridgetoopen))
        (:`else`)))
    (:`then_1`
      (bind _assecond_gameplay_character (cast `/Game/ThirdPersonCPP/Blueprints/SecondGameplayCharacter` (`GameplayStatics.GetPlayerPawn` 0)))
      (`CameraShakeSourceComponent.StartCameraShake` :`self` (`/Game/ThirdPersonCPP/Blueprints/SecondGameplayCharacter.CameraShakeSource` _assecond_gameplay_character) :`InCameraShake` "/Game/Stigma/Blueprints/CamShake.CamShake_C")
      (`AkGameplayStatics.PostEvent` "/Game/Stigma/Sound/Event/Marrec_Events_WU/LEVEL/Wall/Play_Wall_Destruction.Play_Wall_Destruction" self))))

(fn `UserConstructionScript`)