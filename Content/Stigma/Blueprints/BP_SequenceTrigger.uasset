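; BP_SequenceTrigger is a one-shot overlap trigger that plays a Level Sequence for the SecondGameplayCharacter.
; On overlap it repositions the player, hides the ball widgets, locks input and movement, and restores them after the sequence's duration.
; If flagged as ending, it instead shows the ending widget after a fixed delay; the credits fade and menu return are unwired.
; Optionally it repositions the companion and sends it to a target.
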(event `self.CollisionComponent.OnComponentBeginOverlap`
  (params (OverlappedComponent :type "PrimitiveComponent Object Reference") (OtherActor :type "Actor Object Reference") (OtherComp :type "PrimitiveComponent Object Reference") (OtherBodyIndex :type Integer) (bFromSweep :type Boolean) (SweepResult :type "HitResult Structure (by ref)"))
  (bind _companion (`/Game/Stigma/Blueprints/Camille_GM.companion` (cast `/Game/Stigma/Blueprints/Camille_GM` (`GameplayStatics.GetGameMode`) :!pure true)))
  ;[1 1 1] Play a Sequence
  (bind _assecond_gameplay_character (cast `/Game/ThirdPersonCPP/Blueprints/SecondGameplayCharacter` OtherActor))
  (`|ExecutionSequence`
    (:`then_0`
      (`self.K2_SetActorTransform` _assecond_gameplay_character (`KismetMathLibrary.MakeTransform` (`self.PositionOnGround`) (`self.RotationForCamera`) (0.8 0.8 0.8)) false false)
      (`Widget.SetVisibility` (`/Game/ThirdPersonCPP/Blueprints/SecondGameplayCharacter.widgetBallBack` _assecond_gameplay_character) "Collapsed")
      (`Widget.SetVisibility` (`/Game/ThirdPersonCPP/Blueprints/SecondGameplayCharacter.widget Ball In` _assecond_gameplay_character) "Collapsed")
      (`Widget.SetVisibility` (`/Game/ThirdPersonCPP/Blueprints/SecondGameplayCharacter.Widget Ball Out` _assecond_gameplay_character) "Collapsed"))
    (:`then_1`
      (`self.DisableInput` _assecond_gameplay_character (`GameplayStatics.GetPlayerController` 0))
      (set `PrimitiveComponent.bGenerateOverlapEvents` false (`self.CollisionComponent`))
      (bind _charactermovement (`Character.CharacterMovement` _assecond_gameplay_character))
      (`CharacterMovementComponent.DisableMovement` _charactermovement)
      (bind (_outactor _returnvalue) (`LevelSequencePlayer.CreateLevelSequencePlayer` (`self.Sequence To Play`)))
      (`MovieSceneSequencePlayer.Play` _returnvalue)
      (if (`self.Is Ending`)
        (`KismetSystemLibrary.Delay` 34.0)
        (bind _returnvalue_2 (`|CreateWidget` "/Game/Stigma/User_Interface/Ending_Widget.Ending_Widget_C" (`GameplayStatics.GetPlayerController` 0)))
        (`UserWidget.AddToViewport` _returnvalue_2 0)
        (`KismetSystemLibrary.Delay` 2.0)
        (else
          (`KismetSystemLibrary.Delay` (`TimeManagementBlueprintLibrary.Conv_QualifiedFrameTimeToSeconds` (`MovieSceneSequencePlayer.GetDuration` _returnvalue)))
          (`self.EnableInput` _assecond_gameplay_character (`GameplayStatics.GetPlayerController` 0))
          (`CharacterMovementComponent.SetMovementMode` _charactermovement "MOVE_Walking" 0)
          (`Widget.SetVisibility` (`/Game/ThirdPersonCPP/Blueprints/SecondGameplayCharacter.widgetBallBack` _assecond_gameplay_character) "Visible")
          (`Widget.SetVisibility` (`/Game/ThirdPersonCPP/Blueprints/SecondGameplayCharacter.widget Ball In` _assecond_gameplay_character) "Visible")
          (`Widget.SetVisibility` (`/Game/ThirdPersonCPP/Blueprints/SecondGameplayCharacter.Widget Ball Out` _assecond_gameplay_character) "Visible"))))
    (:`then_2`
      (if (`self.isCallCompanion`)
        (if (!= (`self.Position Crackus`) (0.0 0.0 0.0))
          (`self.K2_SetActorLocation` _companion (`self.Position Crackus`) false false)
          (`self.K2_SetActorRotation` _companion (`self.Rotation Crackus`) false))
        (`KismetSystemLibrary.Delay` (`self.companion move delay`))
        (`/Game/Stigma/Blueprints/Companion/BP_Companion.MoveTo` _companion (`self.K2_GetActorLocation` (`self.targetPosition`)))
        (set `/Game/Stigma/Blueprints/Companion/BP_Companion.ToDeactivate` (`self.Deactivate Dog`) _companion)))))

(fn `UserConstructionScript`)