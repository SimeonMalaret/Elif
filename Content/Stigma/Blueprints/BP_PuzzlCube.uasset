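; BP_PuzzlCube is a puzzle cube that slides in a horizontal direction when SecondGameplayCharacter touches one of its four face triggers.
; Each face overlap sets a fixed axis direction and a moving flag, only if the cube is not already moving.
; Tick then moves it by direction and speed with a swept SetActorLocation.
; The graph never clears the moving flag, so nothing here stops further movement attempts.
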(event `self.Face_0.OnComponentBeginOverlap`
  (params (OverlappedComponent :type "PrimitiveComponent Object Reference") (OtherActor :type "Actor Object Reference") (OtherComp :type "PrimitiveComponent Object Reference") (OtherBodyIndex :type Integer) (bFromSweep :type Boolean) (SweepResult :type "HitResult Structure (by ref)"))
  (cast `/Game/ThirdPersonCPP/Blueprints/SecondGameplayCharacter` OtherActor)
  (if (not (`self.isMoving`))
    (set `self.direction` (-1.0 0.0 0.0))
    (set `self.isMoving` true :!label _label)))

(event `self.Face_1.OnComponentBeginOverlap`
  (params (OverlappedComponent :type "PrimitiveComponent Object Reference") (OtherActor :type "Actor Object Reference") (OtherComp :type "PrimitiveComponent Object Reference") (OtherBodyIndex :type Integer) (bFromSweep :type Boolean) (SweepResult :type "HitResult Structure (by ref)"))
  (cast `/Game/ThirdPersonCPP/Blueprints/SecondGameplayCharacter` OtherActor)
  (if (not (`self.isMoving`))
    (set `self.direction` (1.0 0.0 0.0))
    (goto _label)))

(event `self.Face_2.OnComponentBeginOverlap`
  (params (OverlappedComponent :type "PrimitiveComponent Object Reference") (OtherActor :type "Actor Object Reference") (OtherComp :type "PrimitiveComponent Object Reference") (OtherBodyIndex :type Integer) (bFromSweep :type Boolean) (SweepResult :type "HitResult Structure (by ref)"))
  (cast `/Game/ThirdPersonCPP/Blueprints/SecondGameplayCharacter` OtherActor)
  (if (not (`self.isMoving`))
    (set `self.direction` (0.0 -1.0 0.0))
    (goto _label)))

(event `self.Face_3.OnComponentBeginOverlap`
  (params (OverlappedComponent :type "PrimitiveComponent Object Reference") (OtherActor :type "Actor Object Reference") (OtherComp :type "PrimitiveComponent Object Reference") (OtherBodyIndex :type Integer) (bFromSweep :type Boolean) (SweepResult :type "HitResult Structure (by ref)"))
  (cast `/Game/ThirdPersonCPP/Blueprints/SecondGameplayCharacter` OtherActor)
  (if (not (`self.isMoving`))
    (set `self.direction` (0.0 1.0 0.0))
    (goto _label)))

(event `self.ReceiveTick`
  (params (DeltaSeconds :type "Float (single-precision)"))
  (if (`self.isMoving`)
    (`self.K2_SetActorLocation` (+ (* (* (`self.direction`) DeltaSeconds) (`self.speed`)) (`self.K2_GetActorLocation`)) true)))

(fn `UserConstructionScript`)