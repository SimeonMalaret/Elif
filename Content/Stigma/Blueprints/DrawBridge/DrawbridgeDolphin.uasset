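; Drawbridge actor in Stigma that opens and closes in response to button events broadcast by the STIGMA_GM game mode.
; It counts activations against a required threshold, while counted locks force it closed until all are released, reopening if the threshold is still met.
; A timeline with separate opening and closing speeds lerps the actor between start and end transforms, reversing to close, with Wwise sound on movement.
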(event `OpenBrodgeByButton`
  (params (eventName :type "Array of String (by ref)"))
  (if (`KismetArrayLibrary.Array_Contains` eventName (`self.eventName`))
    (bind _output_get (set `self.nbActors` (+ (`self.nbActors`) 1)))
    (if (and (>= _output_get (`self.nbActorToOpen`)) (not (`self.isLock`)))
      (set `self.IsOpen` true)
      (`self.StartOpenBridge`)
      (if (`self.debug`)
        (`KismetSystemLibrary.PrintString` "Open")))))

(event `Lock`
  (params (eventName :type "Array of String (by ref)"))
  (if (`KismetArrayLibrary.Array_Contains` eventName (`self.eventName`))
    (if (`self.debug`)
      (`KismetSystemLibrary.PrintString` "Lock"))
    (set `self.isLock` true)
    (set `self.nbLock` (+ (`self.nbLock`) 1))
    (set `self.IsOpen` false)
    (`self.StartCloseBridge`)))

(event `self.ReceiveBeginPlay`
  (bind _asstigma_gm (cast `/Game/Stigma/Blueprints/STIGMA_GM` (`GameplayStatics.GetGameMode`) :!pure true))
  (add `/Game/Stigma/Blueprints/STIGMA_GM.ActivationByButton` _asstigma_gm (delegate `OpenBrodgeByButton`))
  (add `/Game/Stigma/Blueprints/STIGMA_GM.UnactivationByButton` _asstigma_gm (delegate `CloseBridgeByButton`))
  (add `/Game/Stigma/Blueprints/STIGMA_GM.LockByButton` _asstigma_gm (delegate `Lock`))
  (add `/Game/Stigma/Blueprints/STIGMA_GM.UnLockByButton` _asstigma_gm (delegate `Unlock`)))

(event `Unlock`
  (params (eventName :type "Array of String (by ref)"))
  (if (`KismetArrayLibrary.Array_Contains` eventName (`self.eventName`))
    (if (`self.debug`)
      (`KismetSystemLibrary.PrintString` "unlock"))
    (bind _output_get (set `self.nbLock` (- (`self.nbLock`) 1)))
    (if (<= _output_get 0)
      (set `self.isLock` false)
      (if (>= (`self.nbActors`) (`self.nbActorToOpen`))
        (set `self.IsOpen` true)
        (`self.StartOpenBridge`)))))

(event `CloseBridgeByButton`
  (params (eventName :type "Array of String (by ref)"))
  (if (`KismetArrayLibrary.Array_Contains` eventName (`self.eventName`))
    (bind _output_get (set `self.nbActors` (- (`self.nbActors`) 1)))
    (if (< _output_get (`self.nbActorToOpen`))
      (set `self.IsOpen` false)
      (`self.StartCloseBridge`)
      (if (`self.debug`)
        (`KismetSystemLibrary.PrintString` "Close")))))

(event `StartOpenBridge`
  (`TimelineComponent.SetPlayRate` (`self.TimelineOpening`) (`self.OpeningSpeed`))
  (if (`self.isMoving`)
    (bind (_direction _opening) (`Timeline|TimelineOpening` :!label _label)
      (:`Update`
        (bind _output_get (set `self.Alpha` _opening))
        (`self.K2_SetActorTransform` (`KismetMathLibrary.TLerp` (`self.PositionStart`) (`self.PositionEnd`) _output_get) false true)
        (set `self.isMoving` true))
      (:`Finished`
        (set `self.isMoving` false)
        (`AkGameObject.Stop` (`self.BridgeDownSound`))))
    (elif (< (`self.Alpha`) 2.0)
      (`AkGameObject.PostAssociatedAkEvent` :`self` (`self.BridgeDownSound`))
      (goto _label))))

(event `StartCloseBridge`
  (`TimelineComponent.SetPlayRate` (`self.TimelineOpening`) (`self.ClosingSpeed`))
  (if (`self.isMoving`)
    (goto _label :!via `Reverse`)
    (elif (> (`self.Alpha`) 0.0)
      (`AkGameObject.PostAssociatedAkEvent` :`self` (`self.BridgeDownSound`))
      (goto _label :!via `Reverse`))))

(fn `UserConstructionScript`)