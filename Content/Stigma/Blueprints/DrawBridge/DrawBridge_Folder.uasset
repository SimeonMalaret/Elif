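; Drawbridge actor that opens and closes through button events broadcast by the Camille_GM game mode, filtered by event name.
; Activations are counted against a required number to open, while counted locks force it closed until all are released, then reopen it if enough activations remain.
; Opening and closing play the skeletal mesh animation at separate speed settings, with a Wwise sound posted on opening.
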(event `OpenBridgeByButton`
  (params (eventName :type "Array of String (by ref)"))
  (if (`KismetArrayLibrary.Array_Contains` eventName (`self.eventName`))
    (bind _output_get (set `self.nbActors` (+ (`self.nbActors`) 1)))
    (if (and (>= _output_get (`self.nbActorToOpen`)) (not (`self.isLock`)))
      (set `self.IsOpen` true)
      (`self.StartOpenBridge`)
      (if (`self.debug`)
        (`KismetSystemLibrary.PrintString` "Open")))))

(event `Lock`
  (params (eventName :type "Array of String (by ref)"))
  (if (`KismetArrayLibrary.Array_Contains` eventName (`self.eventName`))
    (if (`self.debug`)
      (`KismetSystemLibrary.PrintString` "Lock"))
    (set `self.isLock` true)
    (set `self.nbLock` (+ (`self.nbLock`) 1))
    (set `self.IsOpen` false)
    (`self.StartCloseBridge`)))

(event `self.ReceiveBeginPlay`
  (bind _ascamille_gm (cast `/Game/Stigma/Blueprints/Camille_GM` (`GameplayStatics.GetGameMode`)))
  (add `/Game/Stigma/Blueprints/Camille_GM.ActivationByButton` _ascamille_gm (delegate `OpenBridgeByButton`))
  (add `/Game/Stigma/Blueprints/Camille_GM.UnactivationByButton` _ascamille_gm (delegate `CloseBridgeByButton`))
  (add `/Game/Stigma/Blueprints/Camille_GM.LockByButton` _ascamille_gm (delegate `Lock`))
  (add `/Game/Stigma/Blueprints/Camille_GM.UnLockByButton` _ascamille_gm (delegate `Unlock`)))

(event `Unlock`
  (params (eventName :type "Array of String (by ref)"))
  (if (`KismetArrayLibrary.Array_Contains` eventName (`self.eventName`))
    (if (`self.debug`)
      (`KismetSystemLibrary.PrintString` "unlock"))
    (bind _output_get (set `self.nbLock` (- (`self.nbLock`) 1)))
    (if (<= _output_get 0)
      (set `self.isLock` false)
      (if (>= (`self.nbActors`) (`self.nbActorToOpen`))
        (set `self.IsOpen` true)
        (`self.StartOpenBridge`)))))

(event `CloseBridgeByButton`
  (params (eventName :type "Array of String (by ref)"))
  (if (`KismetArrayLibrary.Array_Contains` eventName (`self.eventName`))
    (bind _output_get (set `self.nbActors` (- (`self.nbActors`) 1)))
    (if (< _output_get (`self.nbActorToOpen`))
      (set `self.IsOpen` false)
      (`self.StartCloseBridge`)
      (if (`self.debug`)
        (`KismetSystemLibrary.PrintString` "Close")))))

(event `StartOpenBridge`
  (bind _skeletalmesh (`self.SkeletalMesh`))
  (`SkeletalMeshComponent.SetPlayRate` _skeletalmesh (`self.OpeningSpeed`))
  (`SkeletalMeshComponent.Play` _skeletalmesh false)
  (`AkGameObject.PostAssociatedAkEvent` :`self` (`self.Opensound`)))

(event `StartCloseBridge`
  (bind _skeletalmesh (`self.SkeletalMesh`))
  (`SkeletalMeshComponent.SetPlayRate` _skeletalmesh (`self.ClosingSpeed`))
  (`SkeletalMeshComponent.Play` _skeletalmesh false))

(fn `UserConstructionScript`)