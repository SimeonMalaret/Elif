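; Bear drawbridge actor that opens or closes in response to named button events from Camille_GM.
; It opens when enough activations are counted and no lock is held; stacked locks force it closed until all release.
; Timelines lerp the actor between start and end transforms and rotate two gantry "eyebrow" pieces, reversing to close.
; Movement starting from rest triggers Wwise sound and force feedback at the player.
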(event `OpenBrodgeByButton`
  (params (eventName :type "Array of String (by ref)"))
  (if (`KismetArrayLibrary.Array_Contains` eventName (`self.eventName`))
    (bind _output_get (set `self.nbActors` (+ (`self.nbActors`) 1)))
    (`KismetSystemLibrary.PrintString` (`KismetStringLibrary.Conv_IntToString` _output_get))
    (if (and (>= _output_get (`self.nbActorToOpen`)) (not (`self.isLock`)))
      (set `self.IsOpen` true)
      (`self.StartOpenBridge`)
      (if (`self.debug`)
        (`KismetSystemLibrary.PrintString` "Open")))))

(event `Lock`
  (params (eventName :type "Array of String (by ref)"))
  (if (`KismetArrayLibrary.Array_Contains` eventName (`self.eventName`))
    (if (`self.debug`)
      (`KismetSystemLibrary.PrintString` "Lock"))
    (bind _output_get (set `self.isLock` true))
    (`KismetSystemLibrary.PrintString` (`KismetStringLibrary.Conv_BoolToString` _output_get))
    (set `self.nbLock` (+ (`self.nbLock`) 1))
    (set `self.IsOpen` false)
    (`self.StartCloseBridge`)))

(event `self.ReceiveBeginPlay`
  (bind _ascamille_gm (cast `/Game/Stigma/Blueprints/Camille_GM` (`GameplayStatics.GetGameMode`)))
  (add `/Game/Stigma/Blueprints/Camille_GM.ActivationByButton` _ascamille_gm (delegate `OpenBrodgeByButton`))
  (add `/Game/Stigma/Blueprints/Camille_GM.UnactivationByButton` _ascamille_gm (delegate `CloseBridgeByButton`))
  (add `/Game/Stigma/Blueprints/Camille_GM.LockByButton` _ascamille_gm (delegate `Lock`))
  (add `/Game/Stigma/Blueprints/Camille_GM.UnLockByButton` _ascamille_gm (delegate `Unlock`)))

(event `Unlock`
  (params (eventName :type "Array of String (by ref)"))
  (if (`KismetArrayLibrary.Array_Contains` eventName (`self.eventName`))
    (if (`self.debug`)
      (`KismetSystemLibrary.PrintString` "unlock"))
    (bind _output_get (set `self.nbLock` (- (`self.nbLock`) 1)))
    (if (<= _output_get 0)
      (set `self.nbLock` 0)
      (bind _output_get_2 (set `self.isLock` false))
      (`KismetSystemLibrary.PrintString` (`KismetStringLibrary.Conv_BoolToString` _output_get_2))
      (if (>= (`self.nbActors`) (`self.nbActorToOpen`))
        (set `self.IsOpen` true)
        (`self.StartOpenBridge`)))))

(event `CloseBridgeByButton`
  (params (eventName :type "Array of String (by ref)"))
  (if (`KismetArrayLibrary.Array_Contains` eventName (`self.eventName`))
    (bind _output_get (set `self.nbActors` (- (`self.nbActors`) 1)))
    (if (< _output_get (`self.nbActorToOpen`))
      (if (< (`self.nbActors`) 0)
        (set `self.nbActors` 0))
      (set `self.IsOpen` false)
      (`self.StartCloseBridge`)
      (if (`self.debug`)
        (`KismetSystemLibrary.PrintString` "Close")))))

(event `StartOpenBridge`
  (`TimelineComponent.SetPlayRate` (`self.TimelineOpening`) (`self.OpeningSpeed`))
  (if (`self.isMoving`)
    (`|ExecutionSequence` :!label _label
      (:`then_0`
        (bind (_direction _opening) (`Timeline|TimelineOpening` :!label _label_2)
          (:`Update`
            (bind _output_get (set `self.Alpha` _opening))
            (`self.K2_SetActorTransform` (`KismetMathLibrary.TLerp` (`self.PositionStart`) (`self.PositionEnd`) _output_get) false true)
            (set `self.isMoving` true))
          (:`Finished`
            (set `self.isMoving` false)
            (`AkGameObject.Stop` (`self.BridgeDownSound`)))))
      (:`then_1`
        (bind (_direction_2 _eyebrows) (`Timeline|MovementEyebrows` :!label _label_3)
          (:`Update`
            (bind _returnvalue (`KismetMathLibrary.Lerp` 0.0 33.75 _eyebrows))
            (`SceneComponent.K2_SetRelativeRotation` (`self.PROD_SET_Gantry_04`) (`KismetMathLibrary.MakeRotator` _returnvalue) false false)
            (bind _result (`/Engine/EditorBlueprintResources/StandardMacros.NegateFloat` _returnvalue)
              (:`  `
                (`SceneComponent.K2_SetRelativeRotation` (`self.PROD_SET_Gantry_03`) (`KismetMathLibrary.MakeRotator` _result) false false)))))))
    (elif (< (`self.Alpha`) 2.0)
      (`AkGameObject.PostAssociatedAkEvent` :`self` (`self.BridgeDownSound`))
      (`GameplayStatics.SpawnForceFeedbackAtLocation` "/Game/Stigma/Feedback/OpenDoors.OpenDoors" (`self.K2_GetActorLocation` (`GameplayStatics.GetPlayerPawn` 0)) (struct) false 1.0 0.0 null)
      (goto _label))))

(event `StartCloseBridge`
  (`TimelineComponent.SetPlayRate` (`self.TimelineOpening`) (`self.ClosingSpeed`))
  (if (`self.isMoving`)
    (`|ExecutionSequence` :!label _label_4
      (:`then_0`
        (goto _label_2 :!via `Reverse`))
      (:`then_1`
        (goto _label_3 :!via `Reverse`)))
    (elif (> (`self.Alpha`) 0.0)
      (`AkGameObject.PostAssociatedAkEvent` :`self` (`self.BridgeDownSound`))
      (`GameplayStatics.SpawnForceFeedbackAtLocation` "/Game/Stigma/Feedback/OpenDoors.OpenDoors" (`self.K2_GetActorLocation` (`GameplayStatics.GetPlayerPawn` 0)) (struct) false 1.0 0.0 null)
      (goto _label_4))))

(fn `UserConstructionScript`)