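; Drawbridge platform actor that moves between a start and end transform when enough named button activations are registered.
; It binds to the Camille_GM game mode's button activation and deactivation events, counting actors against an opening threshold for its event name.
; Crossing the threshold plays or reverses a timeline that lerps the actor's transform.
; Wwise rocket loop audio accompanies the movement, with an IsMoving flag preventing retriggers.
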(event `OpenBrodgeByButton`
  (params (eventName :type String))
  (if (`KismetStringLibrary.EqualEqual_StrStr` eventName (`self.eventName`))
    (bind _output_get (set `self.nbActors` (+ (`self.nbActors`) 1)))
    (if (>= _output_get (`self.nbActorToOpen`))
      (`self.StartOpenBridge`)
      (if (`self.debug`)
        (`KismetSystemLibrary.PrintString` "Open")))))

(event `self.ReceiveBeginPlay`
  (bind _ascamille_gm (cast `/Game/Stigma/Blueprints/Camille_GM` (`GameplayStatics.GetGameMode`)))
  (add `/Game/Stigma/Blueprints/Camille_GM.ActivationByButton` _ascamille_gm (delegate `OpenBrodgeByButton`))
  (add `/Game/Stigma/Blueprints/Camille_GM.UnactivationByButton` _ascamille_gm (delegate `CloseBridgeByButton`)))

(event `CloseBridgeByButton`
  (params (eventName :type String))
  (if (`KismetStringLibrary.EqualEqual_StrStr` eventName (`self.eventName`))
    (bind _output_get (set `self.nbActors` (- (`self.nbActors`) 1)))
    (if (< _output_get (`self.nbActorToOpen`))
      (`self.StartCloseBridge`)
      (if (`self.debug`)
        (`KismetSystemLibrary.PrintString` "Close")))))

(event `StartOpenBridge`
  (if (`self.isMoving`)
    (bind (_direction _opening) (`Timeline|TimelineOpening` :!label _label)
      (:`Update`
        (`self.K2_SetActorTransform` (`KismetMathLibrary.TLerp` (`self.PositionStart`) (`self.PositionEnd`) _opening) false true)
        (set `self.isMoving` true))
      (:`Finished`
        (set `self.isMoving` false)
        (`AkGameplayStatics.PostEvent` "/Game/Stigma/Sound/Event/DefaultWorkUnit/LEVEL/PROPS/Rocket/Stop_Rocket_Forward_lp.Stop_Rocket_Forward_lp" self)))
    (else
      (`AkGameplayStatics.PostEvent` "/Game/Stigma/Sound/Event/DefaultWorkUnit/LEVEL/PROPS/Rocket/Play_Rocket_Forward_lp.Play_Rocket_Forward_lp" self)
      (goto _label))))

(event `StartCloseBridge`
  (if (`self.isMoving`)
    (goto _label :!via `Reverse`)
    (else
      (`AkGameplayStatics.PostEvent` "/Game/Stigma/Sound/Event/DefaultWorkUnit/LEVEL/PROPS/Rocket/Play_Rocket_Forward_lp.Play_Rocket_Forward_lp" self)
      (goto _label :!via `Reverse`))))

(fn `UserConstructionScript`)