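; Destructible drawbridge piece that shatters when enough button activations arrive.
; Loads its destructible mesh from a soft reference, async if needed, and binds to STIGMA_GM button events to keep an activation count.
; At the threshold, unless locked, it applies damage and an impulse, then destroys itself after a delay.
; On fracture it ignores selected collision channels, including Pawn on its box, and plays force feedback and Wwise sound.
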(event `self.ReceiveBeginPlay`
  (bind _destructiblemeshsoftref (`self.DestructibleMeshSoftRef`))
  (bind _output (`|ConvertAsset` _destructiblemeshsoftref))
  (bind _asstigma_gm (cast `/Game/Stigma/Blueprints/STIGMA_GM` (`GameplayStatics.GetGameMode`) :!pure true))
  (`|ExecutionSequence`
    (:`then_0`
      (`/Engine/EditorBlueprintResources/StandardMacros.IsValid` _output
        (:`Is Valid`
          (`DestructibleComponent.SetDestructibleMesh` (`self.Destructible`) _output))
        (:`Is Not Valid`
          (bind _object (`|LoadAsset` _destructiblemeshsoftref)
            (:`Completed`
              (bind _asdestructible_mesh (cast `DestructibleMesh` _object))
              (`DestructibleComponent.SetDestructibleMesh` (`self.Destructible`) _asdestructible_mesh))))))
    (:`then_1`
      (add `/Game/Stigma/Blueprints/STIGMA_GM.ActivationByButton` _asstigma_gm (delegate `OpenBrodgeByButton`))
      (add `/Game/Stigma/Blueprints/STIGMA_GM.UnactivationByButton` _asstigma_gm (delegate `CloseBridgeByButton`)))))

(event `OpenBrodgeByButton`
  (params (eventName :type "Array of String (by ref)"))
  (bind _destructible (`self.Destructible`))
  (if (`KismetArrayLibrary.Array_Contains` eventName (`self.eventName`))
    (bind _output_get (set `self.nbActors` (+ (`self.nbActors`) 1)))
    (if (and (>= _output_get (`self.nbActorToOpen`)) (not (`self.isLock`)))
      (set `self.IsOpen` true)
      (`DestructibleComponent.ApplyDamage` _destructible 100.0 (`self.K2_GetActorLocation`) (`KismetMathLibrary.MakeVector` 0.0) 0.0)
      (`PrimitiveComponent.AddImpulse` _destructible (`self.Explosion Direction`) "None" true)
      (`KismetSystemLibrary.Delay` (`self.Despawn Delay`))
      (`self.K2_DestroyActor`)
      (if (`self.debug`)
        (`KismetSystemLibrary.PrintString` "Open")))))

(event `CloseBridgeByButton`
  (params (eventName :type "Array of String (by ref)"))
  (if (`KismetArrayLibrary.Array_Contains` eventName (`self.eventName`))
    (bind _output_get (set `self.nbActors` (- (`self.nbActors`) 1)))
    (if (< _output_get (`self.nbActorToOpen`))
      (set `self.IsOpen` false))))

(event `self.Destructible.OnComponentFracture`
  (params (HitPoint :type "Vector Structure (by ref)") (HitDirection :type "Vector Structure (by ref)"))
  (bind _box (`self.Box`))
  (`PrimitiveComponent.SetCollisionResponseToChannel` (`self.Destructible`) "ECC_GameTraceChannel5" "ECR_Ignore")
  (`PrimitiveComponent.SetCollisionResponseToChannel` _box "ECC_GameTraceChannel5" "ECR_Ignore")
  (`PrimitiveComponent.SetCollisionResponseToChannel` _box "ECC_Pawn" "ECR_Ignore")
  (`PrimitiveComponent.SetCollisionResponseToChannel` _box "ECC_GameTraceChannel3" "ECR_Ignore")
  (`GameplayStatics.SpawnForceFeedbackAtLocation` "/Game/Stigma/HapticVibrationsFeedback/BooksDestroyed.BooksDestroyed" (`self.K2_GetActorLocation` (`GameplayStatics.GetPlayerPawn` 0)) (struct) false 1.0 0.0 null)
  (`AkGameObject.PostAssociatedAkEvent` :`self` (`self.DestructionSound`)))

(fn `UserConstructionScript`)