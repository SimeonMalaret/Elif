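; Door actor that swings open and closed in response to named button events broadcast by the Camille_GM game mode.
; Activation and deactivation events adjust an actor count, opening the door once it reaches NbActorToOpen unless locked.
; Lock events stack in a counter and force it closed; releasing the last lock reopens it if the count still suffices.
; Tick eases DoorMesh rotation toward the open or closed angle at OpeningSpeed.
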(event `self.ReceiveBeginPlay`
  (bind _ascamille_gm (cast `/Game/Stigma/Blueprints/Camille_GM` (`GameplayStatics.GetGameMode`) :!pure true))
  (add `/Game/Stigma/Blueprints/Camille_GM.ActivationByButton` _ascamille_gm (delegate `Open`))
  (add `/Game/Stigma/Blueprints/Camille_GM.UnactivationByButton` _ascamille_gm (delegate `Close`))
  (add `/Game/Stigma/Blueprints/Camille_GM.LockByButton` _ascamille_gm (delegate `CustomEvent_0`))
  (add `/Game/Stigma/Blueprints/Camille_GM.UnLockByButton` _ascamille_gm (delegate `UnLock`)))

(event `Open`
  (params (eventName :type "Array of String (by ref)"))
  ;[1 1 1] active
  (if (`KismetArrayLibrary.Array_Contains` eventName (`self.Event name`))
    (bind _output_get (set `self.nbActors` (+ (`self.nbActors`) 1)))
    (if (and (>= _output_get (`self.nbActorToOpen`)) (not (`self.isLock`)))
      (set `self.IsOpen` true))))

(event `CustomEvent_0`
  (params (eventName :type "Array of String (by ref)"))
  (if (`KismetArrayLibrary.Array_Contains` eventName (`self.Event name`))
    (if (`self.debug`)
      (`KismetSystemLibrary.PrintString` "Lock"))
    (set `self.isLock` true)
    (set `self.nbLock` (+ (`self.nbLock`) 1))
    (set `self.IsOpen` false)))

(event `UnLock`
  (params (eventName :type "Array of String (by ref)"))
  (if (`KismetArrayLibrary.Array_Contains` eventName (`self.Event name`))
    (if (`self.debug`)
      (`KismetSystemLibrary.PrintString` "unlock"))
    (bind _output_get (set `self.nbLock` (- (`self.nbLock`) 1)))
    (if (<= _output_get 0)
      (set `self.isLock` false)
      (if (>= (`self.nbActors`) (`self.nbActorToOpen`))
        (set `self.IsOpen` true)))))

(event `Close`
  (params (eventName :type "Array of String (by ref)"))
  ;[1 1 1] reset
  (if (`KismetArrayLibrary.Array_Contains` eventName (`self.Event name`))
    (bind _output_get (set `self.nbActors` (- (`self.nbActors`) 1)))
    (if (< _output_get (`self.nbActorToOpen`))
      (set `self.IsOpen` false)
      (if (`self.debug`)
        (`KismetSystemLibrary.PrintString` "Close")))))

(event `self.ReceiveTick`
  (params (DeltaSeconds :type "Float (single-precision)"))
  (bind _doormesh (`self.DoorMesh`))
  (bind _returnvalue (* DeltaSeconds (`self.OpeningSpeed`)))
  (bind _relativerotation (`SceneComponent.RelativeRotation` _doormesh))
  ;[1 1 1] eventTick
  (if (`self.IsOpen`)
    (`SceneComponent.K2_SetRelativeRotation` _doormesh (`KismetMathLibrary.RLerp` _relativerotation (struct :`Yaw` 90.0) _returnvalue) false false)
    (else
      (`SceneComponent.K2_SetRelativeRotation` _doormesh (`KismetMathLibrary.RLerp` _relativerotation (struct) _returnvalue) false false))))

(fn `CloseDoor`
  (set `self.IsOpen` false))

(fn `OpenDoor`
  (set `self.IsOpen` true))

(fn `UserConstructionScript`)