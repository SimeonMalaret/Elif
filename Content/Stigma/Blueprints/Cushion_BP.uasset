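; Cushion actor that sinks when the SecondGameplayCharacter enters its Box trigger and rises back when the character leaves.
; It records its start location on BeginPlay, then the PressMovement timeline lerps the whole actor between that point and a short drop below it, without sweeping.
; Overlap begin plays the timeline forward and overlap end reverses it.
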(event `self.ReceiveBeginPlay`
  (set `self.StartPosition` (`self.K2_GetActorLocation`)))

(event `self.Box.OnComponentBeginOverlap`
  (params (OverlappedComponent :type "PrimitiveComponent Object Reference") (OtherActor :type "Actor Object Reference") (OtherComp :type "PrimitiveComponent Object Reference") (OtherBodyIndex :type Integer) (bFromSweep :type Boolean) (SweepResult :type "HitResult Structure (by ref)"))
  (bind _startposition (`self.StartPosition`))
  (cast `/Game/ThirdPersonCPP/Blueprints/SecondGameplayCharacter` OtherActor)
  (bind (_direction _newtrack_0) (`Timeline|PressMovement` :!label _label)
    (:`Update`
      (`self.K2_SetActorLocation` (`KismetMathLibrary.VLerp` _startposition (- _startposition (0.0 0.0 30.0)) _newtrack_0)))))

(event `self.Box.OnComponentEndOverlap`
  (params (OverlappedComponent :type "PrimitiveComponent Object Reference") (OtherActor :type "Actor Object Reference") (OtherComp :type "PrimitiveComponent Object Reference") (OtherBodyIndex :type Integer))
  (cast `/Game/ThirdPersonCPP/Blueprints/SecondGameplayCharacter` OtherActor)
  (goto _label :!via `Reverse`))

(fn `UserConstructionScript`)