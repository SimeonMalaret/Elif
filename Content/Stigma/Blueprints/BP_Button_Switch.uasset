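; One-shot floor switch that latches on when an actor with the interactible tag overlaps its box, with no path to release it.
; The first press plays a Wwise sound and passes its parsed EventName to the Camille_GM game mode to trigger activation.
; It also sets linked cables and corners to their active color and plays a timeline rotating four paws and shifting the head.
; Tick lerps the button down to the base's height.
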(event `self.ReceiveBeginPlay`
  (bind (_returnvalue_x _returnvalue_y _returnvalue_z) (`KismetMathLibrary.BreakVector` (`SceneComponent.K2_GetComponentLocation` (`self.Button`))))
  ;[1 1 1] BeginPlay
  (set `self.InitPushPosZ` _returnvalue_z)
  (set `self.InitialURP` (`SceneComponent.RelativeRotation` (`self.UpRightPaw`)))
  (set `self.InitialULP` (`SceneComponent.RelativeRotation` (`self.UpLeftPaw`)))
  (set `self.InitialDRP` (`SceneComponent.RelativeRotation` (`self.DownRightPaw`)))
  (set `self.InitialDLP` (`SceneComponent.RelativeRotation` (`self.DownLeftPaw`)))
  (set `self.InitialHead` (`SceneComponent.RelativeLocation` (`self.Head`))))

(event `self.ReceiveTick`
  (params (DeltaSeconds :type "Float (single-precision)"))
  (bind _lerpbuttonpush (`self.lerpButtonPush`))
  (bind _button (`self.Button`))
  (bind _lerpbuttonpush_2 (`self.lerpButtonPush`))
  (bind (_returnvalue_x _returnvalue_y _returnvalue_z) (`KismetMathLibrary.BreakVector` (`SceneComponent.K2_GetComponentLocation` (`self.Base`))))
  (bind (_returnvalue_x_2 _returnvalue_y_2) (`KismetMathLibrary.BreakVector` (`SceneComponent.K2_GetComponentLocation` _button)))
  (bind _returnvalue (* DeltaSeconds (`self.speedPush`)))
  ;[1 1 1] Event Tick
  (if (`self.isPush`)
    (set `self.lerpButtonPush` (+ _returnvalue _lerpbuttonpush_2))
    (else
      (set `self.lerpButtonPush` (- _lerpbuttonpush_2 _returnvalue))))
  (if (`self.debug`)
    (`KismetSystemLibrary.PrintString` (`KismetStringLibrary.Conv_DoubleToString` _lerpbuttonpush) true true (struct :`G` 0.66 :`B` 1.0 :`A` 1.0) 0.0))
  (if (and (<= _lerpbuttonpush 1.0) (>= (`self.lerpButtonPush`) 0.0))
    _
    (elif (`self.isPush`)
      (set `self.lerpButtonPush` 1.0)
      (else
        (set `self.lerpButtonPush` 0.0))))
  (`SceneComponent.K2_SetWorldLocation` _button (`KismetMathLibrary.MakeVector` _returnvalue_x_2 _returnvalue_y_2 (`KismetMathLibrary.Lerp` (`self.InitPushPosZ`) _returnvalue_z (`self.lerpButtonPush`))) false false))

(event `self.Box.OnComponentBeginOverlap`
  (params (OverlappedComponent :type "PrimitiveComponent Object Reference") (OtherActor :type "Actor Object Reference") (OtherComp :type "PrimitiveComponent Object Reference") (OtherBodyIndex :type Integer) (bFromSweep :type Boolean) (SweepResult :type "HitResult Structure (by ref)"))
  (if (not (`self.IsOn`))
    (if (`self.ActorHasTag` OtherActor (`self.InteractibleTag`))
      (set `self.IsOn` true)
      (`AkGameObject.PostAssociatedAkEvent` :`self` (`self.ButtonSound`))
      (bind _output_get (set `self.nbObjOnButton` (+ (`self.nbObjOnButton`) 1)))
      (if (== _output_get 1)
        (bind _ascamille_gm (cast `/Game/Stigma/Blueprints/Camille_GM` (`GameplayStatics.GetGameMode`)))
        (`/Game/Stigma/Blueprints/Camille_GM.ActivationByButton` _ascamille_gm (`KismetStringLibrary.ParseIntoArray` (`self.eventName`)))
        (`|ExecutionSequence`
          (:`then_0`
            ;[1 1 1] Set Button Pushed
            (bind _output_get_2 (set `self.isPush` true))
            (if (`self.debug`)
              (`KismetSystemLibrary.PrintString` (`KismetStringLibrary.Conv_BoolToString` _output_get_2))))
          (:`then_1`
            ;[1 1 1] Switch Cables color
            (if (!= (`KismetArrayLibrary.Array_Length` (`self.CableList`)) 0)
              (for _array_element (`self.CableList`)
                (`/Game/Stigma/Blueprints/Cables/BP_Cable.SetActiveColor` _array_element)
                (if (!= (`KismetArrayLibrary.Array_Length` (`self.CableCornerList`)) 0)
                  (for _array_element_2 (`self.CableCornerList`)
                    (`/Game/Stigma/Blueprints/Cables/BP_CableCorner.SetActiveColor` _array_element_2))))))
          (:`then_2`
            ;[1 1 1] Rotate Paws
            (bind (_direction _rotate) (`Timeline|PawRotation`)
              (:`Update`
                (`self.PawRotate` _rotate)))))))))

(fn `PawRotate`
  (params (Speed :type "Float (double-precision) (by ref)"))
  (bind _initialhead (`self.InitialHead`))
  (`SceneComponent.K2_SetRelativeRotation` (`self.UpRightPaw`) (`KismetMathLibrary.RLerp` (`self.InitialURP`) (struct :`Yaw` 50.0) Speed) false false)
  (`SceneComponent.K2_SetRelativeRotation` (`self.UpLeftPaw`) (`KismetMathLibrary.RLerp` (`self.InitialULP`) (struct :`Yaw` -40.0) Speed) false false)
  (`SceneComponent.K2_SetRelativeRotation` (`self.DownRightPaw`) (`KismetMathLibrary.RLerp` (`self.InitialDRP`) (struct :`Yaw` 55.0) Speed) false false)
  (`SceneComponent.K2_SetRelativeRotation` (`self.DownLeftPaw`) (`KismetMathLibrary.RLerp` (`self.InitialDLP`) (struct :`Yaw` -50.0) Speed) false false)
  (`SceneComponent.K2_SetRelativeLocation` (`self.Head`) (`KismetMathLibrary.VLerp` _initialhead (- _initialhead (20.0 0.0 0.0)) Speed) false false)
  (return))

(fn `UserConstructionScript`)