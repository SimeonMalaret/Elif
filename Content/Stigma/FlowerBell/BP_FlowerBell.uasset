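; Bell flower actor that sways in the wind and rings when the player character touches it.
; Each tick it reads wind intensity from the MPC_Wind parameter collection, either resetting its roll in still air or playing a timeline that lerps it.
; Overlap with a SecondGameplayCharacter posts the FlowerBell Wwise event; the knockback launch is disconnected, and the saved starting yaw is unused.
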(event `self.ReceiveBeginPlay`
  (bind (_returnvalue_roll _returnvalue_pitch _returnvalue_yaw) (`KismetMathLibrary.BreakRotator` (`self.K2_GetActorRotation`)))
  ;[1 1 1] Get Rotation on Start
  (set `self.OriginalRotation` _returnvalue_yaw))

(event `self.ReceiveTick`
  (params (DeltaSeconds :type "Float (single-precision)"))
  (bind (_returnvalue_roll _returnvalue_pitch _returnvalue_yaw) (`KismetMathLibrary.BreakRotator` (`self.K2_GetActorRotation`)))
  ;[1 1 1] Update Rotation
  (bind _returnvalue (`KismetMaterialLibrary.GetScalarParameterValue` "/Game/Stigma/Foliage_Grass/MPC_Wind.MPC_Wind" "Wind Intensity"))
  (if (== _returnvalue 0.0)
    (`self.K2_SetActorRotation` (`KismetMathLibrary.MakeRotator` 0.0 _returnvalue_pitch _returnvalue_yaw) true)
    (else
      (bind (_direction _wind) (`Timeline|WindOnFlower`)
        (:`Update`
          (`self.K2_SetActorRotation` (`KismetMathLibrary.MakeRotator` (`KismetMathLibrary.Lerp` 20.0 30.0 _wind) _returnvalue_pitch _returnvalue_yaw)))))))

(event `self.ReceiveActorBeginOverlap`
  (params (OtherActor :type "Actor Object Reference"))
  ;[1 1 1] Apply Damage
  (bind _assecond_gameplay_character (cast `/Game/ThirdPersonCPP/Blueprints/SecondGameplayCharacter` OtherActor))
  (`AkGameplayStatics.PostEvent` "/Game/Stigma/Sound/flowerBell.flowerBell" self))

(fn `UserConstructionScript`)