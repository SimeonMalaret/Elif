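; Switch Actor that activates when hit by explosion damage and switches itself off again after a set duration.
; AnyDamage filters for ExplosionDamage, ignores hits while already active, then sets IsActive and turns the Cylinder orange.
; After a Delay of Duration it clears IsActive and restores the yellow material.
; A Zone.TestZoneActivation call exists in the graph but is never executed.
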(event `self.ReceiveAnyDamage`
  (params (Damage :type "Float (single-precision)") (DamageType :type "DamageType Object Reference") (InstigatedBy :type "Controller Object Reference") (DamageCauser :type "Actor Object Reference"))
  (cast `/Game/Blueprints/ExplosionDamage` DamageType)
  (if (not (`self.isActive`))
    (set `self.isActive` true)
    (`PrimitiveComponent.SetMaterial` (`self.Cylinder`) 0 "/Game/Blueprints/Orange.Orange")
    (`KismetSystemLibrary.Delay` (`self.Duration`))
    (set `self.isActive` false)
    (`PrimitiveComponent.SetMaterial` (`self.Cylinder`) 0 "/Game/Blueprints/Yellow.Yellow")))

(fn `UserConstructionScript`)