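; Pillar is an actor that activates when the dashing third-person character overlaps it, as part of a zone puzzle.
; On overlap it checks the character's dash state, with a DashConstraint flag that, when off, lets any overlap by that character activate it.
; Activation marks the pillar active, turns its cylinder green and asks its Zone to test whether the zone should activate.
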(event `self.ReceiveActorBeginOverlap`
  (params (OtherActor :type "Actor Object Reference"))
  (bind _asthird_person_character_dash_simple (cast `/Game/ThirdPersonCPP/Blueprints/ThirdPersonCharacterDashSimple` OtherActor))
  (if (`/Game/ThirdPersonCPP/Blueprints/ThirdPersonCharacterDashSimple.isDashing` _asthird_person_character_dash_simple)
    (set `self.isActive` true :!label _label)
    (`PrimitiveComponent.SetMaterial` (`self.Cylinder`) 0 "/Game/Blueprints/Green.Green")
    (`/Game/Blueprints/PillarZone.TestZoneActivation` (`self.Zone`))
    (elif (not (`self.dashConstraint`))
      (goto _label))))

(fn `UserConstructionScript`)