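; Player character Blueprint with wall jumping and a stamina-limited "night morph" dash that ends in a damaging explosion.
; Holding Dash raises speed, removes gravity, turns the mesh blue and overlaps a custom collision channel.
; Actor overlaps grow the explosion zone; releasing Dash, exhausting stamina or touching NoNightMorph_Blueprint resets movement and damages actors inside it.
; Tick drives stamina and dash cooldown; older launch-dash and DashPoint logic is disconnected.
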(event `self.ReceiveActorEndOverlap`
  (params (OtherActor :type "Actor Object Reference"))
  ;[1 1 1] EndOverlap
  (if (`KismetArrayLibrary.Array_Contains` (`Actor.Tags` OtherActor) "DashPoint")
    (set `self.isNearDashPoint` false)
    (set `self.DashPoint` null)))

(event `self.ReceiveBeginPlay`
  ;[1 1 1] BeginPlay : Creates Stamina UI
  (bind _returnvalue (`|CreateWidget` "/Game/ThirdPersonCPP/Blueprints/SimeonTests/StaminaUI.StaminaUI_C"))
  (`UserWidget.AddToViewport` _returnvalue 0)
  (set `self.ExplosionSize` 0.0)
  (`SceneComponent.SetWorldScale3D` (`self.ExplosionZone`) (0.0 0.0 0.0)))

(event `InputAction|Jump`
  (params (Key :type "Key Structure"))
  ;[1 1 1] Jump & Wall Jump
  (:`Pressed`
    (if (`self.CanJumpBool`)
      (`self.Jump`)
      (`self.WallJump`)))
  (:`Released`
    (`self.StopJumping`)))

(event `InputAction|Dash`
  (params (Key :type "Key Structure"))
  ;[1 1 1] Dash / Sprint
  (:`Pressed`
    (if (`self.CanDash`)
      (`self.Dash Function`)
      (set `self.ExplosionSize` 0.0)
      (`SceneComponent.SetWorldScale3D` (`self.ExplosionZone`) (0.0 0.0 0.0))))
  (:`Released`
    (`self.Reset Dash`)
    (`self.Explosion`)))

(event `self.ReceiveTick`
  (params (DeltaSeconds :type "Float (single-precision)"))
  ;[1 1 1] night morph
  (`|ExecutionSequence`
    (:`then_0`
      (if (not (`self.CanDash`))
        (`KismetSystemLibrary.Delay` (`self.DashCd`))
        (set `self.CanDash` true)))
    (:`then_1`
      (if (`self.StaminaOn`)
        (set `self.Stamina` (`KismetMathLibrary.FClamp` (- (`self.Stamina`) 0.5) 0.0 100.0))
        (elif (not (`NavMovementComponent.IsFalling` (`self.CharacterMovement`)))
          (set `self.Stamina` (`KismetMathLibrary.FClamp` (+ (`self.Stamina`) 0.5) 0.0 100.0)))))
    (:`then_2`
      (if (<= (`self.Stamina`) 0.0)
        (`self.Reset Dash`)
        (set `self.CanDash` false)
        (`self.Explosion`)))))

(event `Key|E`
  (params (Key :type "Key Structure"))
  ;[1 1 1] Dash to Landmark
)

(event `self.ReceiveActorBeginOverlap`
  (params (OtherActor :type "Actor Object Reference"))
  (cast `/Game/Blueprints/NoNightMorph_Blueprint` OtherActor
    (:`then`
      (`self.Reset Dash`)
      (set `self.CanDash` false)
      (`self.Explosion`))
    (:`CastFailed`
      (bind _output_get (set `self.ExplosionSize` (+ (`self.ExplosionSize`) (`self.ExplosionIncrementation`))))
      (if (> _output_get (`self.MaxExplosionSize`))
        (bind _output_get_2 (set `self.ExplosionSize` (`self.MaxExplosionSize`))))
      (`SceneComponent.SetWorldScale3D` (`self.ExplosionZone`) (* (`KismetMathLibrary.Vector_One`) _output_get_2)))))

(event `self.ExplosionZone.OnComponentBeginOverlap`
  (params (OverlappedComponent :type "PrimitiveComponent Object Reference") (OtherActor :type "Actor Object Reference") (OtherComp :type "PrimitiveComponent Object Reference") (OtherBodyIndex :type Integer) (bFromSweep :type Boolean) (SweepResult :type "HitResult Structure (by ref)"))
  (`KismetArrayLibrary.Array_Add` (`self.ActorInExplosionRange`) OtherActor))

(event `self.ExplosionZone.OnComponentEndOverlap`
  (params (OverlappedComponent :type "PrimitiveComponent Object Reference") (OtherActor :type "Actor Object Reference") (OtherComp :type "PrimitiveComponent Object Reference") (OtherBodyIndex :type Integer))
  (`KismetArrayLibrary.Array_RemoveItem` (`self.ActorInExplosionRange`) OtherActor))

(fn `Dash Function`
  (bind _charactermovement (`self.CharacterMovement`))
  (bind (_velocity_x _velocity_y) (`KismetMathLibrary.BreakVector` (`MovementComponent.Velocity` _charactermovement)))
  (if (> (`self.Stamina`) 10.0)
    (set `MovementComponent.Velocity` (`KismetMathLibrary.MakeVector` _velocity_x _velocity_y) _charactermovement)
    (set `CharacterMovementComponent.MaxWalkSpeed` 1400.0 (`self.CharacterMovement`))
    (`PrimitiveComponent.SetMaterial` (`self.Mesh`) 0 "/Game/Blueprints/Blue.Blue")
    (set `self.CanJumpBool` false)
    (set `CharacterMovementComponent.GravityScale` 0.0 (`self.CharacterMovement`))
    (set `self.StaminaOn` true)
    (`PrimitiveComponent.SetCollisionResponseToChannel` (`self.CapsuleComponent`) "ECC_GameTraceChannel1" "ECR_Overlap")))

(fn `Explosion`
  (for _array_element (`self.ActorInExplosionRange`)
    (`GameplayStatics.ApplyDamage` _array_element (* (`self.ExplosionSize`) (`self.ExplosionDamageBySize`)) null null "/Game/Blueprints/ExplosionDamage.ExplosionDamage_C")
    (`KismetSystemLibrary.PrintString` (`KismetSystemLibrary.GetPathName` _array_element)))
  (`SceneComponent.SetWorldScale3D` (`self.ExplosionZone`) (0.0 0.0 0.0)))

(fn `Reset Dash`
  (set `CharacterMovementComponent.MaxWalkSpeed` 700.0 (`self.CharacterMovement`))
  (`PrimitiveComponent.SetMaterial` (`self.Mesh`) 0 "/Game/Mannequin/Character/Materials/M_Male_Body.M_Male_Body")
  (set `self.CanJumpBool` true)
  (set `CharacterMovementComponent.GravityScale` 5.0 (`self.CharacterMovement`))
  (set `self.StaminaOn` false)
  (`PrimitiveComponent.SetCollisionResponseToChannel` (`self.CapsuleComponent`) "ECC_GameTraceChannel1" "ECR_Block"))

(fn `ResetCollisions`
  (`PrimitiveComponent.SetCollisionResponseToChannel` (`self.CapsuleComponent`) "ECC_GameTraceChannel1" "ECR_Block"))

(fn `UserConstructionScript`)

(fn `WallJump`
  (locals (`Jump Velocity` :type "Float (double-precision)" :default 1200.0) (`Radius Offset to Wall Jump` :type "Float (double-precision)" :default 50.0))
  (bind _returnvalue (`self.K2_GetActorLocation`))
  (bind _capsulecomponent (`self.CapsuleComponent`))
  (if (not (`NavMovementComponent.IsMovingOnGround` (`self.CharacterMovement`)))
    (bind (_outhit _returnvalue_2) (`KismetSystemLibrary.CapsuleTraceSingle` :`Start` _returnvalue :`End` _returnvalue :`Radius` (+ (`CapsuleComponent.CapsuleRadius` _capsulecomponent) (`local.Radius Offset to Wall Jump`)) :`HalfHeight` (`CapsuleComponent.CapsuleHalfHeight` _capsulecomponent) :`TraceChannel` "TraceTypeQuery1" :`DrawDebugType` "Persistent"))
    (if _returnvalue_2
      (bind (_returnvalue_x _returnvalue_y) (`KismetMathLibrary.BreakVector` (* (`.ImpactNormal` (`GameplayStatics.BreakHitResult` _outhit)) 500.0)))
      (`self.LaunchCharacter` (`KismetMathLibrary.MakeVector` _returnvalue_x _returnvalue_y (`CharacterMovementComponent.JumpZVelocity` (`self.CharacterMovement`))) true true))))