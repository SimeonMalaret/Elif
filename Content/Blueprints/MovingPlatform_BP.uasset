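; Moving platform actor that travels along a Path array of placed actors, either looping or ping-ponging between the ends.
; BeginPlay snaps it to the current waypoint and picks the next, or prints a warning if the path is too short.
; Tick lerps location between waypoints, switching targets as alpha reaches one and carrying over the remainder.
; Speed advances alpha, so every segment takes equal time regardless of length.
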(event `self.ReceiveBeginPlay`
  (if (<= (`KismetArrayLibrary.Array_Length` (`self.path`)) 1)
    (`KismetSystemLibrary.PrintString` "Moving platform without path" true true (struct :`G` 0.66 :`B` 1.0 :`A` 1.0) 10000000.0)
    (else
      (`self.K2_SetActorLocation` (`self.K2_GetActorLocation` (`|GetArrayItem` (`self.path`) (`self.currentPathId`))) false true)
      (if (`self.isInPostitiveDirection`)
        (set `self.nextPathId` (+ (`self.currentPathId`) 1))
        (else
          (set `self.nextPathId` (- (`self.nextPathId`) 1)))))))

(event `self.ReceiveTick`
  (params (DeltaSeconds :type "Float (single-precision)"))
  (bind _nextpathid (`self.nextPathId`))
  (bind _nextpathid_2 (`self.nextPathId`))
  ;[1 1 1] lerp avencement
  (bind _output_get (set `self.lerpLocationAlpha` (+ (`self.lerpLocationAlpha`) (* (`self.speed`) (`GameplayStatics.GetWorldDeltaSeconds`)))))
  (if (not (< _output_get 1.0))
    (set `self.lerpLocationAlpha` (- (`self.lerpLocationAlpha`) 1.0))
    (if (`self.loop`)
      ;[1 1 1] loop switch target
      (set `self.currentPathId` _nextpathid_2)
      (if (>= _nextpathid_2 (- (`KismetArrayLibrary.Array_Length` (`self.path`)) 1))
        (set `self.nextPathId` 0)
        (else
          (set `self.nextPathId` (+ (`self.nextPathId`) 1))))
      (else
        ;[1 1 1] go back switch target
        (set `self.currentPathId` _nextpathid)
        (if (or (>= _nextpathid (- (`KismetArrayLibrary.Array_Length` (`self.path`)) 1)) (== (`self.nextPathId`) 0))
          (bind _output_get_2 (set `self.isInPostitiveDirection` (not (`self.isInPostitiveDirection`)))))
        (if _output_get_2
          (set `self.nextPathId` (+ (`self.nextPathId`) 1))
          (else
            (set `self.nextPathId` (- (`self.nextPathId`) 1)))))))
  ;[1 1 1] Set location
  (`self.K2_SetActorLocation` (`KismetMathLibrary.VLerp` (`self.K2_GetActorLocation` (`|GetArrayItem` (`self.path`) (`self.currentPathId`))) (`self.K2_GetActorLocation` (`|GetArrayItem` (`self.path`) (`self.nextPathId`))) (`self.lerpLocationAlpha`))))

(fn `UserConstructionScript`)